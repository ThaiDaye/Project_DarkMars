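; RoomPlacer_Master is a room placement marker that previews layout through its Construction Script, with no runtime logic.
; When active, it adds one box for its X/Y radius and another for the grid-sized room footprint, with room X and Y swapped.
; An active connected placer gets two distance-scaled arrows aimed at it.
; Dungeon rooms show a large terrain billboard and two side arrows reflecting dungeon width, length and start direction.
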(fn `UserConstructionScript`
  (bind _returnvalue (`self.GetTransform`))
  (bind _billboard (`self.Billboard`))
  (bind _dungeonstartdirection (`self.DungeonStartDirection`))
  (bind _connectedroomplacer (`self.ConnectedRoomPlacer`))
  (bind _returnvalue_2 (`SceneComponent.K2_GetComponentLocation` (`self.DefaultSceneRoot`)))
  (bind _returnvalue_3 (`self.K2_GetActorLocation` _connectedroomplacer))
  (bind _returnvalue_4 (* (`self.GridSize`) 0.5))
  (bind _returnvalue_5 (select `int` (`self.DungeonStartDirection`) :`0` 0.0 :`1` 90.0 :`2` 180.0 :`3` 270.0 :!type "Float (single-precision)"))
  (bind _returnvalue_6 (`KismetMathLibrary.FindLookAtRotation` _returnvalue_2 _returnvalue_3))
  (bind _returnvalue_7 (or (== _dungeonstartdirection 0) (== _dungeonstartdirection 2)))
  (bind _returnvalue_8 (* (* (`self.DungeonLength`) (`self.GridSize`)) 0.5))
  (bind _returnvalue_9 (* (* (`self.DungeonWidth`) (`self.GridSize`)) 10.0))
  (bind _returnvalue_10 (`KismetMathLibrary.VSize` (- _returnvalue_2 _returnvalue_3)))
  (bind _returnvalue_11 (* _returnvalue_9 -1.0))
  (if (`self.Active`)
    (`/Engine/EditorBlueprintResources/StandardMacros.IsValid` _connectedroomplacer
      (:`Is Valid`
        (if (`/Game/Blueprints/RoomPlacer_Master.Active` (`self.ConnectedRoomPlacer`))
          (`AddComponent|NODE_AddArrowComponent-0` :`RelativeTransform` (`KismetMathLibrary.MakeTransform` (`KismetMathLibrary.InverseTransformLocation` _returnvalue (`KismetMathLibrary.VLerp` _returnvalue_2 _returnvalue_3 0.5)) _returnvalue_6 (`KismetMathLibrary.MakeVector` (/ _returnvalue_10 5000.0) 0.5 0.25)))
          (`AddComponent|NODE_AddArrowComponent-1` :`RelativeTransform` (`KismetMathLibrary.MakeTransform` (`KismetMathLibrary.InverseTransformLocation` _returnvalue _returnvalue_2) _returnvalue_6 (`KismetMathLibrary.MakeVector` (/ _returnvalue_10 4250.0) 0.5 0.25)))))
      (:`Is Not Valid`
        _))
    (bind _returnvalue_12 (`AddComponent|NODE_AddBoxComponent-0` :`RelativeTransform` (`KismetMathLibrary.MakeTransform` (0.0 0.0 0.0))))
    (`BoxComponent.SetBoxExtent` _returnvalue_12 (`KismetMathLibrary.MakeVector` (`self.RadiusX`) (`self.RadiusY`) 100.0) true)
    (bind _returnvalue_13 (`AddComponent|NODE_AddBoxComponent-1` :`RelativeTransform` (`KismetMathLibrary.MakeTransform` (0.0 0.0 0.0))))
    (`BoxComponent.SetBoxExtent` _returnvalue_13 (`KismetMathLibrary.MakeVector` (* (`self.Room Y`) _returnvalue_4) (* (`self.Room X`) _returnvalue_4) 100.0) true)
    (if (`self.IsDungeonRoom`)
      (`BillboardComponent.SetSprite` _billboard "/Engine/EditorResources/S_Terrain.S_Terrain")
      (`SceneComponent.SetWorldScale3D` _billboard (10.0 10.0 10.0))
      (bind _returnvalue_14 (`AddComponent|NODE_AddArrowComponent-2` :`RelativeTransform` (`KismetMathLibrary.MakeTransform` (select `bool` _returnvalue_7 :`false` (`KismetMathLibrary.MakeVector` _returnvalue_9) :`true` (`KismetMathLibrary.MakeVector` 0.0 _returnvalue_9)) (`KismetMathLibrary.MakeRotator` 0.0 0.0 _returnvalue_5))))
      (bind _returnvalue_15 (`AddComponent|NODE_AddArrowComponent-3` :`RelativeTransform` (`KismetMathLibrary.MakeTransform` (select `bool` _returnvalue_7 :`false` (`KismetMathLibrary.MakeVector` _returnvalue_11) :`true` (`KismetMathLibrary.MakeVector` 0.0 _returnvalue_11)) (`KismetMathLibrary.MakeRotator` 0.0 0.0 _returnvalue_5))))
      (set `ArrowComponent.ArrowLength` _returnvalue_8 _returnvalue_15)
      (set `ArrowComponent.ArrowLength` _returnvalue_8 _returnvalue_14))))