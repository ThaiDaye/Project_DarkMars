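; Base projectile Blueprint that damages object and enemy entries on impact.
; On BeginPlay it activates ProjectileMovement, whose activation event sets InitialSpeed from StartVelocity.X.
; Hits on anything but its Parent run a debug-drawn sphere trace at the impact point, then destroy the projectile.
; If no HitTarget is stored yet, a blocking hit on an ObjectEntry_Master or EnemyEntry_Master stores it and applies BaseDamage with a type-specific MaxLost.
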(event `self.ProjectileMovement.OnComponentActivated`
  (params (Component :type "ActorComponent Object Reference") (bReset :type Boolean))
  (set `ProjectileMovementComponent.InitialSpeed` (.x (`self.StartVelocity`)) (`self.ProjectileMovement`)))

(event `self.ReceiveBeginPlay`
  (`ActorComponent.Activate` (`self.ProjectileMovement`) false))

(event `self.ReceiveHit`
  (params (MyComp :type "PrimitiveComponent Object Reference") (Other :type "Actor Object Reference") (OtherComp :type "PrimitiveComponent Object Reference") (bSelfMoved :type Boolean) (HitLocation :type "Vector Structure") (HitNormal :type "Vector Structure") (NormalImpulse :type "Vector Structure") (Hit :type "HitResult Structure (by ref)"))
  (bind (_bblockinghit _binitialoverlap _time _distance _location _impactpoint _normal _impactnormal _physmat _hitactor) (`GameplayStatics.BreakHitResult` Hit))
  (if (not (== Other (`self.Parent`)))
    (`KismetSystemLibrary.SphereTraceSingle` :`Start` HitLocation :`End` HitLocation :`Radius` 15.0 :`TraceChannel` "TraceTypeQuery1" :`DrawDebugType` "ForDuration" :`TraceColor` (struct :`R` 1.0 :`G` 0.653453 :`A` 1.0) :`TraceHitColor` (struct :`R` 1.0 :`G` 0.653453 :`A` 1.0) :`DrawTime` 0.2)
    (`/Engine/EditorBlueprintResources/StandardMacros.IsValid` (`self.HitTarget`)
      (:`Is Valid`
        _)
      (:`Is Not Valid`
        (if _bblockinghit
          (bind _asobject_entry_master (cast `/Game/Blueprints/Objects/ObjectEntry_Master` _hitactor)
            (:`then`
              (set `self.HitTarget` _asobject_entry_master)
              (`/Game/Blueprints/Objects/ObjectEntry_Master.TakeDamage` _asobject_entry_master (`self.BaseDamage`) 0.1))
            (:`CastFailed`
              (bind _asenemy_entry_master (cast `/Game/Blueprints/Enemies/EnemyEntry_Master` _hitactor)
                (:`then`
                  (set `self.HitTarget` _asenemy_entry_master)
                  (`/Game/Blueprints/Enemies/EnemyEntry_Master.TakeDamage` _asenemy_entry_master (`self.BaseDamage`) 0.25 self))
                (:`CastFailed`
                  _)))))))
    (`self.K2_DestroyActor`)))

(fn `UserConstructionScript`)