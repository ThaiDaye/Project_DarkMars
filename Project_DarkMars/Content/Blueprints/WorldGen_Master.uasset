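; World generator Blueprint that builds a random grid of walls on BeginPlay.
; It sizes a 2D map, stored as an array of structs wrapping inner arrays, then randomly marks each cell as wall or empty using GridWallRatio.
; DrawMap then adds an instanced static mesh at each wall cell, spaced by GridSize.
; A ForEachMapEntry macro handles the nested iteration for both filling and drawing.
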(event `self.ReceiveBeginPlay`
  (bind _resized_map (`self.ResizeMap` (`self.Map`)))
  (bind _output_get (set `self.Map` _resized_map))
  (bind (_x _y) (`self.ForEachMapEntry` _output_get)
    (:`LoopBody`
      (`self.SetMapEntry` _output_get _x _y (`KismetSystemLibrary.MakeLiteralInt` (select `bool` (>= (`KismetMathLibrary.RandomFloatInRange` 0.0 1.0) (`self.GridWallRatio`)) :`false` 1))))
    (:`Completed`
      (`self.DrawMap` _output_get))))

(fn `DrawMap`
  (params (Map :type "Array of /Game/Blueprints/Map_Struct Structure"))
  (bind _gridsize (`self.GridSize`))
  (bind (_x _y) (`self.ForEachMapEntry` Map)
    (:`LoopBody`
      (bind _id (`self.GetMapEntry` _x _y))
      (if (select `int` _id :`0` false :`1` true)
        (`InstancedStaticMeshComponent.AddInstance` (`self.InstancedStaticMesh`) (`KismetMathLibrary.MakeTransform` (`KismetMathLibrary.MakeVector` (* (* _y -1) _gridsize) (* _x _gridsize))) false)))
    (:`Completed`
      (return))))

(fn `GetMapEntry`
  (params (x :type Integer) (y :type Integer))
  (returns (ID :type Integer))
  (return (`|GetArrayItem` (`.Y_3_B90EE5EB443401C914354FAE18D1B269` (break `/Game/Blueprints/Map_Struct` (`|GetArrayItem` (`self.Map`) x))) y)))

(fn `ResizeMap`
  (params (Map :type "Array of /Game/Blueprints/Map_Struct Structure (by ref)"))
  (returns (`Resized Map` :type "Array of /Game/Blueprints/Map_Struct Structure"))
  (`KismetArrayLibrary.Array_Resize` (`self.Temp_Array`) (`self.Height Y`))
  (for _index (range (`self.Width X`))
    (`KismetArrayLibrary.Array_Set` Map _index (make `/Game/Blueprints/Map_Struct` (`self.Temp_Array`)) true))
  (return Map))

(fn `SetMapEntry`
  (params (Map :type "Array of /Game/Blueprints/Map_Struct Structure (by ref)") (X :type Integer) (Y :type Integer) (`Desired ID` :type Integer))
  (locals (array :type "Array of Integer"))
  ;[1 1 1] set
  (set `local.array` (`.Y_3_B90EE5EB443401C914354FAE18D1B269` (break `/Game/Blueprints/Map_Struct` (`|GetArrayItem` Map X))))
  (`KismetArrayLibrary.Array_Set` (`local.array`) Y `Desired ID` true)
  (`KismetArrayLibrary.Array_Set` Map X (make `/Game/Blueprints/Map_Struct` (`local.array`)) true))

(fn `UserConstructionScript`)