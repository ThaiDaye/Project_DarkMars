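; RoomGen_Master is a room or hallway piece for grid-based room generation, drawn as box outlines.
; Its construction script sizes an outer box from width, height and grid size, plus an inner box inset by the border size, both snapped to a 100-unit grid.
; Hallways also get an arrow component, and a billboard at random height shows a sprite by piece type.
; The event graph is unused.
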(fn `UserConstructionScript`
  (bind _returnvalue (`KismetMathLibrary.MakeTransform` (0.0 0.0 0.0)))
  (bind _returnvalue_2 (`KismetMathLibrary.MakeTransform` (0.0 0.0 0.0)))
  (bind _billboard (`self.Billboard`))
  (bind _bordervisual (`self.BorderVisual`))
  (bind _visual (`self.Visual`))
  (bind _returnvalue_3 (* (`self.GridSize`) 0.5))
  (bind _returnvalue_4 (* (`self.GridSize`) 0.5))
  (bind _returnvalue_5 (`KismetMathLibrary.Vector_SnappedToGrid` (`SceneComponent.K2_GetComponentLocation` _visual) 100.0))
  (bind _returnvalue_6 (* (`KismetSystemLibrary.MakeLiteralInt` (`self.RoomBorderSize`)) 2))
  (if (`self.IsHallway`)
    (if (`self.XHallway`)
      (`AddComponent|NODE_AddArrowComponent-0`)
      (else
        (`AddComponent|NODE_AddArrowComponent-1`)))
    (bind _returnvalue_7 (`AddComponent|NODE_AddBoxComponent-2` :`RelativeTransform` _returnvalue_2))
    (set `self.Visual` _returnvalue_7)
    (else
      (bind _returnvalue_8 (`AddComponent|NODE_AddBoxComponent-0` :`RelativeTransform` _returnvalue_2))
      (set `self.Visual` _returnvalue_8)))
  (`BoxComponent.SetBoxExtent` _visual (`KismetMathLibrary.MakeVector` (* (`self.Height Y`) _returnvalue_4) (* (`self.Width X`) _returnvalue_4) 100.0) true)
  (`SceneComponent.K2_SetWorldLocation` _visual _returnvalue_5 false false)
  (`SceneComponent.K2_SetWorldLocation` _billboard (`KismetMathLibrary.MakeVector` (.x _returnvalue_5) (.y _returnvalue_5) (`KismetMathLibrary.RandomFloatInRange` 200.0 800.0)) false false)
  (`BillboardComponent.SetSprite` _billboard (select `bool` (`self.IsMainRoom`) :`false` (select `bool` (`self.IsHallway`) :`false` "/Engine/EditorResources/S_VectorFieldVol.S_VectorFieldVol" :!type "Texture2D Object Reference") :`true` "/Engine/EditorResources/LevelInstance.LevelInstance"))
  (if (`self.IsHallway`)
    (bind _returnvalue_9 (`AddComponent|NODE_AddBoxComponent-3` :`RelativeTransform` _returnvalue))
    (set `self.BorderVisual` _returnvalue_9)
    (else
      (bind _returnvalue_10 (`AddComponent|NODE_AddBoxComponent-1` :`RelativeTransform` _returnvalue))
      (set `self.BorderVisual` _returnvalue_10)))
  (`BoxComponent.SetBoxExtent` _bordervisual (`KismetMathLibrary.MakeVector` (* (- (`self.Height Y`) _returnvalue_6) _returnvalue_3) (* (- (`self.Width X`) _returnvalue_6) _returnvalue_3) 100.0) true)
  (`SceneComponent.K2_SetWorldLocation` _bordervisual (`KismetMathLibrary.Vector_SnappedToGrid` (`SceneComponent.K2_GetComponentLocation` _bordervisual) 100.0) false false))