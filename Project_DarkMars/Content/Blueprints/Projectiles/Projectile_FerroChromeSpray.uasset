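; Ferro-chrome spray projectile that calls heal-damage functions on objects and enemies of two substance types, and can chrome-plate what it hits.
; A false heal result spawns the success particle system, and a random roll swaps the hit component's materials to chrome.
; A fast timer lowers CustomTimeDilation to a floor, slowing the projectile.
; A second timer damages the Parent top-down character while it overlaps the sphere.
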(event `self.ReceiveBeginPlay`
  (`parent.ReceiveBeginPlay`)
  (`KismetSystemLibrary.K2_SetTimerDelegate` (delegate `ReduceSpeed`) 0.01 true)
  (`KismetSystemLibrary.K2_SetTimerDelegate` (delegate `TickPlayerDamage`) 1.0 true))

(event `ReduceSpeed`
  (set `self.CustomTimeDilation` (`KismetMathLibrary.FClamp` (- (`self.CustomTimeDilation`) 0.0075) 0.2)))

(event `self.ReceiveHit`
  (params (MyComp :type "PrimitiveComponent Object Reference") (Other :type "Actor Object Reference") (OtherComp :type "PrimitiveComponent Object Reference") (bSelfMoved :type Boolean) (HitLocation :type "Vector Structure") (HitNormal :type "Vector Structure") (NormalImpulse :type "Vector Structure") (Hit :type "HitResult Structure (by ref)"))
  (`parent.ReceiveHit` MyComp Other OtherComp bSelfMoved HitLocation HitNormal NormalImpulse Hit)
  (bind _asobject_entry_master (cast `/Game/Blueprints/Objects/ObjectEntry_Master` Other)
    (:`then`
      (bind _object_substance (`/Game/Blueprints/Objects/ObjectEntry_Master.Object Substance` _asobject_entry_master))
      (if (or (`|EnumEquality` _object_substance "NewEnumerator6") (`|EnumEquality` _object_substance "NewEnumerator3"))
        (bind _fullhealth (`/Game/Blueprints/Objects/ObjectEntry_Master.HealDamage_Object` _asobject_entry_master 10.0 0.75))
        (if (not _fullhealth)
          (`NiagaraFunctionLibrary.SpawnSystemAtLocation` "/Game/VFX/Spray_SUCCESS_Projectile_particle_System.Spray_SUCCESS_Projectile_particle_System" HitLocation :!label _label)))
      (if (`KismetMathLibrary.RandomBoolWithWeight` 0.2) :!label _label_2
        (for _index (range (`PrimitiveComponent.GetNumMaterials` OtherComp))
          (`PrimitiveComponent.SetMaterial` OtherComp _index "/Game/ScienceLab/Materials/Rooms/Wall/MI_Metal_CRHOME.MI_Metal_CRHOME"))))
    (:`CastFailed`
      (bind _asenemy_entry_master (cast `/Game/Blueprints/Enemies/EnemyEntry_Master` Other))
      (bind _enemy_substance (`/Game/Blueprints/Enemies/EnemyEntry_Master.Enemy Substance` _asenemy_entry_master))
      (if (or (`|EnumEquality` _enemy_substance "NewEnumerator6") (`|EnumEquality` _enemy_substance "NewEnumerator3"))
        (bind _fullhealth_2 (`/Game/Blueprints/Enemies/EnemyEntry_Master.HealDamage_Enemy` _asenemy_entry_master 5.0 0.5))
        (if _fullhealth_2
          (goto _label_2)
          (else
            (goto _label)))))))

(event `TickPlayerDamage`
  (bind _parent (`self.Parent`))
  (if (`PrimitiveComponent.IsOverlappingActor` (`self.Sphere`) _parent)
    (bind _asbp_top_down_character (cast `/Game/Blueprints/BP_TopDownCharacter` _parent))
    (`/Game/Blueprints/BP_TopDownCharacter.TakeDamage` _asbp_top_down_character 5.0 0.0 0.0 0.0 (`self.Parent`))))

(fn `UserConstructionScript`
  (`parent.UserConstructionScript`))