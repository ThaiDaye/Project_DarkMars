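; Master gib projectile that leaves blood decals where it hits and triggers bloody footsteps when the player overlaps its sphere.
; BeginPlay randomly sets AttachOnDestroy and, if RandomVisual is on, picks a random mesh and material.
; Hits pass through a gate that reopens after a short delay, throttling decals and deactivating the Niagara component.
; Decals are Niagara systems aligned to the impact normal, attached to hit objects or enemy bones, otherwise placed in world.
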(event `self.ReceiveBeginPlay`
  (bind _visual (`self.Visual`))
  (`parent.ReceiveBeginPlay`)
  (set `self.AttachOnDestroy` (`KismetMathLibrary.RandomBoolWithWeight` 0.5))
  (if (`self.RandomVisual`)
    (`StaticMeshComponent.SetStaticMesh` _visual (select `int` (`KismetMathLibrary.RandomIntegerInRange` 0 2) :`0` "/Game/Meshes/BodyParts/Gib_Mesh1.Gib_Mesh1" :`1` "/Game/Meshes/BodyParts/Gib_Mesh2.Gib_Mesh2" :`2` "/Game/Meshes/BodyParts/Gib_Mesh3.Gib_Mesh3" :!type "StaticMesh Object Reference"))
    (`PrimitiveComponent.SetMaterial` _visual 0 (select `int` (`KismetMathLibrary.RandomIntegerInRange` 0 2) :`0` "/Game/Materials/BasicMat_Gibs_4.BasicMat_Gibs_4" :`1` "/Game/Materials/BasicMat_Gibs_3.BasicMat_Gibs_3" :`2` "/Game/Materials/BasicMat_Gibs_2.BasicMat_Gibs_2" :!type "MaterialInterface Object Reference"))))

(event `self.ReceiveHit`
  (params (MyComp :type "PrimitiveComponent Object Reference") (Other :type "Actor Object Reference") (OtherComp :type "PrimitiveComponent Object Reference") (bSelfMoved :type Boolean) (HitLocation :type "Vector Structure") (HitNormal :type "Vector Structure") (NormalImpulse :type "Vector Structure") (Hit :type "HitResult Structure (by ref)"))
  (bind (_bblockinghit _binitialoverlap _time _distance _location _impactpoint _normal _impactnormal _physmat _hitactor _hitcomponent _hitbonename) (`GameplayStatics.BreakHitResult` Hit))
  (bind _returnvalue (`KismetMathLibrary.MakeRotator` (.roll (`KismetMathLibrary.Conv_VectorToRotator` _impactnormal)) (+ (.pitch (`KismetMathLibrary.Conv_VectorToRotator` _impactnormal)) -90.0) (.yaw (`KismetMathLibrary.Conv_VectorToRotator` _impactnormal))))
  (`parent.ReceiveHit` MyComp Other OtherComp bSelfMoved HitLocation HitNormal NormalImpulse Hit)
  (`|ExecutionSequence`
    (:`then_0`
      (`/Engine/EditorBlueprintResources/StandardMacros.Gate` false :!label _label
        (:`Exit`
          (`|ExecutionSequence`
            (:`then_0`
              (`ActorComponent.Deactivate` (`self.Niagara`))
              (bind _asobject_entry_master (cast `/Game/Blueprints/Objects/ObjectEntry_Master` _hitactor)
                (:`then`
                  ;[1 1 1] decal
                  (`NiagaraFunctionLibrary.SpawnSystemAttached` "/Game/VFX/Systems/Decal/DecalBlood_ParticleSystem_2.DecalBlood_ParticleSystem_2" (`/Game/Blueprints/Objects/ObjectEntry_Master.visual` _asobject_entry_master) "None" _impactpoint _returnvalue "KeepWorldPosition" true))
                (:`CastFailed`
                  (bind _asenemy_entry_master (cast `/Game/Blueprints/Enemies/EnemyEntry_Master` _hitactor)
                    (:`then`
                      (`NiagaraFunctionLibrary.SpawnSystemAttached` "/Game/VFX/Systems/Decal/DecalBlood_ParticleSystem_2.DecalBlood_ParticleSystem_2" (`Character.Mesh` _asenemy_entry_master) _hitbonename _impactpoint _returnvalue "KeepWorldPosition" true))
                    (:`CastFailed`
                      (`NiagaraFunctionLibrary.SpawnSystemAtLocation` "/Game/VFX/Systems/Decal/DecalBlood_ParticleSystem_2.DecalBlood_ParticleSystem_2" _impactpoint _returnvalue))))))
            (:`then_1`
              (`KismetSystemLibrary.Delay` 0.2)
              (goto _label :!via `Open`))))))
    (:`then_1`
      (goto _label :!via `Close`))))

(event `self.Sphere.OnComponentBeginOverlap`
  (params (OverlappedComponent :type "PrimitiveComponent Object Reference") (OtherActor :type "Actor Object Reference") (OtherComp :type "PrimitiveComponent Object Reference") (OtherBodyIndex :type Integer) (bFromSweep :type Boolean) (SweepResult :type "HitResult Structure (by ref)"))
  (bind _playerref (`self.PlayerRef`))
  (if (== OtherActor _playerref)
    (`/Game/Blueprints/BP_TopDownCharacter.BloodyFootsteps` _playerref)))

(fn `UserConstructionScript`
  (`parent.UserConstructionScript`))