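; Throwable repair grenade projectile that hovers and sprays healing projectiles after it lands.
; The first hit arms it; after a short delay it disables gravity, levels out and rises on a timeline.
; A fast looping timer then spins and jitters the sphere, spawning slowed FerroHealSpray projectiles at random pitches.
; After a few seconds spraying stops, then the material changes, gravity returns and the sphere simulates physics.
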(event `self.ReceiveBeginPlay`
  (`parent.ReceiveBeginPlay`)
  (`KismetSystemLibrary.K2_SetTimerDelegate` (delegate `SprayHeal`) 0.03 true))

(event `SprayHeal`
  (bind _sphere (`self.Sphere`))
  (bind _sphere_2 (`self.Sphere`))
  (bind (_returnvalue_roll _returnvalue_pitch _returnvalue_yaw) (`KismetMathLibrary.BreakRotator` (`SceneComponent.K2_GetComponentRotation` _sphere_2)))
  (if (`self.Detonated`)
    (if (not (`self.Finished`))
      (`SceneComponent.K2_AddRelativeRotation` _sphere (struct :`Yaw` 50.0) false false)
      (`SceneComponent.K2_AddWorldOffset` _sphere (`KismetMathLibrary.MakeVector` (`KismetMathLibrary.RandomFloatInRange` -1.0 1.0) (`KismetMathLibrary.RandomFloatInRange` -1.0 1.0) (`KismetMathLibrary.RandomFloatInRange` -0.25 0.25)) true false)
      (bind _returnvalue (`|SpawnActorFromClass` "/Game/Blueprints/Projectiles/Projectile_FerroHealSpray.Projectile_FerroHealSpray_C" (`KismetMathLibrary.MakeTransform` (`SceneComponent.K2_GetComponentLocation` _sphere_2) (`KismetMathLibrary.MakeRotator` 0.0 (`KismetMathLibrary.RandomFloatInRange` -60.0 30.0) _returnvalue_yaw)) "AlwaysSpawn" "OverrideRootScale" null (`self.Parent`) 0.0 0.0 0.0 0.0 0.0 0.0 0.0 "NewEnumerator0" false true false (`self.VFXData`) null))
      (set `Actor.CustomTimeDilation` 0.5 _returnvalue))))

(event `self.ReceiveHit`
  (params (MyComp :type "PrimitiveComponent Object Reference") (Other :type "Actor Object Reference") (OtherComp :type "PrimitiveComponent Object Reference") (bSelfMoved :type Boolean) (HitLocation :type "Vector Structure") (HitNormal :type "Vector Structure") (NormalImpulse :type "Vector Structure") (Hit :type "HitResult Structure (by ref)"))
  (bind (_returnvalue_x _returnvalue_y _returnvalue_z) (`KismetMathLibrary.BreakVector` (`self.K2_GetActorLocation`)))
  (bind _visual (`self.Visual`))
  (bind (_returnvalue_roll _returnvalue_pitch _returnvalue_yaw) (`KismetMathLibrary.BreakRotator` (`SceneComponent.K2_GetComponentRotation` _visual)))
  (`parent.ReceiveHit` MyComp Other OtherComp bSelfMoved HitLocation HitNormal NormalImpulse Hit)
  (if (not (`self.Armed`))
    (set `self.Finished` true)
    (set `self.Armed` true)
    (`KismetSystemLibrary.Delay` 1.5)
    (`PrimitiveComponent.SetMaterial` (`self.Visual`) 3 "/Game/Materials/BasicUnlit_Container_1.BasicUnlit_Container_1")
    (set `ProjectileMovementComponent.ProjectileGravityScale` 0.0 (`self.ProjectileMovement`))
    (set `self.Detonated` true)
    (`SceneComponent.K2_SetWorldRotation` _visual (`KismetMathLibrary.MakeRotator` 0.0 0.0 _returnvalue_yaw) false false)
    (set `self.Return Value Z` _returnvalue_z)
    (bind (_direction _newtrack_0 _newtrack_1) (`Timeline|Timeline_0`)
      (:`Update`
        (`self.K2_SetActorLocation` (`KismetMathLibrary.MakeVector` _returnvalue_x _returnvalue_y (+ (`self.Return Value Z`) (`KismetMathLibrary.Lerp` 0.0 175.0 _newtrack_1))) true))
      (:`Finished`
        (set `self.Finished` false)
        (`KismetSystemLibrary.Delay` 4.0)
        (set `self.Finished` true)
        (`KismetSystemLibrary.Delay` 1.0)
        (`PrimitiveComponent.SetMaterial` (`self.Visual`) 3 "/Game/Materials/BasicUnlit_Container_2.BasicUnlit_Container_2")
        (set `ProjectileMovementComponent.ProjectileGravityScale` 1.0 (`self.ProjectileMovement`))
        (`PrimitiveComponent.SetSimulatePhysics` (`self.Sphere`) true)))))

(fn `UserConstructionScript`
  (`parent.UserConstructionScript`))