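; Concussion grenade throwable that arms on first impact and explodes after a short fuse, swapping visual materials as a countdown.
; Detonation plays VFX and runs a sphere trace, affecting each actor once.
; Enemies (capsule hits only) and players take damage, stagger and knockback, with player damage scaled by self-damage; objects take damage and other throwables are triggered to detonate.
; It then shakes the screen through its parent character and destroys itself.
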(event `self.ReceiveHit`
  (params (MyComp :type "PrimitiveComponent Object Reference") (Other :type "Actor Object Reference") (OtherComp :type "PrimitiveComponent Object Reference") (bSelfMoved :type Boolean) (HitLocation :type "Vector Structure") (HitNormal :type "Vector Structure") (NormalImpulse :type "Vector Structure") (Hit :type "HitResult Structure (by ref)"))
  (bind _returnvalue (`self.K2_GetActorLocation`))
  (bind _visual (`self.Visual`))
  (bind _visual_2 (`self.Visual`))
  (`parent.ReceiveHit` MyComp Other OtherComp bSelfMoved HitLocation HitNormal NormalImpulse Hit)
  (if (not (`self.Armed`))
    (set `self.Armed` true)
    (`KismetSystemLibrary.Delay` 1.0)
    (`PrimitiveComponent.SetMaterial` _visual_2 2 "/Game/Materials/BasicUnlit_Master_Inst6.BasicUnlit_Master_Inst6")
    (`PrimitiveComponent.SetMaterial` _visual_2 3 "/Game/Materials/BasicUnlit_Master_Inst6.BasicUnlit_Master_Inst6")
    (`KismetSystemLibrary.Delay` 1.0)
    (`PrimitiveComponent.SetMaterial` _visual 0 "/Game/Materials/BasicUnlit_Master_Inst7.BasicUnlit_Master_Inst7")
    (`PrimitiveComponent.SetMaterial` _visual 1 "/Game/Materials/BasicUnlit_Master_Inst7.BasicUnlit_Master_Inst7")
    (`PrimitiveComponent.SetMaterial` _visual 2 "/Game/Materials/BasicUnlit_Master_Inst7.BasicUnlit_Master_Inst7")
    (`PrimitiveComponent.SetMaterial` _visual 3 "/Game/Materials/BasicUnlit_Master_Inst7.BasicUnlit_Master_Inst7")
    (`KismetSystemLibrary.Delay` 0.1)
    (`self.DetonationVFX` (`self.K2_GetActorLocation`))
    (bind _outhits (`KismetSystemLibrary.SphereTraceMulti` :`Start` _returnvalue :`End` _returnvalue :`Radius` (`self.DetonationRadius`) :`TraceChannel` "TraceTypeQuery1" :`DrawTime` 0.2))
    (for _array_element _outhits
      (bind (_bblockinghit _binitialoverlap _time _distance _location _impactpoint _normal _impactnormal _physmat _hitactor _hitcomponent) (`GameplayStatics.BreakHitResult` _array_element))
      (if _bblockinghit
        (if (not (`KismetArrayLibrary.Array_Contains` (`self.Hit Actors`) _hitactor))
          (bind _asenemy_entry_master (cast `/Game/Blueprints/Enemies/EnemyEntry_Master` _hitactor)
            (:`then`
              (if (== (`Character.CapsuleComponent` _asenemy_entry_master) _hitcomponent)
                (`/Game/Blueprints/Enemies/EnemyEntry_Master.TakeDamage_Enemy` _asenemy_entry_master (`self.BaseDamage`) (`self.DestructionDamage`) self (`self.Stagger Duration`) (`self.Knockback Amount`) (`self.NoStagger/Knockback`))
                (`KismetArrayLibrary.Array_Add` (`self.Hit Actors`) _hitactor :!label _label)
                (`/Game/Blueprints/BP_TopDownCharacter.ImpactVFX` (`self.PlayerRef`) (`self.K2_GetActorLocation` _hitactor) (`KismetMathLibrary.Conv_VectorToRotator` _impactnormal) false (`self.VFXData`) (`self.BaseDamage`))))
            (:`CastFailed`
              (bind _asobject_entry_master (cast `/Game/Blueprints/Objects/ObjectEntry_Master` _hitactor)
                (:`then`
                  (`/Game/Blueprints/Objects/ObjectEntry_Master.TakeDamage_Object` _asobject_entry_master (`self.BaseDamage`) (`self.DestructionDamage`))
                  (goto _label))
                (:`CastFailed`
                  (bind _asbp_top_down_character (cast `/Game/Blueprints/BP_TopDownCharacter` _hitactor)
                    (:`then`
                      (`/Game/Blueprints/BP_TopDownCharacter.TakeDamage` _asbp_top_down_character (* (`self.BaseDamage`) (`/Game/Blueprints/BP_TopDownCharacter.SelfDamageAmount` _asbp_top_down_character)) (`self.DestructionDamage`) (`self.Stagger Duration`) (`self.Knockback Amount`) self)
                      (goto _label))
                    (:`CastFailed`
                      (bind _asprojectile_throwable_master (cast `/Game/Blueprints/Projectiles/Projectile_Throwable_master` _hitactor))
                      (set `self.HitTarget` _asprojectile_throwable_master)
                      (`self.TriggerDetonation` _asprojectile_throwable_master)
                      (goto _label))))))))))
    (bind _asbp_top_down_character_2 (cast `/Game/Blueprints/BP_TopDownCharacter` (`self.Parent`))
      (:`then`
        (`/Game/Blueprints/BP_TopDownCharacter.ScreenShake` _asbp_top_down_character_2 2 "NewEnumerator0" 1000.0 (`self.K2_GetActorLocation`)))
      (:`CastFailed`
        _))
    (`self.K2_DestroyActor`)))

(fn `UserConstructionScript`
  (`parent.UserConstructionScript`))