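; Throwable trip mine projectile that sticks out a laser tripwire from the surface it hits and explodes when triggered.
; On first hit it aligns to the surface, sizes beam and trigger box by line trace, then arms after a delay and checks for characters already inside.
; Player, enemy capsule or projectile overlaps, or external detonation, cause a delayed sphere-sweep blast along its facing, damaging characters and objects and chain-detonating other throwables.
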(event `self.TriggerBox.OnComponentBeginOverlap`
  (params (OverlappedComponent :type "PrimitiveComponent Object Reference") (OtherActor :type "Actor Object Reference") (OtherComp :type "PrimitiveComponent Object Reference") (OtherBodyIndex :type Integer) (bFromSweep :type Boolean) (SweepResult :type "HitResult Structure (by ref)"))
  (cast `/Game/Blueprints/BP_TopDownCharacter` OtherActor
    (:`then`
      (if (`self.Armed`) :!label _label
        (set `self.HitTarget` OtherActor)
        (`self.Explode`)))
    (:`CastFailed`
      (bind _asenemy_entry_master (cast `/Game/Blueprints/Enemies/EnemyEntry_Master` OtherActor)
        (:`then`
          (if (== (`Character.CapsuleComponent` _asenemy_entry_master) OtherComp)
            (goto _label)))
        (:`CastFailed`
          (cast `/Game/Blueprints/Projectiles/Projectile_Master` OtherActor)
          (goto _label))))))

(event `self.TriggerDetonation`
  (`self.Explode`))

(event `Explode`
  (bind _visual (`self.Visual`))
  (bind _returnvalue (`SceneComponent.GetUpVector` _visual))
  (bind _returnvalue_2 (`SceneComponent.K2_GetComponentLocation` _visual))
  (if (not (`self.Detonated`))
    (set `self.Detonated` true)
    (`PrimitiveComponent.SetMaterial` (`self.w`) 0 "/Game/Materials/BasicUnlit_Master_Inst8.BasicUnlit_Master_Inst8")
    (`KismetSystemLibrary.Delay` 0.4)
    (`self.DetonationVFX` (`self.K2_GetActorLocation`))
    (bind _outhits (`KismetSystemLibrary.SphereTraceMultiForObjects` :`Start` (+ _returnvalue_2 (* _returnvalue 25.0)) :`End` (+ _returnvalue_2 (* _returnvalue 350.0)) :`Radius` 75.0 :`ObjectTypes` (`|MakeArray` "ObjectTypeQuery7" "ObjectTypeQuery12" "ObjectTypeQuery8" "ObjectTypeQuery11" :!type "EObjectTypeQuery Enum") :`DrawTime` 0.2))
    (for _array_element _outhits
      (bind (_bblockinghit _binitialoverlap _time _distance _location _impactpoint _normal _impactnormal _physmat _hitactor _hitcomponent) (`GameplayStatics.BreakHitResult` _array_element))
      (if _bblockinghit
        (if (not (`KismetArrayLibrary.Array_Contains` (`self.Hit Actors`) _hitactor))
          (bind _asenemy_entry_master (cast `/Game/Blueprints/Enemies/EnemyEntry_Master` _hitactor)
            (:`then`
              (if (== (`Character.CapsuleComponent` _asenemy_entry_master) _hitcomponent)
                (`/Game/Blueprints/Enemies/EnemyEntry_Master.TakeDamage_Enemy` _asenemy_entry_master (`self.BaseDamage`) (`self.DestructionDamage`) self (`self.Stagger Duration`) (`self.Knockback Amount`) (`self.NoStagger/Knockback`))
                (`KismetArrayLibrary.Array_Add` (`self.Hit Actors`) _hitactor :!label _label_2)
                (`/Game/Blueprints/BP_TopDownCharacter.ImpactVFX` (`self.PlayerRef`) (`self.K2_GetActorLocation` _hitactor) (`KismetMathLibrary.Conv_VectorToRotator` _impactnormal) false (`self.VFXData`) (`self.BaseDamage`))))
            (:`CastFailed`
              (bind _asobject_entry_master (cast `/Game/Blueprints/Objects/ObjectEntry_Master` _hitactor)
                (:`then`
                  (`/Game/Blueprints/Objects/ObjectEntry_Master.TakeDamage_Object` _asobject_entry_master (`self.BaseDamage`) (`self.DestructionDamage`))
                  (goto _label_2))
                (:`CastFailed`
                  (bind _asbp_top_down_character (cast `/Game/Blueprints/BP_TopDownCharacter` _hitactor)
                    (:`then`
                      (`/Game/Blueprints/BP_TopDownCharacter.TakeDamage` _asbp_top_down_character (* (`self.BaseDamage`) (`/Game/Blueprints/BP_TopDownCharacter.SelfDamageAmount` _asbp_top_down_character)) (`self.DestructionDamage`) (`self.Stagger Duration`) (`self.Knockback Amount`) self false)
                      (goto _label_2))
                    (:`CastFailed`
                      (bind _asprojectile_throwable_master (cast `/Game/Blueprints/Projectiles/Projectile_Throwable_master` _hitactor))
                      (set `self.HitTarget` _asprojectile_throwable_master)
                      (`self.TriggerDetonation` _asprojectile_throwable_master)
                      (goto _label_2))))))))))
    (`SceneComponent.SetHiddenInGame` (`self.Sphere`) true true)
    (bind _asbp_top_down_character_2 (cast `/Game/Blueprints/BP_TopDownCharacter` (`self.Parent`))
      (:`then`
        (`/Game/Blueprints/BP_TopDownCharacter.ScreenShake` _asbp_top_down_character_2 2 "NewEnumerator0" 1000.0 (`self.K2_GetActorLocation`)))
      (:`CastFailed`
        _))
    (`KismetSystemLibrary.Delay` 1.0)
    (`self.K2_DestroyActor`)))

(event `self.ReceiveBeginPlay`
  (`parent.ReceiveBeginPlay`))

(event `self.ReceiveHit`
  (params (MyComp :type "PrimitiveComponent Object Reference") (Other :type "Actor Object Reference") (OtherComp :type "PrimitiveComponent Object Reference") (bSelfMoved :type Boolean) (HitLocation :type "Vector Structure") (HitNormal :type "Vector Structure") (NormalImpulse :type "Vector Structure") (Hit :type "HitResult Structure (by ref)"))
  (bind _visual (`self.Visual`))
  (bind _triggerbox (`self.TriggerBox`))
  (bind _beam (`self.Beam`))
  (bind _triggerbox_2 (`self.TriggerBox`))
  (bind _triggerbox_3 (`self.TriggerBox`))
  (bind _triggerbox_4 (`self.TriggerBox`))
  (bind _triggerbox_5 (`self.TriggerBox`))
  (bind _triggerbox_6 (`self.TriggerBox`))
  (bind _returnvalue (`SceneComponent.K2_GetComponentLocation` _triggerbox_4))
  (bind _returnvalue_2 (`SceneComponent.K2_GetComponentLocation` _triggerbox_6))
  (`parent.ReceiveHit` MyComp Other OtherComp bSelfMoved HitLocation HitNormal NormalImpulse Hit)
  (`/Engine/EditorBlueprintResources/StandardMacros.DoOnce` false
    (:`Completed`
      (`SceneComponent.K2_SetRelativeRotation` :`self` _visual)
      (`SceneComponent.K2_SetWorldRotation` _visual (`KismetMathLibrary.MakeRotator` (.roll (`KismetMathLibrary.Conv_VectorToRotator` HitNormal)) (+ (.pitch (`KismetMathLibrary.Conv_VectorToRotator` HitNormal)) -90.0) (.yaw (`KismetMathLibrary.Conv_VectorToRotator` HitNormal))) false false)
      (`SceneComponent.K2_SetWorldRotation` (`self.TriggerBox`) (`KismetMathLibrary.MakeRotator` (.roll (`KismetMathLibrary.Conv_VectorToRotator` HitNormal)) (+ (.pitch (`KismetMathLibrary.Conv_VectorToRotator` HitNormal)) -90.0) (.yaw (`KismetMathLibrary.Conv_VectorToRotator` HitNormal))) false false)
      (`SceneComponent.K2_SetWorldRotation` (`self.Beam`) (`KismetMathLibrary.MakeRotator` (.roll (`KismetMathLibrary.Conv_VectorToRotator` HitNormal)) (+ (.pitch (`KismetMathLibrary.Conv_VectorToRotator` HitNormal)) -90.0) (.yaw (`KismetMathLibrary.Conv_VectorToRotator` HitNormal))) false false)
      (bind _outhit (`KismetSystemLibrary.LineTraceSingleForObjects` _returnvalue (+ _returnvalue (* (`SceneComponent.GetUpVector` _triggerbox_4) 1000000.0)) (`|MakeArray` "ObjectTypeQuery1" "ObjectTypeQuery2" "ObjectTypeQuery8" :!type "EObjectTypeQuery Enum")))
      (bind (_bblockinghit _binitialoverlap _time _distance) (`GameplayStatics.BreakHitResult` _outhit))
      (if _bblockinghit
        (`SceneComponent.SetRelativeScale3D` _beam (`KismetMathLibrary.MakeVector` 0.005 0.005 (* _distance 0.01)))
        (bind _returnvalue_3 (* _distance 0.5))
        (`BoxComponent.SetBoxExtent` _triggerbox_2 (`KismetMathLibrary.MakeVector` 5.0 5.0 _returnvalue_3) true)
        (`SceneComponent.K2_SetWorldLocation` _triggerbox_3 (+ (`SceneComponent.K2_GetComponentLocation` _triggerbox_5) (* (`SceneComponent.GetUpVector` _triggerbox_5) _returnvalue_3)) false false)
        (else
          (`SceneComponent.SetRelativeScale3D` _beam (0.005 0.005 10.0))
          (`BoxComponent.SetBoxExtent` _triggerbox_2 (5.0 5.0 500.0) true)
          (`SceneComponent.K2_SetWorldLocation` _triggerbox_3 (+ (`SceneComponent.K2_GetComponentLocation` _triggerbox) (* (`SceneComponent.GetUpVector` _triggerbox) 50.0)) false false)))
      (`KismetSystemLibrary.Delay` 1.0)
      (`PrimitiveComponent.SetMaterial` (`self.w`) 0 "/Game/Materials/BasicUnlit_Master_Inst2.BasicUnlit_Master_Inst2")
      (set `self.Armed` true)
      (`SceneComponent.SetVisibility` (`self.Beam`) true false)
      (bind _outhits (`KismetSystemLibrary.BoxTraceMulti` :`Start` _returnvalue_2 :`End` _returnvalue_2 :`HalfSize` (`BoxComponent.GetScaledBoxExtent` _triggerbox_6) :`Orientation` (`SceneComponent.K2_GetComponentRotation` _triggerbox_6) :`TraceChannel` "TraceTypeQuery1" :`DrawTime` 0.2))
      (for _array_element _outhits
        (bind (_bblockinghit_2 _binitialoverlap_2 _time_2 _distance_2 _location _impactpoint _normal _impactnormal _physmat _hitactor _hitcomponent) (`GameplayStatics.BreakHitResult` _array_element))
        (bind _asbp_top_down_character (cast `/Game/Blueprints/BP_TopDownCharacter` _hitactor)
          (:`then`
            (set `self.HitTarget` _asbp_top_down_character)
            (`self.Explode` :!label _label_3))
          (:`CastFailed`
            (bind _asenemy_entry_master (cast `/Game/Blueprints/Enemies/EnemyEntry_Master` _hitactor)
              (:`then`
                (if (== (`Character.CapsuleComponent` _asenemy_entry_master) _hitcomponent)
                  (set `self.HitTarget` _asenemy_entry_master)
                  (goto _label_3)
                  (else
                    _)))
              (:`CastFailed`
                _))
            (set `self.HitTarget` null)))))))

(fn `UserConstructionScript`
  (`parent.UserConstructionScript`))