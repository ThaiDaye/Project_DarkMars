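; Master Blueprint for throwable projectiles that provides in-flight spin and surface-aligned detonation effects, with TriggerDetonation left empty.
; From BeginPlay, a delay loop rotates the visual by ThrowRotation, if non-zero, until a hit closes its gate.
; DetonationVFX shakes the player's screen, then traces short rays along the six local axes.
; The first blocking surface orients debris, dust and hit effects and receives an attached decal effect.
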(event `DetonationVFX`
  (params (Loc :type "Vector Structure"))
  (`/Game/Blueprints/BP_TopDownCharacter.ScreenShake` (`self.PlayerRef`) 2 "NewEnumerator0" 2000.0 Loc)
  (for _index (range 6)
    (if (not (`self.Surfacehit`))
      (bind _outhit (`KismetSystemLibrary.LineTraceSingleForObjects` Loc (+ (+ (* (select `int` (select `int` _index :`0` 0 :`1` 2 :`2` 1 :`3` 1 :`4` 1 :`5` 1) :`0` -100.0 :`1` 0.0 :`2` 100.0) (`self.GetActorUpVector`)) (* (select `int` (select `int` _index :`0` 1 :`1` 1 :`2` 0 :`3` 2 :`4` 1 :`5` 1) :`0` -100.0 :`1` 0.0 :`2` 100.0) (`self.GetActorRightVector`)) (* (select `int` (select `int` _index :`0` 1 :`1` 1 :`2` 1 :`3` 1 :`4` 0 :`5` 2) :`0` -100.0 :`1` 0.0 :`2` 100.0) (`self.GetActorForwardVector`))) Loc) (`|MakeArray` "ObjectTypeQuery1" "ObjectTypeQuery2" "ObjectTypeQuery8" :!type "EObjectTypeQuery Enum")))
      (bind (_bblockinghit _binitialoverlap _time _distance _location _impactpoint _normal _impactnormal _physmat _hitactor _hitcomponent) (`GameplayStatics.BreakHitResult` _outhit))
      (if _bblockinghit
        (set `self.Surfacehit` true)
        (bind _returnvalue (`KismetMathLibrary.MakeRotator` (.roll (`KismetMathLibrary.Conv_VectorToRotator` _impactnormal)) (+ (.pitch (`KismetMathLibrary.Conv_VectorToRotator` _impactnormal)) -90.0) (.yaw (`KismetMathLibrary.Conv_VectorToRotator` _impactnormal))))
        (`NiagaraFunctionLibrary.SpawnSystemAtLocation` (`self.ThrowDebrisVFX`) Loc _returnvalue)
        (`NiagaraFunctionLibrary.SpawnSystemAttached` (`self.ThrowDecalVFX`) _hitcomponent "None" _impactpoint _returnvalue "KeepWorldPosition" true)
        (`NiagaraFunctionLibrary.SpawnSystemAtLocation` (`self.ThrowDustVFX`) Loc _returnvalue)
        (`NiagaraFunctionLibrary.SpawnSystemAtLocation` (`self.ThrowHitEffectVFX`) Loc _returnvalue)))))

(event `TriggerDetonation`)

(event `self.ReceiveBeginPlay`
  (`parent.ReceiveBeginPlay`)
  (if (not (== (`self.ThrowRotation`) (struct)))
    (`|ExecutionSequence` :!label _label
      (:`then_0`
        (`/Engine/EditorBlueprintResources/StandardMacros.Gate` false :!label _label_2
          (:`Exit`
            (`SceneComponent.K2_AddLocalRotation` (`self.Visual`) (`self.ThrowRotation`) false false))))
      (:`then_1`
        (`KismetSystemLibrary.Delay` 0.01)
        (goto _label)))))

(event `self.ReceiveHit`
  (params (MyComp :type "PrimitiveComponent Object Reference") (Other :type "Actor Object Reference") (OtherComp :type "PrimitiveComponent Object Reference") (bSelfMoved :type Boolean) (HitLocation :type "Vector Structure") (HitNormal :type "Vector Structure") (NormalImpulse :type "Vector Structure") (Hit :type "HitResult Structure (by ref)"))
  (`parent.ReceiveHit` MyComp Other OtherComp bSelfMoved HitLocation HitNormal NormalImpulse Hit)
  (goto _label_2 :!via `Close`))

(fn `UserConstructionScript`
  (`parent.UserConstructionScript`))