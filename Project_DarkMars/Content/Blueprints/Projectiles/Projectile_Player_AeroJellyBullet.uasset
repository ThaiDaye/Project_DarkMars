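; Player AeroJelly bullet projectile that deals area damage when it is destroyed.
; On Destroyed it runs a small multi-sphere trace at its location against two object types.
; Hit ObjectEntry_Master actors take object damage, while EnemyEntry_Master actors take damage with stagger and knockback, only when the hit component is their capsule.
; BeginPlay and construction just defer to the parent projectile.
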(event `self.ReceiveBeginPlay`
  (`parent.ReceiveBeginPlay`))

(event `self.ReceiveDestroyed`
  (bind _returnvalue (`self.K2_GetActorLocation`))
  (bind _destructiondamage (`self.DestructionDamage`))
  (bind _basedamage (`self.BaseDamage`))
  (`parent.ReceiveDestroyed`)
  (bind _outhits (`KismetSystemLibrary.SphereTraceMultiForObjects` :`Start` _returnvalue :`End` _returnvalue :`Radius` 50.0 :`ObjectTypes` (`|MakeArray` "ObjectTypeQuery8" "ObjectTypeQuery12" :!type "EObjectTypeQuery Enum") :`TraceColor` (struct :`R` 1.0 :`G` 0.651406 :`A` 1.0) :`DrawTime` 0.08))
  (for _array_element _outhits
    (bind (_bblockinghit _binitialoverlap _time _distance _location _impactpoint _normal _impactnormal _physmat _hitactor _hitcomponent) (`GameplayStatics.BreakHitResult` _array_element))
    (if _bblockinghit
      (bind _asobject_entry_master (cast `/Game/Blueprints/Objects/ObjectEntry_Master` _hitactor)
        (:`then`
          (`/Game/Blueprints/Objects/ObjectEntry_Master.TakeDamage_Object` _asobject_entry_master _basedamage _destructiondamage))
        (:`CastFailed`
          (bind _asenemy_entry_master (cast `/Game/Blueprints/Enemies/EnemyEntry_Master` _hitactor))
          (if (== _hitcomponent (`Character.CapsuleComponent` _asenemy_entry_master))
            (`/Game/Blueprints/Enemies/EnemyEntry_Master.TakeDamage_Enemy` _asenemy_entry_master _basedamage _destructiondamage (`self.Parent`) (`self.Stagger Duration`) (`self.Knockback Amount`) (`self.NoStagger/Knockback`))))))))

(fn `UserConstructionScript`
  (`parent.UserConstructionScript`))