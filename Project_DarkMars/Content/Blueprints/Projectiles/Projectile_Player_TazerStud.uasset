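; Player tazer stud projectile that stays tethered to the shooter by a cable and repeatedly shocks the enemy it hits.
; On BeginPlay it attaches the cable end to the Muzzle socket of the owning character's equipment, then starts two endless delay loops.
; A fast loop randomizes the cable force to fake electric jitter, while a slower one applies damage, stagger and knockback to HitTarget.
; Hit handling is left to the parent class.
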(event `self.ReceiveBeginPlay`
  (bind _returnvalue (`KismetMathLibrary.RandomBool`))
  (`parent.ReceiveBeginPlay`)
  (bind _asbp_top_down_character (cast `/Game/Blueprints/BP_TopDownCharacter` (`self.Parent`)))
  (`CableComponent.SetAttachEndToComponent` (`self.Cable`) (`/Game/Blueprints/BP_TopDownCharacter.EquipmentVisual` _asbp_top_down_character) "Muzzle")
  (`|ExecutionSequence`
    (:`then_0`
      (`|ExecutionSequence` :!label _label
        (:`then_0`
          (set `CableComponent.CableForce` (`KismetMathLibrary.MakeVector` (select `bool` _returnvalue :`false` -10000.0 :`true` 10000.0) (select `bool` _returnvalue :`false` -10000.0 :`true` 10000.0) (+ (select `bool` _returnvalue :`false` -5000.0 :`true` 5000.0) (`KismetMathLibrary.RandomFloatInRange` 5000.0 20000.0))) (`self.Cable`)))
        (:`then_1`
          (`KismetSystemLibrary.Delay` 0.1)
          (goto _label))))
    (:`then_1`
      (`|ExecutionSequence` :!label _label_2
        (:`then_0`
          (bind _asenemy_entry_master (cast `/Game/Blueprints/Enemies/EnemyEntry_Master` (`self.HitTarget`)))
          (`/Game/Blueprints/Enemies/EnemyEntry_Master.TakeDamage_Enemy` _asenemy_entry_master (`self.BaseDamage`) (`self.DestructionDamage`) (`self.Parent`) (`self.Stagger Duration`) (`self.Knockback Amount`) false))
        (:`then_1`
          (`KismetSystemLibrary.Delay` 2.0)
          (goto _label_2))))))

(event `self.ReceiveHit`
  (params (MyComp :type "PrimitiveComponent Object Reference") (Other :type "Actor Object Reference") (OtherComp :type "PrimitiveComponent Object Reference") (bSelfMoved :type Boolean) (HitLocation :type "Vector Structure") (HitNormal :type "Vector Structure") (NormalImpulse :type "Vector Structure") (Hit :type "HitResult Structure (by ref)"))
  (`parent.ReceiveHit` MyComp Other OtherComp bSelfMoved HitLocation HitNormal NormalImpulse Hit))

(fn `UserConstructionScript`
  (`parent.UserConstructionScript`))