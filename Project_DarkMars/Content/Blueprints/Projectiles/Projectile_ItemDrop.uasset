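; Projectile actor for a dropped item that flies out and becomes an item pickup where it lands.
; Component activation randomly scales the start velocity and feeds it to ProjectileMovement, while BeginPlay randomizes the visual's rotation and ignores Parent for collision.
; The first hit spawns ObjectEntry_ItemPickup with ItemID and Stack at a nearby random navigable point, falling back to the hit location.
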(event `self.ProjectileMovement.OnComponentActivated`
  (params (Component :type "ActorComponent Object Reference") (bReset :type Boolean))
  (bind _projectilemovement (`self.ProjectileMovement`))
  (bind _startvelocity (`self.StartVelocity`))
  (set `self.StartVelocity` (* _startvelocity (`KismetMathLibrary.RandomFloatInRange` 0.5 1.5)))
  (bind _output_get (set `ProjectileMovementComponent.InitialSpeed` (.x _startvelocity) _projectilemovement))
  (set `ProjectileMovementComponent.MaxSpeed` _output_get _projectilemovement)
  (set `MovementComponent.Velocity` _startvelocity (`self.ProjectileMovement`)))

(event `self.ReceiveBeginPlay`
  (`parent.ReceiveBeginPlay`)
  (`PrimitiveComponent.IgnoreActorWhenMoving` (`self.Sphere`) (`self.Parent`) true)
  (`SceneComponent.K2_SetRelativeRotation` (`self.Visual`) (`KismetMathLibrary.RandomRotator` true) false false))

(event `self.ReceiveHit`
  (params (MyComp :type "PrimitiveComponent Object Reference") (Other :type "Actor Object Reference") (OtherComp :type "PrimitiveComponent Object Reference") (bSelfMoved :type Boolean) (HitLocation :type "Vector Structure") (HitNormal :type "Vector Structure") (NormalImpulse :type "Vector Structure") (Hit :type "HitResult Structure (by ref)"))
  (`parent.ReceiveHit` MyComp Other OtherComp bSelfMoved HitLocation HitNormal NormalImpulse Hit)
  (`/Engine/EditorBlueprintResources/StandardMacros.DoOnce` false
    (:`Completed`
      (bind (_randomlocation _returnvalue) (`NavigationSystemV1.K2_GetRandomLocationInNavigableRadius` (`KismetMathLibrary.MakeVector` (.x HitLocation) (.y HitLocation)) 25.0 null null))
      (`|SpawnActorFromClass` "/Game/Blueprints/Objects/ObjectEntry_ItemPickup.ObjectEntry_ItemPickup_C" (`KismetMathLibrary.MakeTransform` (select `bool` _returnvalue :`false` HitLocation :`true` _randomlocation) (`KismetMathLibrary.MakeRotator` 0.0 0.0 (`KismetMathLibrary.RandomFloatInRange` 0.0 360.0))) "Undefined" "OverrideRootScale" null (`self.Item ID`) -1 (`self.Stack`) 0 "None" "NewEnumerator0" null))))

(fn `UserConstructionScript`
  (`parent.UserConstructionScript`))