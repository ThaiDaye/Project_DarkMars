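; Base projectile actor that damages objects and enemies or detonates throwable projectiles on impact.
; On BeginPlay it applies any max-charge damage bonus, then activates ProjectileMovement, which launches it at StartVelocity.
; Hits ignore Parent, draw a debug sphere trace and affect only the first valid target, unless impact damage is disabled.
; It can attach to struck objects or enemy meshes with collision disabled, then destroys itself after a delay.
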(event `self.ProjectileMovement.OnComponentActivated`
  (params (Component :type "ActorComponent Object Reference") (bReset :type Boolean))
  (bind _projectilemovement (`self.ProjectileMovement`))
  (bind _startvelocity (`self.StartVelocity`))
  (bind _output_get (set `ProjectileMovementComponent.InitialSpeed` (.x _startvelocity) _projectilemovement))
  (set `ProjectileMovementComponent.MaxSpeed` _output_get _projectilemovement)
  (set `MovementComponent.Velocity` _startvelocity (`self.ProjectileMovement`)))

(event `self.ReceiveBeginPlay`
  (bind _basedamage (`self.BaseDamage`))
  (set `self.BaseDamage` (select `bool` (`self.ChargeIsMax`) :`false` _basedamage :`true` (select `/Game/Blueprints/Data/RangeChargeMaxAction_Type` (`self.ChargeActionType`) :`NewEnumerator0` _basedamage :`NewEnumerator1` (* _basedamage 1.5))))
  (`ActorComponent.Activate` (`self.ProjectileMovement`) false))

(event `self.ReceiveHit`
  (params (MyComp :type "PrimitiveComponent Object Reference") (Other :type "Actor Object Reference") (OtherComp :type "PrimitiveComponent Object Reference") (bSelfMoved :type Boolean) (HitLocation :type "Vector Structure") (HitNormal :type "Vector Structure") (NormalImpulse :type "Vector Structure") (Hit :type "HitResult Structure (by ref)"))
  (bind (_bblockinghit _binitialoverlap _time _distance _location _impactpoint _normal _impactnormal _physmat _hitactor _hitcomponent) (`GameplayStatics.BreakHitResult` Hit))
  (bind _hittarget (`self.HitTarget`))
  (bind _visual (`self.Visual`))
  (if (not (== Other (`self.Parent`)))
    (`KismetSystemLibrary.SphereTraceSingle` :`Start` HitLocation :`End` HitLocation :`Radius` 15.0 :`TraceChannel` "TraceTypeQuery1" :`DrawDebugType` "ForDuration" :`TraceColor` (struct :`R` 1.0 :`G` 0.653453 :`A` 1.0) :`TraceHitColor` (struct :`R` 1.0 :`G` 0.653453 :`A` 1.0) :`DrawTime` 0.2)
    (`/Engine/EditorBlueprintResources/StandardMacros.IsValid` (`self.HitTarget`)
      (:`Is Valid`
        _)
      (:`Is Not Valid`
        (if _bblockinghit
          (bind _asobject_entry_master (cast `/Game/Blueprints/Objects/ObjectEntry_Master` _hitactor)
            (:`then`
              (set `self.HitTarget` _asobject_entry_master)
              (if (not (`self.NoDamageOnImpact`))
                (`/Game/Blueprints/Objects/ObjectEntry_Master.TakeDamage_Object` _asobject_entry_master (`self.BaseDamage`) (`self.DestructionDamage`))))
            (:`CastFailed`
              (bind _asenemy_entry_master (cast `/Game/Blueprints/Enemies/EnemyEntry_Master` _hitactor)
                (:`then`
                  (set `self.HitTarget` _asenemy_entry_master)
                  (if (not (`self.NoDamageOnImpact`))
                    (`/Game/Blueprints/Enemies/EnemyEntry_Master.TakeDamage_Enemy` _asenemy_entry_master (`self.BaseDamage`) (`self.DestructionDamage`) (`self.Parent`) (`self.Stagger Duration`) (`self.Knockback Amount`) (`self.NoStagger/Knockback`))))
                (:`CastFailed`
                  (bind _asprojectile_throwable_master (cast `/Game/Blueprints/Projectiles/Projectile_Throwable_master` _hitactor)
                    (:`then`
                      (set `self.HitTarget` _asprojectile_throwable_master)
                      (if (not (`self.NoDamageOnImpact`))
                        (`/Game/Blueprints/Projectiles/Projectile_Throwable_master.TriggerDetonation` _asprojectile_throwable_master)))
                    (:`CastFailed`
                      _)))))))))
    (if (`self.AttachOnDestroy`)
      (`/Engine/EditorBlueprintResources/StandardMacros.IsValid` _hittarget
        (:`Is Valid`
          (cast `/Game/Blueprints/Objects/ObjectEntry_Master` _hittarget
            (:`then`
              (`self.K2_AttachToComponent` _hitcomponent "None" "KeepWorld" "KeepWorld" "KeepWorld")
              (`PrimitiveComponent.SetCollisionEnabled` (`self.Sphere`) "NoCollision" :!label _label)
              (`/Engine/EditorBlueprintResources/StandardMacros.IsValid` _visual
                (:`Is Valid`
                  (`PrimitiveComponent.SetCollisionEnabled` _visual "NoCollision"))
                (:`Is Not Valid`
                  _)))
            (:`CastFailed`
              (bind _asenemy_entry_master_2 (cast `/Game/Blueprints/Enemies/EnemyEntry_Master` _hittarget)
                (:`then`
                  (`self.K2_AttachToComponent` (`Character.Mesh` _asenemy_entry_master_2) "None" "KeepWorld" "KeepWorld" "KeepWorld")
                  (goto _label))
                (:`CastFailed`
                  _)))))
        (:`Is Not Valid`
          _)))
    (`KismetSystemLibrary.Delay` (`self.DestroyDelay`))
    (`self.K2_DestroyActor`)))

(fn `UserConstructionScript`)