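; Throwable device jammer projectile that disrupts whatever it first hits, aligning its visual to the surface normal.
; After a short delay it unlocks and damages containers, interrupts fuse slot power, or deals full-health damage to CCTV cameras.
; Enemies take repeated damage and stagger through a custom delayed for-loop macro.
; An indicator material swap distinguishes successful container jams from other outcomes, except CCTV hits, which leave it unchanged.
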(event `self.ReceiveHit`
  (params (MyComp :type "PrimitiveComponent Object Reference") (Other :type "Actor Object Reference") (OtherComp :type "PrimitiveComponent Object Reference") (bSelfMoved :type Boolean) (HitLocation :type "Vector Structure") (HitNormal :type "Vector Structure") (NormalImpulse :type "Vector Structure") (Hit :type "HitResult Structure (by ref)"))
  (bind _visual1 (`self.Visual1`))
  (bind _hittarget (`self.HitTarget`))
  (`parent.ReceiveHit` MyComp Other OtherComp bSelfMoved HitLocation HitNormal NormalImpulse Hit)
  (`/Engine/EditorBlueprintResources/StandardMacros.DoOnce` false
    (:`Completed`
      (set `self.HitTarget` Other)
      (`SceneComponent.K2_SetWorldRotation` (`self.Visual`) (`KismetMathLibrary.MakeRotator` (.roll (`KismetMathLibrary.Conv_VectorToRotator` HitNormal)) (+ (.pitch (`KismetMathLibrary.Conv_VectorToRotator` HitNormal)) -90.0) (.yaw (`KismetMathLibrary.Conv_VectorToRotator` HitNormal))) false false)
      (`KismetSystemLibrary.Delay` 0.2)
      (bind _asobject_entry_container (cast `/Game/Blueprints/Objects/ObjectEntry_Container` _hittarget)
        (:`then`
          (set `self.WasLocked` (`/Game/Blueprints/Objects/ObjectEntry_Container.Locked` _asobject_entry_container))
          (set `/Game/Blueprints/Objects/ObjectEntry_Container.Locked` false _asobject_entry_container)
          (`/Game/Blueprints/Objects/ObjectEntry_Container.SetContainerVisual` _asobject_entry_container)
          (`/Game/Blueprints/Objects/ObjectEntry_Master.TakeDamage_Object` _asobject_entry_container (`self.BaseDamage`) (`self.DestructionDamage`))
          (bind _asobject_entry_container_fuse_slot (cast `/Game/Blueprints/Objects/ObjectEntry_Container_FuseSlot` _asobject_entry_container)
            (:`then`
              (set `/Game/Blueprints/Objects/ObjectEntry_Container_FuseSlot.IsPowerInterupted` true _asobject_entry_container_fuse_slot)
              (`/Game/Blueprints/Objects/ObjectEntry_Container.SetContainerVisual` _asobject_entry_container_fuse_slot)
              (`KismetSystemLibrary.Delay` 0.8 :!label _label)
              (`PrimitiveComponent.SetMaterial` _visual1 0 "/Game/Materials/BasicUnlit_Container_1.BasicUnlit_Container_1"))
            (:`CastFailed`
              (if (`self.WasLocked`)
                (goto _label)
                (else
                  (`PrimitiveComponent.SetMaterial` _visual1 0 "/Game/Materials/BasicUnlit_Container_2.BasicUnlit_Container_2" :!label _label_2))))))
        (:`CastFailed`
          (bind _asenemy_entry_master (cast `/Game/Blueprints/Enemies/EnemyEntry_Master` _hittarget)
            (:`then`
              (`self.ForLoopDelay` 0 3 :!label _label_3
                (:`LoopBody`
                  (`/Game/Blueprints/Enemies/EnemyEntry_Master.TakeDamage_Enemy` _asenemy_entry_master (`self.BaseDamage`) (`self.DestructionDamage`) (`self.Parent`) (`self.Stagger Duration`) (`self.Knockback Amount`) (`self.NoStagger/Knockback`)))
                (:`Complete`
                  (goto _label_2))
                (:`OutDelay`
                  (`KismetSystemLibrary.Delay` 2.0)
                  (goto _label_3 :!via `InDelay`))))
            (:`CastFailed`
              (bind _asobject_entry_cctv (cast `/Game/Blueprints/Objects/ObjectEntry_CCTV` _hittarget)
                (:`then`
                  (`/Game/Blueprints/Objects/ObjectEntry_Master.TakeDamage_Object` _asobject_entry_cctv (`/Game/Blueprints/Objects/ObjectEntry_Master.Health_TotalMax` _asobject_entry_cctv) 1.0))
                (:`CastFailed`
                  (goto _label_2))))))))))

(fn `UserConstructionScript`
  (`parent.UserConstructionScript`))