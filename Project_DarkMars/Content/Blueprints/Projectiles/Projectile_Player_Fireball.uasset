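; Player fireball projectile that slows in flight and acts as a lingering area-damage hazard.
; A timeline eases max speed toward a fifth of launch speed, and the Niagara effect deactivates after a delay.
; An open Gate and Delay loop pulses damage each second to enemies and objects whose capsule or visual overlaps Sphere1.
; An overlapping player character stored as Parent takes half damage.
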(event `self.ReceiveBeginPlay`
  (bind _sphere1 (`self.Sphere1`))
  (bind _destructiondamage (`self.DestructionDamage`))
  (bind _parent (`self.Parent`))
  (bind _basedamage (`self.BaseDamage`))
  (bind _parent_2 (`self.Parent`))
  (bind _stagger_duration (`self.Stagger Duration`))
  (bind _knockback_amount (`self.Knockback Amount`))
  (bind _x (.x (`self.StartVelocity`)))
  (`parent.ReceiveBeginPlay`)
  (`|ExecutionSequence`
    (:`then_0`
      (bind (_direction _newtrack_0) (`Timeline|Timeline_0` :!via `PlayFromStart`)
        (:`Update`
          (set `ProjectileMovementComponent.MaxSpeed` (`KismetMathLibrary.Lerp` _x (* _x 0.2) _newtrack_0) (`self.ProjectileMovement`))
          (`KismetSystemLibrary.Delay` 4.0)
          (`ActorComponent.Deactivate` (`self.Niagara`)))))
    (:`then_1`
      (`/Engine/EditorBlueprintResources/StandardMacros.Gate` false :!label _label
        (:`Exit`
          (`|ExecutionSequence`
            (:`then_0`
              (set `self.FoundEnemyNear` false)
              (for _array_element (`PrimitiveComponent.GetOverlappingActors` _sphere1 "/Game/Blueprints/Enemies/EnemyEntry_Master.EnemyEntry_Master_C")
                (bind _asenemy_entry_master (cast `/Game/Blueprints/Enemies/EnemyEntry_Master` _array_element))
                (if (`PrimitiveComponent.IsOverlappingComponent` _sphere1 (`Character.CapsuleComponent` _asenemy_entry_master))
                  (`/Game/Blueprints/Enemies/EnemyEntry_Master.TakeDamage_Enemy` _asenemy_entry_master _basedamage _destructiondamage _parent_2 _stagger_duration _knockback_amount (`self.NoStagger/Knockback`))))
              (for _array_element_2 (`PrimitiveComponent.GetOverlappingActors` _sphere1 "/Game/Blueprints/Objects/ObjectEntry_Master.ObjectEntry_Master_C")
                (bind _asobject_entry_master (cast `/Game/Blueprints/Objects/ObjectEntry_Master` _array_element_2))
                (if (`PrimitiveComponent.IsOverlappingComponent` _sphere1 (`/Game/Blueprints/Objects/ObjectEntry_Master.visual` _asobject_entry_master))
                  (`/Game/Blueprints/Objects/ObjectEntry_Master.TakeDamage_Object` _asobject_entry_master _basedamage _destructiondamage)))
              (if (`PrimitiveComponent.IsOverlappingActor` _sphere1 _parent)
                (bind _asbp_top_down_character (cast `/Game/Blueprints/BP_TopDownCharacter` _parent))
                (`/Game/Blueprints/BP_TopDownCharacter.TakeDamage` _asbp_top_down_character (* _basedamage 0.5) (* _destructiondamage 0.5) _stagger_duration _knockback_amount _parent_2)))
            (:`then_1`
              (`KismetSystemLibrary.Delay` 1.0)
              (goto _label))))))))

(event `self.ReceiveHit`
  (params (MyComp :type "PrimitiveComponent Object Reference") (Other :type "Actor Object Reference") (OtherComp :type "PrimitiveComponent Object Reference") (bSelfMoved :type Boolean) (HitLocation :type "Vector Structure") (HitNormal :type "Vector Structure") (NormalImpulse :type "Vector Structure") (Hit :type "HitResult Structure (by ref)"))
  (`parent.ReceiveHit` MyComp Other OtherComp bSelfMoved HitLocation HitNormal NormalImpulse Hit))

(fn `UserConstructionScript`
  (`parent.UserConstructionScript`))