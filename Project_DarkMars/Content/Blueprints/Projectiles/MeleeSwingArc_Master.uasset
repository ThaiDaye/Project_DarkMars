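; MeleeSwingArc_Master is a melee swing arc Blueprint, filed under projectiles, that shows a visual which fades after spawning.
; On BeginPlay it gives the Visual component a small random roll.
; A self-repeating short Delay loop then steadily lowers Fade and writes it, clamped at zero or above, to the material scalar O2.
; The loop has no exit condition and the graph contains no destroy call.
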(event `self.ReceiveBeginPlay`
  (`parent.ReceiveBeginPlay`)
  (`SceneComponent.K2_AddLocalRotation` (`self.Visual`) (`KismetMathLibrary.MakeRotator` (`KismetMathLibrary.RandomFloatInRange` -15.0 15.0)) false false)
  (`|ExecutionSequence` :!label _label
    (:`then_0`
      (bind _output_get (set `self.Fade` (- (`self.Fade`) 0.025)))
      (`MeshComponent.SetScalarParameterValueOnMaterials` (`self.Visual`) "O2" (`KismetMathLibrary.FClamp` _output_get 0.0 999.0)))
    (:`then_1`
      (`KismetSystemLibrary.Delay` 0.01)
      (goto _label))))

(fn `UserConstructionScript`
  (`parent.UserConstructionScript`))