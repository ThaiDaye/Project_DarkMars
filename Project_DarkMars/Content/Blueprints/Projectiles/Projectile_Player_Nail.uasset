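; Player nail projectile that becomes stronger when fired at maximum charge.
; On BeginPlay, a max-charge nail swaps to an unlit material, doubles its custom time dilation to move faster and doubles destruction damage, clamped.
; The knockback boost is immediately overwritten by scaled StaggerDuration, leaving stagger itself unchanged.
; Hit handling and construction only call the parent class.
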(event `self.ReceiveBeginPlay`
  (`parent.ReceiveBeginPlay`)
  (if (`self.ChargeIsMax`)
    (`PrimitiveComponent.SetMaterial` (`self.Visual`) 0 "/Game/Materials/BasicUnlit_Master_Inst5.BasicUnlit_Master_Inst5")
    (set `self.CustomTimeDilation` 2.0)
    (set `self.Knockback Amount` (* (`self.Knockback Amount`) 1.5))
    (set `self.Knockback Amount` (* (`self.Stagger Duration`) 1.5))
    (set `self.DestructionDamage` (`KismetMathLibrary.FClamp` (* (`self.DestructionDamage`) 2.0)))))

(event `self.ReceiveHit`
  (params (MyComp :type "PrimitiveComponent Object Reference") (Other :type "Actor Object Reference") (OtherComp :type "PrimitiveComponent Object Reference") (bSelfMoved :type Boolean) (HitLocation :type "Vector Structure") (HitNormal :type "Vector Structure") (NormalImpulse :type "Vector Structure") (Hit :type "HitResult Structure (by ref)"))
  (`parent.ReceiveHit` MyComp Other OtherComp bSelfMoved HitLocation HitNormal NormalImpulse Hit))

(fn `UserConstructionScript`
  (`parent.UserConstructionScript`))