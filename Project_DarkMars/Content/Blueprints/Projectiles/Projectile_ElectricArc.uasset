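; Electric arc projectile that draws a jittering cable-based lightning link back to its parent actor.
; On BeginPlay it spawns a spark burst particle system, then attaches the cable's end to the parent, destroying itself if no valid parent exists.
; A delayed loop re-randomizes the cable force on each axis ten times a second, with extra upward bias, to make the arc whip erratically.
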(event `self.ReceiveBeginPlay`
  (bind _returnvalue (`KismetMathLibrary.RandomBool`))
  (bind _parent (`self.Parent`))
  (`parent.ReceiveBeginPlay`)
  (`NiagaraFunctionLibrary.SpawnSystemAtLocation` "/Game/VFX/Spark_Burst_ParticleSystem.Spark_Burst_ParticleSystem" (`self.K2_GetActorLocation`))
  (`/Engine/EditorBlueprintResources/StandardMacros.IsValid` _parent
    (:`Is Valid`
      (`CableComponent.SetAttachEndTo` (`self.Cable`) _parent "None" "None")
      (`|ExecutionSequence` :!label _label
        (:`then_0`
          (set `CableComponent.CableForce` (`KismetMathLibrary.MakeVector` (select `bool` _returnvalue :`false` -10000.0 :`true` 10000.0) (select `bool` _returnvalue :`false` -10000.0 :`true` 10000.0) (+ (select `bool` _returnvalue :`false` -10000.0 :`true` 10000.0) (`KismetMathLibrary.RandomFloatInRange` 5000.0 20000.0))) (`self.Cable`)))
        (:`then_1`
          (`KismetSystemLibrary.Delay` 0.1)
          (goto _label))))
    (:`Is Not Valid`
      (`self.K2_DestroyActor`))))

(fn `UserConstructionScript`
  (`parent.UserConstructionScript`))