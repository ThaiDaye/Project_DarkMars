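; Throwable flare projectile that acts as a temporary light source and burns out over time.
; On BeginPlay it arms itself and, if its Parent is a top-down character, adds itself to that character's OtherLightsRef list.
; A gated Delay loop then steadily shrinks DetonationRadius, deactivating the flare particle system and closing the gate at zero.
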(event `self.ReceiveBeginPlay`
  (`parent.ReceiveBeginPlay`)
  (set `self.Armed` true)
  (bind _asbp_top_down_character (cast `/Game/Blueprints/BP_TopDownCharacter` (`self.Parent`)))
  (`KismetArrayLibrary.Array_Add` (`/Game/Blueprints/BP_TopDownCharacter.OtherLightsRef` _asbp_top_down_character) self)
  (`/Engine/EditorBlueprintResources/StandardMacros.Gate` false :!label _label
    (:`Exit`
      (`|ExecutionSequence`
        (:`then_0`
          (bind _output_get (set `self.DetonationRadius` (`KismetMathLibrary.FClamp` (- (`self.DetonationRadius`) 2.5) 0.0 9999.0)))
          (if (== _output_get 0.0)
            (`ActorComponent.Deactivate` (`self.Flare_Particle_System`))
            (goto _label :!via `Close`)))
        (:`then_1`
          (`KismetSystemLibrary.Delay` 0.1)
          (goto _label))))))

(fn `UserConstructionScript`
  (`parent.UserConstructionScript`))