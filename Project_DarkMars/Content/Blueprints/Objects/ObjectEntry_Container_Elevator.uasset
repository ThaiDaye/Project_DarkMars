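; Elevator container object that moves the player between linked elevators, with a loading variant that swaps shaft meshes.
; The loading variant polls until world generation completes, links its destination to the home elevator and triggers travel.
; Travel teleports the player with relative position, rotation and camera yaw preserved; non-loading elevators then trigger any needed map generation.
; Non-loading elevators find their door by line trace; interaction toggles it alongside a timeline-driven lid animation.
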(event `self.OnOpenCloseContainerVisual`
  (params (Open :type Boolean))
  (if Open
    ;[1 1 1] open close visuak
    (bind (_direction _newtrack_0) (`Timeline|Timeline_1` :!label _label)
      (:`Update`
        (`SceneComponent.K2_SetRelativeTransform` (`self.ContainerLidVisual1`) (`KismetMathLibrary.TLerp` (`self.CloseLidTransform_2`) (`self.OpenLidTransform_2`) _newtrack_0) false false)))
    (else
      (goto _label :!via `Reverse`))))

(event `self.OnInteract`
  (bind _doorref (`self.DoorRef`))
  ;[1 1 1] open close visuak
  (`parent.OnInteract`)
  (`/Engine/EditorBlueprintResources/StandardMacros.IsValid` _doorref
    (:`Is Valid`
      (set `/Game/Blueprints/Objects/ObjectEntry_Door.Open` (not (`self.Open`)) _doorref)
      (`/Game/Blueprints/Objects/ObjectEntry_Door.ProxyDoorInteract` _doorref)
      (`/Engine/EditorBlueprintResources/StandardMacros.IsValid` (`SceneComponent.GetChildComponent` (`self.ContainerLidVisual1`) 0)
        (:`Is Valid`
          (if (`/Game/Blueprints/Objects/ObjectEntry_Door.Open` _doorref)
            (goto _label)
            (else
              (goto _label :!via `Reverse`))))))))

(event `self.ReceiveBeginPlay`
  (bind _connectedelevator (`self.ConnectedElevator`))
  (`parent.ReceiveBeginPlay`)
  (if (`self.LoadingElevator`)
    (`self.DoAfterWorldGen` :!label _label_2
      (:`GenComplete`
        (`/Engine/EditorBlueprintResources/StandardMacros.IsValid` _connectedelevator
          (:`Is Valid`
            (set `/Game/Blueprints/Objects/ObjectEntry_Container_Elevator.ConnectedElevator` _connectedelevator (`/Game/Blueprints/WorldGen_Master.HomeElevator` (`self.WorldGenRef`)))
            (`/Game/Blueprints/BP_TopDownCharacter.PlaySFXFromSoundBank` (`self.PlayerRef`) "NewEnumerator16" (`SceneComponent.K2_GetComponentLocation` (`/Game/Blueprints/Objects/ObjectEntry_Container_Elevator.StaticMesh4` _connectedelevator)))
            (`self.TravelUsingElevator`)
            (`self.SetupConnectedElevatorIndex` (`self.MapLocationIndex`))
            (set `/Game/Blueprints/Objects/ObjectEntry_Container_Elevator.ConnectedElevator` (`/Game/Blueprints/WorldGen_Master.HomeElevator` (`self.WorldGenRef`)) _connectedelevator))
          (:`Is Not Valid`
            (`KismetSystemLibrary.Delay` 0.2)
            (goto _label_2)))))
    (else
      (`PrimitiveComponent.SetMaterial` (`self.StaticMesh4`) 0 "/Game/Materials/BasicUnlit_Container_1.BasicUnlit_Container_1")
      (`self.ConnectDoors`)
      ;[1 1 1] open close visuak
      (`/Engine/EditorBlueprintResources/StandardMacros.IsValid` (`self.DoorRef`)
        (:`Is Valid`
          (goto _label))))))

(event `TravelUsingElevator`
  (bind _connectedelevator (`self.ConnectedElevator`))
  (bind _playerref (`self.PlayerRef`))
  (bind _doorref (`self.DoorRef`))
  (bind _playerref_2 (`self.PlayerRef`))
  (bind _returnvalue (`SceneComponent.K2_GetComponentToWorld` (`self.Scene`)))
  (bind _rootcomponent (`Actor.RootComponent` _playerref))
  (bind _springarm (`/Game/Blueprints/BP_TopDownCharacter.SpringArm` _playerref_2))
  (bind (_returnvalue_roll _returnvalue_pitch) (`KismetMathLibrary.BreakRotator` (`SceneComponent.K2_GetComponentRotation` _springarm)))
  (bind _returnvalue_2 (`SceneComponent.K2_GetComponentToWorld` (`/Game/Blueprints/Objects/ObjectEntry_Container_Elevator.Scene` _connectedelevator)))
  (`/Engine/EditorBlueprintResources/StandardMacros.IsValid` _connectedelevator
    (:`Is Valid`
      (if (`self.LoadingElevator`)
        (if (`/Game/Blueprints/WorldGen_Master.FloorGenerated` (`self.WorldGenRef`))
          (`self.K2_SetActorLocationAndRotation` _playerref_2 (`KismetMathLibrary.TransformLocation` _returnvalue_2 (`KismetMathLibrary.InverseTransformLocation` _returnvalue (`SceneComponent.K2_GetComponentLocation` _rootcomponent))) (`KismetMathLibrary.TransformRotation` _returnvalue_2 (`KismetMathLibrary.InverseTransformRotation` _returnvalue (`SceneComponent.K2_GetComponentRotation` _rootcomponent))) false true :!label _label_3)
          (`SceneComponent.K2_SetWorldRotation` _springarm (`KismetMathLibrary.MakeRotator` _returnvalue_roll _returnvalue_pitch (.yaw (`KismetMathLibrary.TransformRotation` _returnvalue_2 (`KismetMathLibrary.InverseTransformRotation` _returnvalue (`SceneComponent.K2_GetComponentRotation` (`/Game/Blueprints/BP_TopDownCharacter.SpringArm` _playerref)))))) false false)
          (if (not (`self.LoadingElevator`))
            (`|ExecutionSequence`
              (:`then_0`
                (if (not (`/Game/Blueprints/WorldGen_Master.FloorGenerated` (`self.WorldGenRef`)))
                  (`/Game/Blueprints/WorldGen_Master.GenerateMap` (`self.WorldGenRef`))))
              (:`then_1`
                (`self.Open/CloseContainerVisual` false)
                (`self.OnOpenCloseContainerVisual` true)
                (`/Engine/EditorBlueprintResources/StandardMacros.IsValid` _doorref
                  (:`Is Valid`
                    (set `/Game/Blueprints/Objects/ObjectEntry_Door.Open` true _doorref)
                    (`/Game/Blueprints/Objects/ObjectEntry_Door.ProxyDoorInteract` _doorref)))))))
        (else
          (goto _label_3))))))

(event `SetupConnectedElevatorIndex`
  (params (Index :type Integer))
  (bind _connectedelevator (`self.ConnectedElevator`))
  (`/Engine/EditorBlueprintResources/StandardMacros.IsValid` _connectedelevator
    (:`Is Valid`
      (set `/Game/Blueprints/Objects/ObjectEntry_Container_Elevator.MapLocationIndex` Index _connectedelevator))))

(fn `ConnectDoors`
  (bind _defaultsceneroot (`self.DefaultSceneRoot`))
  (bind _returnvalue (`KismetMathLibrary.MakeVector` (.x (`SceneComponent.K2_GetComponentLocation` _defaultsceneroot)) (.y (`SceneComponent.K2_GetComponentLocation` _defaultsceneroot)) 150.0))
  (bind _outhit (`KismetSystemLibrary.LineTraceSingleForObjects` _returnvalue (`KismetMathLibrary.MakeVector` (.x (+ _returnvalue (`SceneComponent.GetRightVector` _defaultsceneroot))) (.y (+ _returnvalue (`SceneComponent.GetRightVector` _defaultsceneroot))) 150.0) (`|MakeArray` "ObjectTypeQuery8" :!type "EObjectTypeQuery Enum")))
  (bind (_bblockinghit _binitialoverlap _time _distance _location _impactpoint _normal _impactnormal _physmat _hitactor) (`GameplayStatics.BreakHitResult` _outhit))
  (if _bblockinghit
    (bind _asobject_entry_door (cast `/Game/Blueprints/Objects/ObjectEntry_Door` _hitactor))
    (set `self.DoorRef` _asobject_entry_door)))

(fn `UserConstructionScript`
  (bind _loadingelevator (`self.LoadingElevator`))
  (bind _returnvalue (select `bool` _loadingelevator :`false` "/Game/ScienceLab/Meshes/Rooms/Lift/SM_Lift01Shaft01.SM_Lift01Shaft01" :`true` "/Game/ScienceLab/Meshes/Rooms/Lift/SM_Lift01Shaft03.SM_Lift01Shaft03" :!type "StaticMesh Object Reference"))
  (`parent.UserConstructionScript`)
  (`StaticMeshComponent.SetStaticMesh` (`self.StaticMesh`) _returnvalue)
  (`StaticMeshComponent.SetStaticMesh` (`self.StaticMesh8`) _returnvalue)
  (if _loadingelevator
    (`ActorComponent.K2_DestroyComponent` (`self.StaticMesh10`))
    (`ActorComponent.K2_DestroyComponent` (`self.StaticMesh5`))
    (else
      (`ActorComponent.K2_DestroyComponent` (`self.StaticMesh3`))
      (`ActorComponent.K2_DestroyComponent` (`self.StaticMesh2`)))))