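; Fuse slot container that powers machines in nearby rooms while it holds a power cell.
; After world gen it links non-hallway rooms and their machines; inventory changes update visuals and, without a connected transformer, switch those machines, respecting other live fuses.
; On death it turns volatile, ejects the cell and periodically fires electric arcs while the player is near.
; Arcs favour conductive, line-of-sight targets through substance-weighted rolls, otherwise striking random ground.
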(event `EjectCellFunction`
  (bind _returnvalue (`SceneComponent.K2_GetComponentLocation` (`self.ArcStart`)))
  ;[1 1 1] begfin
  (if (`self.IsVolatile`) :!label _label
    (if (`self.HasPowerCell`)
      (`self.OnThisContainerEdit`)
      (for _ (range 26)
        (if (not (`self.EjectedPowerCell`))
          (bind _randomlocation (`NavigationSystemV1.K2_GetRandomLocationInNavigableRadius` _returnvalue 3000.0 null null))
          (bind _outhit (`KismetSystemLibrary.SphereTraceSingle` _returnvalue _randomlocation 15.0 "TraceTypeQuery1"))
          (bind (_bblockinghit _binitialoverlap _time _distance _location) (`GameplayStatics.BreakHitResult` _outhit))
          (if (>= _distance 500.0)
            (if _bblockinghit
              (set `self.EjectedPowerCell` true)
              (`|SpawnActorFromClass` "/Game/Blueprints/Objects/ObjectEntry_ItemPickup.ObjectEntry_ItemPickup_C" (`KismetMathLibrary.MakeTransform` (`KismetMathLibrary.MakeVector` (.x _location) (.y _location) 50.0)) "Undefined" "OverrideRootScale" null "17" -1 1 0 false "None" "NewEnumerator0" null null)
              (else
                (set `self.EjectedPowerCell` true)
                (`|SpawnActorFromClass` "/Game/Blueprints/Objects/ObjectEntry_ItemPickup.ObjectEntry_ItemPickup_C" (`KismetMathLibrary.MakeTransform` (+ _randomlocation (0.0 0.0 50.0))) "Undefined" "OverrideRootScale" null "17" -1 1 0 false "None" "NewEnumerator0" null null))))))
      (if (`self.EjectedPowerCell`)
        (`/Game/Blueprints/BP_TopDownCharacter.Debug_PrintString_Internal` :`self` (`self.PlayerRef`) :`Text` "Power Cell Pooped" :`Colour` (struct :`R` 0.177083 :`G` 0.064165 :`B` 0.008455 :`A` 1.0))
        (bind (_found _foundatleastone _indexes) (`/Game/Blueprints/BP_TopDownCharacter.Inv_FindItem` (`self.PlayerRef`) "17" 1 self))
        (for (_ _array_index) _indexes
          (`KismetArrayLibrary.Array_Remove` (`self.ItemInventoryList`) _array_index))
        (`self.OnThisContainerEdit`)
        (set `self.Open` true)
        (set `self.Locked` false)
        (`self.SetContainerVisual`))
      (else
        (`self.OnThisContainerEdit` :!label _label_2)))
    (else
      (goto _label_2))))

(event `self.ReceiveBeginPlay`
  ;[1 1 1] begfin
  (`parent.ReceiveBeginPlay`)
  (`self.OnThisContainerEdit`)
  (`self.DoAfterWorldGen`
    (:`GenComplete`
      (`self.SetStartState__` (select `/Game/Blueprints/Data/EnemyStartingState_Type` (`self.ObjectStartState`) :`NewEnumerator0` "NewEnumerator0" :`NewEnumerator1` "NewEnumerator1" :`NewEnumerator2` "NewEnumerator2" :`NewEnumerator3` "NewEnumerator0" :!type "/Game/Blueprints/Data/EnemyStartingState_Type Enum") "NewEnumerator0" 140.0 true 300.0)
      (if (`self.TransformerConnected`)
        (goto _label)
        (else
          (`self.SetConnectedRooms`)
          (goto _label))))))

(event `StartElectricArc`
  (bind _niagara (`self.Niagara`))
  (bind _playerref (`self.PlayerRef`))
  (bind _returnvalue (`SceneComponent.K2_GetComponentLocation` (`self.ArcStart`)))
  ;[1 1 1] find arc target
  (if (`self.IsVolatile`)
    (`|ExecutionSequence`
      (:`then_0`
        (goto _label_3 :!via `Open`))
      (:`then_1`
        (`/Engine/EditorBlueprintResources/StandardMacros.Gate` true :!label _label_3
          (:`Exit`
            (`|ExecutionSequence`
              (:`then_0`
                (if (and (`self.Open`) (not (`self.IsPowerInterupted`)))
                  (`/Engine/EditorBlueprintResources/StandardMacros.IsValid` _playerref
                    (:`Is Valid`
                      ;;[1 1 1] Comment
                      (if (<= (`KismetMathLibrary.VSize` (- (`self.K2_GetActorLocation` _playerref) (`self.K2_GetActorLocation`))) 2000.0)
                        (`SceneComponent.SetVisibility` _niagara (`self.IsVolatile`) false)
                        (bind _outhits (`KismetSystemLibrary.SphereTraceMultiForObjects` _returnvalue _returnvalue (* (`KismetSystemLibrary.MakeLiteralDouble` (`self.ElectricArcRadius`)) 0.75) (`|MakeArray` "ObjectTypeQuery7" "ObjectTypeQuery8" "ObjectTypeQuery12" "ObjectTypeQuery11" "ObjectTypeQuery9" "ObjectTypeQuery10" :!type "EObjectTypeQuery Enum")))
                        (set `self.TargetSubstance` "NewEnumerator4")
                        (set `self.HasFoundArcTarget` false)
                        (set `self.FoundArcTarget` null)
                        (for _array_element _outhits
                          (bind (_bblockinghit _binitialoverlap _time _distance _location _impactpoint _normal _impactnormal _physmat _hitactor _hitcomponent) (`GameplayStatics.BreakHitResult` _array_element))
                          (if _bblockinghit
                            (bind _asprojectile_master (cast `/Game/Blueprints/Projectiles/Projectile_Master` _hitactor)
                              (:`then`
                                (bind _projectile_substance (`/Game/Blueprints/Projectiles/Projectile_Master.Projectile Substance` _asprojectile_master))
                                (if (> (`KismetMathLibrary.Conv_ByteToInt` _projectile_substance) (`KismetMathLibrary.Conv_ByteToInt` (`self.TargetSubstance`)))
                                  (if (`KismetMathLibrary.RandomBoolWithWeight` (select `/Game/Blueprints/Data/EntrySubstance_Type` _projectile_substance :`NewEnumerator4` 0.3 :`NewEnumerator7` 0.5 :`NewEnumerator2` 0.75 :`NewEnumerator1` 0.75 :`NewEnumerator6` 1.0 :`NewEnumerator3` 1.0 :`NewEnumerator8` 0.2 :!type "Float (single-precision)"))
                                    (if (not (or (`|EnumEquality` _projectile_substance "NewEnumerator5") (`|EnumEquality` "NewEnumerator0" _projectile_substance)))
                                      (bind _outhit (`KismetSystemLibrary.LineTraceSingleForObjects` (`SceneComponent.K2_GetComponentLocation` (`self.ArcStart`)) (`self.K2_GetActorLocation` _asprojectile_master) (`|MakeArray` "ObjectTypeQuery1" "ObjectTypeQuery2" "ObjectTypeQuery8" :!type "EObjectTypeQuery Enum")))
                                      (if (not (`GameplayStatics.BreakHitResult` _outhit))
                                        (set `self.TargetSubstance` _projectile_substance)
                                        (set `self.FoundArcTarget` _asprojectile_master)
                                        (set `self.HasFoundArcTarget` true))))))
                              (:`CastFailed`
                                (bind _asobject_entry_item_pickup (cast `/Game/Blueprints/Objects/ObjectEntry_ItemPickup` _hitactor)
                                  (:`then`
                                    (bind _object_substance (`/Game/Blueprints/Objects/ObjectEntry_Master.Object Substance` _asobject_entry_item_pickup))
                                    (if (> (`KismetMathLibrary.Conv_ByteToInt` _object_substance) (`KismetMathLibrary.Conv_ByteToInt` (`self.TargetSubstance`)))
                                      (if (`KismetMathLibrary.RandomBoolWithWeight` (select `/Game/Blueprints/Data/EntrySubstance_Type` _object_substance :`NewEnumerator4` 0.15 :`NewEnumerator7` 0.25 :`NewEnumerator2` 0.5 :`NewEnumerator1` 0.5 :`NewEnumerator6` 0.75 :`NewEnumerator3` 0.75 :`NewEnumerator8` 0.1 :!type "Float (single-precision)"))
                                        (if (not (or (`|EnumEquality` _object_substance "NewEnumerator5") (`|EnumEquality` "NewEnumerator0" _object_substance)))
                                          (bind _outhit_2 (`KismetSystemLibrary.LineTraceSingleForObjects` (`SceneComponent.K2_GetComponentLocation` (`self.ArcStart`)) (`self.K2_GetActorLocation` _asobject_entry_item_pickup) (`|MakeArray` "ObjectTypeQuery1" "ObjectTypeQuery2" "ObjectTypeQuery8" :!type "EObjectTypeQuery Enum")))
                                          (if (not (`GameplayStatics.BreakHitResult` _outhit_2))
                                            (set `self.TargetSubstance` _object_substance)
                                            (set `self.FoundArcTarget` _asobject_entry_item_pickup)
                                            (set `self.HasFoundArcTarget` true))))))
                                  (:`CastFailed`
                                    (bind _asenemy_entry_master (cast `/Game/Blueprints/Enemies/EnemyEntry_Master` _hitactor)
                                      (:`then`
                                        (if (== (`Character.CapsuleComponent` _asenemy_entry_master) _hitcomponent)
                                          (bind _enemy_substance (`/Game/Blueprints/Enemies/EnemyEntry_Master.Enemy Substance` _asenemy_entry_master))
                                          (if (> (`KismetMathLibrary.Conv_ByteToInt` _enemy_substance) (`KismetMathLibrary.Conv_ByteToInt` (`self.TargetSubstance`)))
                                            (if (`KismetMathLibrary.RandomBoolWithWeight` (select `/Game/Blueprints/Data/EntrySubstance_Type` _enemy_substance :`NewEnumerator4` 0.25 :`NewEnumerator7` 0.5 :`NewEnumerator2` 0.65 :`NewEnumerator1` 0.65 :`NewEnumerator6` 0.75 :`NewEnumerator3` 0.75 :`NewEnumerator8` 0.2 :!type "Float (single-precision)"))
                                              (if (not (or (`|EnumEquality` _enemy_substance "NewEnumerator5") (`|EnumEquality` _enemy_substance "NewEnumerator0")))
                                                (bind _outhit_3 (`KismetSystemLibrary.LineTraceSingleForObjects` (`SceneComponent.K2_GetComponentLocation` (`self.ArcStart`)) (`self.K2_GetActorLocation` _asenemy_entry_master) (`|MakeArray` "ObjectTypeQuery1" "ObjectTypeQuery2" "ObjectTypeQuery8" :!type "EObjectTypeQuery Enum")))
                                                (if (not (`GameplayStatics.BreakHitResult` _outhit_3))
                                                  (set `self.TargetSubstance` _enemy_substance)
                                                  (set `self.FoundArcTarget` _asenemy_entry_master)
                                                  (set `self.HasFoundArcTarget` true)))))
                                          (else
                                            (bind _asobject_entry_master (cast `/Game/Blueprints/Objects/ObjectEntry_Master` _hitactor :!label _label_4)
                                              (:`then`
                                                (bind _object_substance_2 (`/Game/Blueprints/Objects/ObjectEntry_Master.Object Substance` _asobject_entry_master))
                                                (if (> (`KismetMathLibrary.Conv_ByteToInt` _object_substance_2) (`KismetMathLibrary.Conv_ByteToInt` (`self.TargetSubstance`)))
                                                  (if (`KismetMathLibrary.RandomBoolWithWeight` (select `/Game/Blueprints/Data/EntrySubstance_Type` _object_substance_2 :`NewEnumerator4` 0.05 :`NewEnumerator7` 0.15 :`NewEnumerator2` 0.25 :`NewEnumerator1` 0.25 :`NewEnumerator6` 0.5 :`NewEnumerator3` 0.5 :`NewEnumerator8` 0.05 :!type "Float (single-precision)"))
                                                    (if (not (or (`|EnumEquality` _object_substance_2 "NewEnumerator5") (`|EnumEquality` "NewEnumerator0" _object_substance_2)))
                                                      (bind _outhit_4 (`KismetSystemLibrary.LineTraceSingleForObjects` (`SceneComponent.K2_GetComponentLocation` (`self.ArcStart`)) (`self.K2_GetActorLocation` _asobject_entry_master) (`|MakeArray` "ObjectTypeQuery1" "ObjectTypeQuery2" "ObjectTypeQuery8" :!type "EObjectTypeQuery Enum")))
                                                      (if (not (`GameplayStatics.BreakHitResult` _outhit_4))
                                                        (set `self.TargetSubstance` _object_substance_2)
                                                        (set `self.FoundArcTarget` _asobject_entry_master)
                                                        (set `self.HasFoundArcTarget` true))))))
                                              (:`CastFailed`
                                                (bind _asbp_top_down_character (cast `/Game/Blueprints/BP_TopDownCharacter` _hitactor))
                                                (bind _player_substance (`/Game/Blueprints/BP_TopDownCharacter.Player Substance` _asbp_top_down_character))
                                                (bind _equipment_substance (`/Game/Blueprints/BP_TopDownCharacter.Equipment Substance` _asbp_top_down_character))
                                                (bind _returnvalue_2 (select `bool` (>= (`KismetMathLibrary.Conv_ByteToInt` _player_substance) (`KismetMathLibrary.Conv_ByteToInt` _equipment_substance)) :`false` _player_substance :`true` _equipment_substance))
                                                (if (> (`KismetMathLibrary.Conv_ByteToInt` _returnvalue_2) (`KismetMathLibrary.Conv_ByteToInt` (`self.TargetSubstance`)))
                                                  (if (`KismetMathLibrary.RandomBoolWithWeight` (select `/Game/Blueprints/Data/EntrySubstance_Type` _returnvalue_2 :`NewEnumerator4` 0.15 :`NewEnumerator7` 0.25 :`NewEnumerator2` 0.5 :`NewEnumerator1` 0.5 :`NewEnumerator6` 0.75 :`NewEnumerator3` 0.75 :`NewEnumerator8` 0.1 :!type "Float (single-precision)"))
                                                    (if (not (`|EnumEquality` _returnvalue_2 "NewEnumerator5"))
                                                      (bind _outhit_5 (`KismetSystemLibrary.LineTraceSingleForObjects` (`SceneComponent.K2_GetComponentLocation` (`self.ArcStart`)) (`self.K2_GetActorLocation` _asbp_top_down_character) (`|MakeArray` "ObjectTypeQuery1" "ObjectTypeQuery2" "ObjectTypeQuery8" :!type "EObjectTypeQuery Enum")))
                                                      (if (not (`GameplayStatics.BreakHitResult` _outhit_5))
                                                        (set `self.TargetSubstance` _returnvalue_2)
                                                        (set `self.FoundArcTarget` _asbp_top_down_character)
                                                        (set `self.HasFoundArcTarget` true))))))))))
                                      (:`CastFailed`
                                        (goto _label_4)))))))))
                        (if (`self.HasFoundArcTarget`)
                          (if (`KismetMathLibrary.RandomBoolWithWeight` 0.75)
                            (`self.ElectricArcToTarget`)
                            (else
                              (`self.ElectricArcToGround` :!label _label_5)))
                          (else
                            (goto _label_5)))
                        (else
                          (`SceneComponent.SetVisibility` _niagara false false :!label _label_6)))))
                  (else
                    (goto _label_6))))
              (:`then_1`
                (`KismetSystemLibrary.Delay` (+ (`KismetMathLibrary.RandomFloatInRange` 0.0 3.0) 0.5))
                (if (`self.IsVolatile`)
                  (goto _label_3)
                  (else
                    (goto _label_3 :!via `Close`)))))))))
    (else
      (goto _label_6))))

(event `self.OnDeath`
  (bind _niagara (`self.Niagara`))
  ;[1 1 1] set volatile
  (`parent.OnDeath`)
  (set `self.IsVolatile` true)
  (set `self.Open` true)
  (`self.EjectCellFunction`)
  (`self.Open/CloseContainerVisual` true)
  (`self.SetContainerVisual`)
  (`self.StartElectricArc`)
  (if (`self.IsVolatile`)
    (`ActorComponent.Activate` _niagara true)
    (else
      (`ActorComponent.Deactivate` _niagara))))

(event `self.OnThisContainerEdit`
  (bind _connectedtransformer (`self.ConnectedTransformer`))
  (bind _playerref (`self.PlayerRef`))
  ;[1 1 1] container update
  (`parent.OnThisContainerEdit`)
  (`/Engine/EditorBlueprintResources/StandardMacros.IsValid` _playerref
    (:`Is Valid`
      (bind (_found _foundatleastone) (`/Game/Blueprints/BP_TopDownCharacter.Inv_FindItem` _playerref "17" 1 self))
      (if _foundatleastone
        (set `self.HasPowerCell` true)
        (else
          (set `self.HasPowerCell` false)))
      (`self.SetContainerVisual`)
      (`/Engine/EditorBlueprintResources/StandardMacros.IsValid` _connectedtransformer
        (:`Is Valid`
          (`self.SetContainerVisual` _connectedtransformer))))))

(event `self.OnRevived`
  ;[1 1 1] on revivied
  (`parent.OnRevived`)
  (set `self.IsVolatile` false)
  (`self.SetContainerVisual`))

(event `self.SetContainerVisual`
  (bind _transformerconnected (`self.TransformerConnected`))
  (bind _lidvent_main (`self.LidVent_Main`))
  (bind _returnvalue (and (`self.IsPowerFlowing`) (`self.HasPowerCell`)))
  ;[1 1 1] udpate viduals
  (`parent.SetContainerVisual`)
  (if (`self.TransformerConnected`)
    (if (`self.HasPowerCell`)
      (if (or (`self.IsPowerInterupted`) (`self.IsVolatile`)) :!label _label_7
        (set `self.IsPowerFlowing` false :!label _label_8)
        (else
          (set `self.IsPowerFlowing` true)))
      (else
        (goto _label_8)))
    (else
      (goto _label_7)))
  (`|ExecutionSequence`
    (:`then_0`
      (if _returnvalue
        (`|ExecutionSequence`
          (:`then_0`
            (`/Engine/EditorBlueprintResources/StandardMacros.DoOnce` false :!label _label_9
              (:`Completed`
                (`self.PlaySFXFromLibrary` 0 true))))
          (:`then_1`
            (goto _label_10 :!via `Reset`)))
        (else
          (`|ExecutionSequence`
            (:`then_0`
              (`/Engine/EditorBlueprintResources/StandardMacros.DoOnce` false :!label _label_10
                (:`Completed`
                  (`self.PlaySFXFromLibrary` 1 true))))
            (:`then_1`
              (goto _label_9 :!via `Reset`))))))
    (:`then_1`
      (`self.SetRoomsMachinePower` _returnvalue (`self.IsPowerInterupted`))
      (`PrimitiveComponent.SetMaterial` (`self.visual`) 1 (select `bool` (or (`self.IsDead`) (== (`self.Health`) 0.0) (`self.IsPowerInterupted`)) :`false` (select `bool` (`self.IsPowerFlowing`) :`false` "/Game/Materials/BasicUnlit_Container_2.BasicUnlit_Container_2" :`true` (select `bool` (`self.HasPowerCell`) :`false` "/Game/Materials/BasicUnlit_Container_2.BasicUnlit_Container_2" :`true` "/Game/Materials/BasicUnlit_Container_1.BasicUnlit_Container_1" :!type "MaterialInterface Object Reference")) :`true` "/Game/Materials/BasicUnlit_Master_Inst.BasicUnlit_Master_Inst"))
      (`SceneComponent.SetVisibility` (`self.Cell`) (`self.HasPowerCell`) false)
      (if (not (`self.IsVolatile`))
        (`SceneComponent.SetVisibility` (`self.Niagara`) false false))
      (`SceneComponent.SetVisibility` (`self.LidVent`) (not _transformerconnected) false)
      (`SceneComponent.SetVisibility` _lidvent_main _transformerconnected false)
      (`PrimitiveComponent.SetMaterial` _lidvent_main 1 (`PrimitiveComponent.GetMaterial` (`self.visual`) 1))
      (if (`self.MarkOnRadar`)
        (if (`self.IsPowerFlowing`)
          (`self.MarkObjectOnRadar` false))))))

(event `ElectricArcToGround`
  (bind _returnvalue (`SceneComponent.K2_GetComponentLocation` (`self.ArcStart`)))
  ;[1 1 1] arc ranodm
  (bind _randomlocation (`NavigationSystemV1.K2_GetRandomLocationInNavigableRadius` _returnvalue (`KismetSystemLibrary.MakeLiteralDouble` (`self.ElectricArcRadius`)) null null))
  (bind _outhit (`KismetSystemLibrary.LineTraceSingleForObjects` _returnvalue _randomlocation (`|MakeArray` "ObjectTypeQuery1" "ObjectTypeQuery2" "ObjectTypeQuery8" :!type "EObjectTypeQuery Enum")))
  (if (not (`GameplayStatics.BreakHitResult` _outhit))
    (`|SpawnActorFromClass` "/Game/Blueprints/Projectiles/Projectile_ElectricArc.Projectile_ElectricArc_C" (`KismetMathLibrary.MakeTransform` _randomlocation) "Undefined" "OverrideRootScale" null self 0.0 0.1 0.0 0.25 0.0 0.0 0.0 "NewEnumerator0" false false false (struct) "ECC_GameTraceChannel3" null)
    (`/Game/Blueprints/BP_TopDownCharacter.ScreenShake` (`self.PlayerRef`) 2 "NewEnumerator0" 750.0 _randomlocation)))

(event `ElectricArcToTarget`
  (bind _foundarctarget (`self.FoundArcTarget`))
  (bind _returnvalue (`self.K2_GetActorLocation` (`self.FoundArcTarget`)))
  ;[1 1 1] arc taregt
  (bind _outhit (`KismetSystemLibrary.LineTraceSingleForObjects` _returnvalue (`SceneComponent.K2_GetComponentLocation` (`self.ArcStart`)) (`|MakeArray` "ObjectTypeQuery1" "ObjectTypeQuery2" "ObjectTypeQuery8" :!type "EObjectTypeQuery Enum")))
  (if (not (`GameplayStatics.BreakHitResult` _outhit))
    (bind _returnvalue_2 (`|SpawnActorFromClass` "/Game/Blueprints/Projectiles/Projectile_ElectricArc.Projectile_ElectricArc_C" (`KismetMathLibrary.MakeTransform` _returnvalue) "AlwaysSpawn" "OverrideRootScale" null self 0.0 0.1 0.0 0.25 0.0 0.0 0.0 "NewEnumerator0" false false false (struct) "ECC_GameTraceChannel3" null))
    (`/Game/Blueprints/BP_TopDownCharacter.ScreenShake` (`self.PlayerRef`) 2 "NewEnumerator0" 750.0 _returnvalue)
    (bind _asprojectile_master (cast `/Game/Blueprints/Projectiles/Projectile_Master` _foundarctarget)
      (:`then`
        (`self.K2_DestroyActor` _asprojectile_master))
      (:`CastFailed`
        (bind _asobject_entry_master (cast `/Game/Blueprints/Objects/ObjectEntry_Master` _foundarctarget)
          (:`then`
            (`self.TakeDamage_Object` _asobject_entry_master (`self.Electric_Damage`) (`self.Electric_Destruction`)))
          (:`CastFailed`
            (bind _asenemy_entry_master (cast `/Game/Blueprints/Enemies/EnemyEntry_Master` _foundarctarget)
              (:`then`
                (`/Game/Blueprints/Enemies/EnemyEntry_Master.TakeDamage_Enemy` _asenemy_entry_master (`self.Electric_Damage`) (`self.Electric_Destruction`) _returnvalue_2 2.0 0.0 false))
              (:`CastFailed`
                (bind _asbp_top_down_character (cast `/Game/Blueprints/BP_TopDownCharacter` _foundarctarget))
                (`/Game/Blueprints/BP_TopDownCharacter.TakeDamage` _asbp_top_down_character (`self.Electric_Damage`) (`self.Electric_Destruction`) 1.0 0.0 _returnvalue_2)))))))))

(fn `SetConnectedRooms`
  (bind _connectedrooms (`self.ConnectedRooms`))
  (bind _returnvalue (`KismetMathLibrary.MakeVector` (.x (`self.K2_GetActorLocation`)) (.y (`self.K2_GetActorLocation`)) 150.0))
  (bind _outhits (`KismetSystemLibrary.SphereTraceMultiForObjects` _returnvalue _returnvalue 500.0 (`|MakeArray` "ObjectTypeQuery13" :!type "EObjectTypeQuery Enum")))
  (for _array_element _outhits
    (bind _asroom_gen_master (cast `/Game/Blueprints/RoomGen_Master` (`.HitActor` (`GameplayStatics.BreakHitResult` _array_element))))
    (if (`/Game/Blueprints/RoomGen_Master.IsHallway` _asroom_gen_master)
      _
      (elif (not (`KismetArrayLibrary.Array_Contains` _connectedrooms _asroom_gen_master))
        (`KismetArrayLibrary.Array_Add` _connectedrooms _asroom_gen_master)
        (for _array_element_2 (`/Game/Blueprints/RoomGen_Master.ConnectedSideRooms` _asroom_gen_master)
          (`/Engine/EditorBlueprintResources/StandardMacros.IsValid` _array_element_2
            (:`Is Valid`
              (if (not (`/Game/Blueprints/RoomGen_Master.IsHallway` _array_element_2))
                (`KismetArrayLibrary.Array_Add` _connectedrooms _array_element_2))))))))
  (for _array_element_3 (`self.ConnectedRooms`)
    (`/Engine/EditorBlueprintResources/StandardMacros.IsValid` _array_element_3
      (:`Is Valid`
        (bind _bordervisual (`/Game/Blueprints/RoomGen_Master.BorderVisual` _array_element_3))
        (`/Engine/EditorBlueprintResources/StandardMacros.IsValid` _bordervisual
          (:`Is Valid`
            (bind _returnvalue_2 (`SceneComponent.K2_GetComponentLocation` _bordervisual))
            (bind (_x _y) (`KismetMathLibrary.BreakVector3f` (`BoxComponent.GetScaledBoxExtent` _bordervisual)))
            (bind _outhits_2 (`KismetSystemLibrary.BoxTraceMultiForObjects` _returnvalue_2 _returnvalue_2 (`KismetMathLibrary.MakeVector` (* _x 1.25) (* _y 1.25) 500.0) (struct) (`|MakeArray` "ObjectTypeQuery8" "ObjectTypeQuery12" "ObjectTypeQuery11" :!type "EObjectTypeQuery Enum")))
            (for _array_element_4 _outhits_2
              (bind (_bblockinghit _binitialoverlap _time _distance _location _impactpoint _normal _impactnormal _physmat _hitactor) (`GameplayStatics.BreakHitResult` _array_element_4))
              (if _bblockinghit
                (bind _asobject_entry_master (cast `/Game/Blueprints/Objects/ObjectEntry_Master` _hitactor))
                (cast `/Game/Blueprints/Objects/ObjectEntry_Container_FuseSlot` _hitactor
                  (:`CastFailed`
                    (if (`/Game/Blueprints/Objects/ObjectEntry_Master.IsMachine` _asobject_entry_master)
                      (set `/Game/Blueprints/Objects/ObjectEntry_Master.Machine_MainPowered` false _asobject_entry_master)
                      (bind _machinefuseparents (`/Game/Blueprints/Objects/ObjectEntry_Master.MachineFuseParents` _asobject_entry_master))
                      (if (not (`KismetArrayLibrary.Array_Contains` _machinefuseparents self))
                        (`KismetArrayLibrary.Array_Add` _machinefuseparents self))))))))))))
  (if (not (and (`self.IsPowerFlowing`) (`self.HasPowerCell`)))
    (`self.SetRoomsMachinePower` false true)))

(fn `SetRoomsMachinePower`
  (params (IsOn :type Boolean) (Init :type Boolean))
  (locals (InitRef :type Boolean :default true))
  (bind _connecteddevices (`self.ConnectedDevices`))
  (set `local.InitRef` Init)
  (if (not (`self.TransformerConnected`))
    (for _array_element (`self.ConnectedRooms`)
      (bind _bordervisual (`/Game/Blueprints/RoomGen_Master.BorderVisual` _array_element))
      (bind _returnvalue (`SceneComponent.K2_GetComponentLocation` _bordervisual))
      (bind (_x _y) (`KismetMathLibrary.BreakVector3f` (`BoxComponent.GetScaledBoxExtent` _bordervisual)))
      (bind _outhits (`KismetSystemLibrary.BoxTraceMultiForObjects` _returnvalue _returnvalue (`KismetMathLibrary.MakeVector` (* _x 1.25) (* _y 1.25) 500.0) (struct) (`|MakeArray` "ObjectTypeQuery8" "ObjectTypeQuery12" "ObjectTypeQuery11" :!type "EObjectTypeQuery Enum")))
      (for _array_element_2 _outhits
        (bind (_bblockinghit _binitialoverlap _time _distance _location _impactpoint _normal _impactnormal _physmat _hitactor) (`GameplayStatics.BreakHitResult` _array_element_2))
        (if _bblockinghit
          (bind _asobject_entry_master (cast `/Game/Blueprints/Objects/ObjectEntry_Master` _hitactor))
          (cast `/Game/Blueprints/Objects/ObjectEntry_Container_Generator` _hitactor
            (:`CastFailed`
              (cast `/Game/Blueprints/Objects/ObjectEntry_Container_Transformer` _hitactor
                (:`CastFailed`
                  (if (and (`/Game/Blueprints/Objects/ObjectEntry_Master.IsMachine` _asobject_entry_master) (not (`/Game/Blueprints/Objects/ObjectEntry_Master.Machine_MainPowered` _asobject_entry_master)))
                    (if (`local.InitRef`)
                      (`self.SetMachinePower` _asobject_entry_master IsOn)
                      (if (not (`KismetArrayLibrary.Array_Contains` _connecteddevices _asobject_entry_master))
                        (`KismetArrayLibrary.Array_Add` _connecteddevices _asobject_entry_master))
                      (elif IsOn
                        (`self.SetMachinePower` _asobject_entry_master IsOn :!label _label)
                        (else
                          (bind _afusehaspower (`self.FindFuseFlowingPower` _asobject_entry_master))
                          (if (not _afusehaspower)
                            (goto _label)))))))))))))))

(fn `UserConstructionScript`
  (`parent.UserConstructionScript`))