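; Interactable world container object holding an item list, which toggles open on interact and brings up the player's inventory, or shakes its lid when locked.
; SetContainerVisual sets the button material and lid transform from the Locked/Open state and clamps item stacks to data table maximums.
; Timelines animate the lid and shake, death clears the lock, and a DoAfterWorldGen macro polls until world generation completes.
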(event `self.ReceiveBeginPlay`
  (`parent.ReceiveBeginPlay`)
  (`self.SetContainerVisual`)
  (`/Game/Blueprints/BP_TopDownCharacter.SetItemUniqueNum` (`self.PlayerRef`) (`self.ItemInventoryList`)))

(event `OnThisContainerEdit`)

(event `self.OnInteract`
  (bind _playerref (`self.PlayerRef`))
  (bind _open (`self.Open`))
  (`parent.OnInteract`)
  (if (`/Game/Blueprints/BP_TopDownCharacter.MeleeAttacking` (`self.PlayerRef`))
    _
    (elif (`self.CanInteractWhenDead`)
      (if (`self.Locked`) :!label _label
        (`self.LockInteractShake`)
        (`self.SetContainerVisual`)
        (else
          (`/Game/Blueprints/BP_TopDownCharacter.Debug_PrintString_Internal` :`self` (`self.PlayerRef`) :`Text` "Container Opened" :`Colour` (struct :`R` 0.547744 :`G` 1.0 :`B` 0.611465 :`A` 1.0))
          (if (`/Game/Blueprints/BP_TopDownCharacter.InInventory` _playerref)
            (set `self.Open` (not _open))
            (else
              (if (not _open)
                (set `self.Open` true))
              (`/Game/Blueprints/BP_TopDownCharacter.Inv_SetInventoryVisuals` _playerref true)))
          (`self.SetContainerVisual`)
          (`self.Open/CloseContainerVisual` (`self.Open`))))
      (elif (not (`self.IsDead`))
        (goto _label)))))

(event `self.OnDeath`
  (`parent.OnDeath`)
  (set `self.Locked` false)
  (`self.SetContainerVisual`))

(event `Open/CloseContainerVisual`
  (params (Open :type Boolean :default true))
  (bind _containerlidvisual (`self.ContainerLidVisual`))
  ;[1 1 1] open close visuak
  (`/Engine/EditorBlueprintResources/StandardMacros.IsValid` (`SceneComponent.GetChildComponent` _containerlidvisual 0)
    (:`Is Valid`
      (if Open
        (bind (_direction _newtrack_0) (`Timeline|Open/Close` :!label _label_2)
          (:`Update`
            (`SceneComponent.K2_SetRelativeTransform` _containerlidvisual (`KismetMathLibrary.TLerp` (`self.CloseLidTransform`) (`self.OpenLidTransform`) _newtrack_0) false false)))
        (else
          (goto _label_2 :!via `Reverse`))))))

(event `LockInteractShake`
  (bind _containerlidvisual (`self.ContainerLidVisual`))
  (bind _openlidtransform_location (`KismetMathLibrary.BreakTransform` (`self.OpenLidTransform`)))
  (bind _closelidtransform_location (`KismetMathLibrary.BreakTransform` (`self.CloseLidTransform`)))
  (bind _returnvalue (* 1.0 -1.0))
  (bind _returnvalue_2 (* 1.0 0.5))
  (bind _returnvalue_3 (select `bool` (`self.Open`) :`false` _closelidtransform_location :`true` _openlidtransform_location))
  ;[1 1 1] lock shake
  (bind (_direction _x _y _z) (`Timeline|Timeline_0` :!via `PlayFromStart`)
    (:`Update`
      (`SceneComponent.K2_SetRelativeLocation` _containerlidvisual (+ _returnvalue_3 (`KismetMathLibrary.MakeVector` (`KismetMathLibrary.Lerp` 1.0 _returnvalue (`KismetMathLibrary.FClamp` _x -1.0)) (`KismetMathLibrary.Lerp` 1.0 _returnvalue (`KismetMathLibrary.FClamp` _y -1.0)) (`KismetMathLibrary.Lerp` _returnvalue_2 (* _returnvalue_2 -1.0) (`KismetMathLibrary.FClamp` _z -1.0)))) false false))
    (:`Finished`
      (`SceneComponent.K2_SetRelativeLocation` _containerlidvisual _returnvalue_3 false false))))

(fn `ClampItemListStack`
  (bind _iteminventorylist (`self.ItemInventoryList`))
  (for (_array_element _array_index) _iteminventorylist
    (bind (_itemid _uniquenumber _sizex _sizey _rotated _entryindex _stack _currentammo) (break `/Game/Blueprints/Data/ItemData_Struct` _array_element))
    (bind _returnvalue (`|GetDataTableRow` "/Game/Blueprints/Data/ItemID_Table.ItemID_Table" _itemid)
      (:`then`
        (`KismetArrayLibrary.Array_Set` _iteminventorylist _array_index (make `/Game/Blueprints/Data/ItemData_Struct` _itemid _uniquenumber _sizex _sizey _rotated _entryindex (`KismetMathLibrary.Clamp` _stack 0 (`.ItemMaxStack_36_F4AD081E4B2758961C11FA9F2A05277D` (break `/Game/Blueprints/Data/ItemID_Struct` _returnvalue))) _currentammo) true)))))

(fn `SetContainerVisual`
  (bind _containerlidvisual (`self.ContainerLidVisual`))
  (`PrimitiveComponent.SetMaterial` (`self.Button`) 0 (select `bool` (`self.Locked`) :`false` (select `bool` (`self.Open`) :`false` "/Game/Materials/BasicUnlit_Container_3.BasicUnlit_Container_3" :`true` "/Game/Materials/BasicUnlit_Container_1.BasicUnlit_Container_1" :!type "MaterialInterface Object Reference") :`true` "/Game/Materials/BasicUnlit_Container_2.BasicUnlit_Container_2"))
  (`self.ClampItemListStack`)
  (`/Engine/EditorBlueprintResources/StandardMacros.IsValid` (`SceneComponent.GetChildComponent` _containerlidvisual 0)
    (:`Is Valid`
      (`SceneComponent.K2_SetRelativeTransform` _containerlidvisual (select `bool` (`self.Open`) :`false` (`self.CloseLidTransform`) :`true` (`self.OpenLidTransform`)) false false))
    (:`Is Not Valid`
      _))
  (if (`self.Locked`)
    (set `self.Open` false)))

(fn `UserConstructionScript`
  (`parent.UserConstructionScript`)
  (`self.SetContainerVisual`))