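; Ticket kiosk container object, a powered-machine child that hooks its parent's power, edit, death and revive events to visual refreshes.
; Begin play waits on a macro that polls every few seconds until world generation completes, then runs the container edit event.
; Edits refresh visuals when the player reference is valid; death and revival refresh directly.
; The visual override checks generator or machine power, but both outcomes are empty beyond the parent call.
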(event `self.SetMachinePower`
  (params (PowerOn :type Boolean))
  (`parent.SetMachinePower` PowerOn)
  (`self.OnThisContainerEdit`))

(event `self.ReceiveBeginPlay`
  (`parent.ReceiveBeginPlay`)
  (`self.DoAfterWorldGen`
    (:`GenComplete`
      (`self.OnThisContainerEdit`))))

(event `self.OnThisContainerEdit`
  (`parent.OnThisContainerEdit`)
  (`/Engine/EditorBlueprintResources/StandardMacros.IsValid` (`self.PlayerRef`)
    (:`Is Valid`
      (`self.SetContainerVisual`))))

(event `self.SetContainerVisual`
  (`parent.SetContainerVisual`)
  (`/Engine/EditorBlueprintResources/StandardMacros.IsValid` (`self.WorldGenRef`)
    (:`Is Valid`
      (if (select `bool` (`self.Machine_MainPowered`) :`false` (`self.Machine_PowerOn`) :`true` (`/Game/Blueprints/WorldGen_Master.GeneratorPowered` (`self.WorldGenRef`)))
        _))))

(event `self.OnDeath`
  (`parent.OnDeath`)
  (`self.SetContainerVisual` :!label _label))

(event `self.OnRevived`
  (`parent.OnRevived`)
  (goto _label))

(fn `UserConstructionScript`
  (`parent.UserConstructionScript`))