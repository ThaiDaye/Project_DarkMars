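; Recharge station container object that powers on while it holds at least one item of ID 17, apparently a fuse.
; Container edits, and an initial check once world generation completes (polled by a delay-gate macro), toggle PowerOn and refresh visuals.
; The visual update shows the power beam when powered and alive, swaps a material on death or revival, and switches the inventory widget between fuse slot and recharge monitor.
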(event `self.ReceiveBeginPlay`
  (`parent.ReceiveBeginPlay`)
  (`self.DoAfterWorldGen`
    (:`GenComplete`
      (`self.OnThisContainerEdit`))))

(event `self.OnThisContainerEdit`
  (bind _poweron (`self.PowerOn`))
  (`parent.OnThisContainerEdit`)
  (bind (_found _foundatleastone) (`/Game/Blueprints/BP_TopDownCharacter.Inv_FindItem` (`self.PlayerRef`) "17" 1 self))
  (if _foundatleastone
    (if (not _poweron)
      (set `self.PowerOn` true)
      (`self.SetContainerVisual` :!label _label))
    (elif _poweron
      (set `self.PowerOn` false)
      (goto _label))))

(event `self.SetContainerVisual`
  (bind _powerbeam (`self.PowerBeam`))
  (bind _poweron (`self.PowerOn`))
  (bind _playerref (`self.PlayerRef`))
  (`parent.SetContainerVisual`)
  (`PrimitiveComponent.SetMaterial` (`self.visual`) 3 (select `bool` (`self.IsDead`) :`false` "/Game/Materials/BasicMaskMat_Cube8.BasicMaskMat_Cube8" :`true` "/Game/Materials/BasicMaskMat_Cube9.BasicMaskMat_Cube9" :!type "MaterialInterface Object Reference"))
  (if (`self.IsDead`)
    (`SceneComponent.SetVisibility` _powerbeam false false)
    (else
      (`SceneComponent.SetVisibility` _powerbeam _poweron false)))
  (set `self.InventoryBP` (select `bool` _poweron :`false` "/Game/Blueprints/Inventory/Inventroy_Instances/Inventory3DWidget_FuseSlot.Inventory3DWidget_FuseSlot_C" :`true` "/Game/Blueprints/Inventory/Inventroy_Instances/Inventory3DWidget_RechargeMonitor.Inventory3DWidget_RechargeMonitor_C" :!type "/Game/Blueprints/Inventory/Inventory3DWidget_Master Class Reference"))
  (`/Engine/EditorBlueprintResources/StandardMacros.IsValid` _playerref
    (:`Is Valid`
      (`/Game/Blueprints/BP_TopDownCharacter.Inv_TickSetContainerVisuals` _playerref true))))

(event `self.OnDeath`
  (`parent.OnDeath`)
  (`self.SetContainerVisual` :!label _label_2))

(event `self.OnRevived`
  (`parent.OnRevived`)
  (goto _label_2))

(fn `UserConstructionScript`
  (`parent.UserConstructionScript`))