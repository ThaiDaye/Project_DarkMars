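; A CCTV camera object that turns its eye to face the player while they are inside its detection sphere.
; Sphere overlaps set or clear the target while the camera is alive, and death clears it.
; A looping timer line-traces to the target and, if nothing blocks visibility, plays a timeline that eases the eye's pitch and yaw toward it, keeping roll at zero.
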(event `self.ReceiveBeginPlay`
  (`parent.ReceiveBeginPlay`)
  (`KismetSystemLibrary.K2_SetTimerDelegate` (delegate `LookAtTarget`) 2.0 true))

(event `LookAtTarget`
  (bind _target (`self.Target`))
  (bind _eyeoffset (`self.EyeOffset`))
  (bind _target_2 (`self.Target`))
  (bind _returnvalue (`SceneComponent.K2_GetComponentLocation` (`self.EyeOffset`)))
  (`/Engine/EditorBlueprintResources/StandardMacros.IsValid` _target
    (:`Is Valid`
      (bind _outhit (`KismetSystemLibrary.LineTraceSingle` _returnvalue (`SceneComponent.K2_GetComponentLocation` (`Actor.RootComponent` _target)) "TraceTypeQuery1"))
      (if (not (`GameplayStatics.BreakHitResult` _outhit))
        (set `self.TurnStart` _returnvalue)
        (bind (_direction _newtrack_0) (`Timeline|Timeline_0` :!via `PlayFromStart`)
          (:`Update`
            (`/Engine/EditorBlueprintResources/StandardMacros.IsValid` _target_2
              (:`Is Valid`
                (`SceneComponent.K2_SetWorldRotation` _eyeoffset (`KismetMathLibrary.MakeRotator` 0.0 (.pitch (`KismetMathLibrary.RLerp` (`SceneComponent.K2_GetComponentRotation` _eyeoffset) (`KismetMathLibrary.FindLookAtRotation` (`self.TurnStart`) (`SceneComponent.K2_GetComponentLocation` (`Actor.RootComponent` _target_2))) _newtrack_0 true)) (.yaw (`KismetMathLibrary.RLerp` (`SceneComponent.K2_GetComponentRotation` _eyeoffset) (`KismetMathLibrary.FindLookAtRotation` (`self.TurnStart`) (`SceneComponent.K2_GetComponentLocation` (`Actor.RootComponent` _target_2))) _newtrack_0 true))) false false)))))))))

(event `self.OnDeath`
  (`parent.OnDeath`)
  (set `self.Target` null))

(event `self.Sphere.OnComponentBeginOverlap`
  (params (OverlappedComponent :type "PrimitiveComponent Object Reference") (OtherActor :type "Actor Object Reference") (OtherComp :type "PrimitiveComponent Object Reference") (OtherBodyIndex :type Integer) (bFromSweep :type Boolean) (SweepResult :type "HitResult Structure (by ref)"))
  (if (`self.IsDead`)
    _
    (elif (== OtherActor (`self.PlayerRef`))
      (set `self.Target` OtherActor))))

(event `self.Sphere.OnComponentEndOverlap`
  (params (OverlappedComponent :type "PrimitiveComponent Object Reference") (OtherActor :type "Actor Object Reference") (OtherComp :type "PrimitiveComponent Object Reference") (OtherBodyIndex :type Integer))
  (if (`self.IsDead`)
    _
    (elif (== OtherActor (`self.Target`))
      (set `self.Target` null))))

(fn `UserConstructionScript`
  (`parent.UserConstructionScript`))