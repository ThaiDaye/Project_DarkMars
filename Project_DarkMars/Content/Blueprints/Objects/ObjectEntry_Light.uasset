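; Placeable light object that snaps itself to a wall or ceiling in the generated world and scales brightness by player proximity.
; On BeginPlay it registers with the player, then a gated delay loop polls until world generation completes.
; Four horizontal traces pick the nearest wall, with an upward trace as ceiling fallback.
; A looping timer then lerps spotlight intensity by horizontal player distance while lit and in range.
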(event `self.OnInteract`
  (`parent.OnInteract`))

(event `SetLightOn`
  (params (IsOn :type Boolean))
  (bind _spotlight (`self.SpotLight`))
  (bind _output_get (set `self.LightOn` IsOn))
  (if _output_get
    (`LightComponent.SetIntensity` _spotlight (`self.LightIntensity`))
    (else
      (`LightComponent.SetIntensity` _spotlight 0.0))))

(event `self.ReceiveBeginPlay`
  (`parent.ReceiveBeginPlay`)
  (`self.SetLightOn` (`self.LightOn`))
  (`/Game/Blueprints/BP_TopDownCharacter.RegisterLightEntry` (`self.PlayerRef`))
  (`self.DoAfterWorldGen`
    (:`GenComplete`
      (`self.SetStartingState` (`self.LightOnWall`))
      (`self.FadeLightIn`)
      (`KismetSystemLibrary.K2_SetTimerDelegate` (delegate `FadeLightIn`) 0.2 true))))

(event `FadeLightIn`
  (bind (_returnvalue_x _returnvalue_y) (`KismetMathLibrary.BreakVector` (`self.K2_GetActorLocation`)))
  (bind _playerref (`self.PlayerRef`))
  (bind (_returnvalue_x_2 _returnvalue_y_2) (`KismetMathLibrary.BreakVector` (`self.K2_GetActorLocation` _playerref)))
  (bind _lightcompactivationdistance (`/Game/Blueprints/BP_TopDownCharacter.LightCompActivationDistance` _playerref))
  (if (and (<= (`self.GetDistanceTo` _playerref) _lightcompactivationdistance) (`self.LightOn`))
    (bind _output_get (set `self.LightIntensity` (`KismetMathLibrary.Lerp` (`self.LightIntensityDefault`) 0.0 (`KismetMathLibrary.FClamp` (- (/ (`KismetMathLibrary.VSize` (- (`KismetMathLibrary.MakeVector` _returnvalue_x_2 _returnvalue_y_2) (`KismetMathLibrary.MakeVector` _returnvalue_x _returnvalue_y))) _lightcompactivationdistance) 0.2)))))
    (`LightComponent.SetIntensity` (`self.SpotLight`) _output_get)))

(fn `SetStartingState`
  (params (IsWall :type Boolean :default true) (WallPlaceHeight :type "Float (double-precision)" :default 250.0))
  (locals (FoundWall :type Boolean :default false) (Location :type "Vector Structure" :default (0.0 0.0 0.0)) (ImpactNormal :type "Vector Structure" :default (0.0 0.0 0.0)) (StartRot :type "Rotator Structure" :default (struct)) (ShortestDistance :type "Float (double-precision)"))
  (bind (_returnvalue_roll _returnvalue_pitch) (`KismetMathLibrary.BreakRotator` (`self.K2_GetActorRotation`)))
  (bind _returnvalue (`self.K2_GetActorLocation`))
  (bind _returnvalue_2 (`KismetMathLibrary.MakeVector` (.x (`self.K2_GetActorLocation`)) (.y (`self.K2_GetActorLocation`)) WallPlaceHeight))
  (bind _output_get (set `self.LightOnWall` IsWall))
  (`SceneComponent.K2_SetRelativeRotation` (`self.Offset`) (select `bool` (`self.LightOnWall`) :`false` (struct :`Pitch` -90.0) :!type "Rotator Structure") false false)
  (if _output_get
    (set `local.ShortestDistance` 99999999999.0)
    (for _index (range 4)
      (bind _outhit (`KismetSystemLibrary.LineTraceSingleForObjects` _returnvalue_2 (+ _returnvalue_2 (* (`KismetMathLibrary.Conv_RotatorToVector` (`KismetMathLibrary.MakeRotator` (.roll (struct)) (.pitch (struct)) (+ (.yaw (struct)) (* _index 90)))) 1000.0)) (`|MakeArray` "ObjectTypeQuery2" :!type "EObjectTypeQuery Enum")))
      (bind (_bblockinghit _binitialoverlap _time _distance _location _impactpoint _normal) (`GameplayStatics.BreakHitResult` _outhit))
      (if _bblockinghit
        (if (< _distance (`local.ShortestDistance`))
          (set `local.ShortestDistance` _distance)
          (set `local.FoundWall` true)
          (set `local.Location` _location)
          (set `local.ImpactNormal` _normal))))
    (if (`local.FoundWall`)
      (`self.K2_SetActorLocationAndRotation` (`local.Location`) (`KismetMathLibrary.MakeRotator` _returnvalue_roll _returnvalue_pitch (.yaw (`KismetMathLibrary.MakeRotFromX` (`local.ImpactNormal`)))))
      (`self.K2_SetActorLocation` (+ (* (`SceneComponent.GetForwardVector` (`self.Arrow`)) 2.5) (`local.Location`)))
      (else
        (set `self.LightOnWall` false)
        (`SceneComponent.K2_SetRelativeRotation` (`self.Offset`) (select `bool` (`self.LightOnWall`) :`false` (struct :`Pitch` -90.0) :!type "Rotator Structure") false false)
        (bind _outhit_2 (`KismetSystemLibrary.LineTraceSingleForObjects` _returnvalue (+ _returnvalue (0.0 0.0 1000.0)) (`|MakeArray` "ObjectTypeQuery1" :!type "EObjectTypeQuery Enum") :!label _label))
        (bind (_bblockinghit_2 _binitialoverlap_2 _time_2 _distance_2 _location_2) (`GameplayStatics.BreakHitResult` _outhit_2))
        (if _bblockinghit_2
          (`self.K2_SetActorLocation` _location_2))))
    (else
      (goto _label))))

(fn `UserConstructionScript`
  (`parent.UserConstructionScript`))