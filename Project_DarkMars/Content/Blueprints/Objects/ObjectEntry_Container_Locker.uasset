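; Locker container object that may start locked in the generated world.
; On BeginPlay it waits for world generation through a DoAfterWorldGen macro, which polls the generator's completion flag every few seconds using a gate and delay loop.
; Once generation completes, it rolls a low-weight locked chance from the world seed stream and refreshes the container visual.
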(event `self.ReceiveBeginPlay`
  (`parent.ReceiveBeginPlay`)
  (`self.DoAfterWorldGen`
    (:`GenComplete`
      (set `self.Locked` (`KismetMathLibrary.RandomBoolWithWeightFromStream` 0.15 (`/Game/Blueprints/WorldGen_Master.Seed` (`self.WorldGenRef`))))
      (`self.SetContainerVisual`))))

(fn `UserConstructionScript`
  (`parent.UserConstructionScript`))