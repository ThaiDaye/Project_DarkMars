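; Signpost object that labels directions to nearby main rooms in the generated world.
; After polling for world generation to finish, it traces outward through connected hallways to their doors, picking one per main room up to MaxSigns.
; Each target gets a stacked runtime-built board, snapped to whichever of ArrowL or ArrowR better faces that door.
; Boards show the room name on both sides, truncated by SignWidth.
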(event `self.ReceiveBeginPlay`
  (`parent.ReceiveBeginPlay`)
  (`self.DoAfterWorldGen`
    (:`GenComplete`
      (`self.GetTargets`)
      (`self.SetSignTargetsVisual`))))

(fn `GetTargets`
  (locals (SignDoors :type "Array of Actor Object Reference") (FoundRooms :type "Array of /Game/Blueprints/RoomGen_Master Object Reference") (ConnectedRoomsRef :type "Array of /Game/Blueprints/RoomGen_Master Object Reference"))
  (bind _returnvalue (enumliteral `EDrawDebugTrace` "None"))
  (bind _array (`|MakeArray` "ObjectTypeQuery13" :!type "EObjectTypeQuery Enum"))
  (bind _signtargets (`self.SignTargets`))
  (bind _signdoors (`local.SignDoors`))
  (bind _foundrooms (`local.FoundRooms`))
  (bind _connectedroomsref (`local.ConnectedRoomsRef`))
  (bind _returnvalue_2 (`KismetMathLibrary.MakeVector` (.x (`self.K2_GetActorLocation`)) (.y (`self.K2_GetActorLocation`)) 150.0))
  (`KismetArrayLibrary.Array_Clear` (`self.SignTargets`))
  (`KismetArrayLibrary.Array_Clear` (`local.ConnectedRoomsRef`))
  (`KismetArrayLibrary.Array_Clear` (`self.SignTargets_MainRoom`))
  (bind _outhits (`KismetSystemLibrary.SphereTraceMultiForObjects` :`Start` _returnvalue_2 :`End` _returnvalue_2 :`Radius` 150.0 :`ObjectTypes` _array :`DrawDebugType` _returnvalue :`DrawTime` 30.0))
  (for _array_element _outhits
    (bind _asroom_gen_master (cast `/Game/Blueprints/RoomGen_Master` (`.HitActor` (`GameplayStatics.BreakHitResult` _array_element))))
    (if (`/Game/Blueprints/RoomGen_Master.IsHallway` _asroom_gen_master)
      (if (not (`KismetArrayLibrary.Array_Contains` _connectedroomsref _asroom_gen_master))
        (`KismetArrayLibrary.Array_Add` _connectedroomsref _asroom_gen_master))))
  (for _array_element_2 (`local.ConnectedRoomsRef`)
    (`/Engine/EditorBlueprintResources/StandardMacros.IsValid` _array_element_2
      (:`Is Valid`
        (bind _bordervisual (`/Game/Blueprints/RoomGen_Master.BorderVisual` _array_element_2))
        (`/Engine/EditorBlueprintResources/StandardMacros.IsValid` _bordervisual
          (:`Is Valid`
            (bind _returnvalue_3 (`SceneComponent.K2_GetComponentLocation` _bordervisual))
            (bind (_x _y) (`KismetMathLibrary.BreakVector3f` (`BoxComponent.GetScaledBoxExtent` _bordervisual)))
            (bind _outhits_2 (`KismetSystemLibrary.BoxTraceMultiForObjects` :`Start` _returnvalue_3 :`End` _returnvalue_3 :`HalfSize` (`KismetMathLibrary.MakeVector` (* _x 1.0) (* _y 1.0) 500.0) :`ObjectTypes` _array :`DrawDebugType` _returnvalue :`DrawTime` 30.0))
            (for _array_element_3 _outhits_2
              (bind (_bblockinghit _binitialoverlap _time _distance _location _impactpoint _normal _impactnormal _physmat _hitactor) (`GameplayStatics.BreakHitResult` _array_element_3))
              (if _bblockinghit
                (bind _asroom_gen_master_2 (cast `/Game/Blueprints/RoomGen_Master` _hitactor))
                (if (`/Game/Blueprints/RoomGen_Master.IsHallway` _asroom_gen_master_2)
                  (if (not (`KismetArrayLibrary.Array_Contains` (`local.ConnectedRoomsRef`) _asroom_gen_master_2))
                    (`KismetArrayLibrary.Array_Add` (`local.ConnectedRoomsRef`) _asroom_gen_master_2))))))))))
  (for _array_element_4 (`local.ConnectedRoomsRef`)
    (`/Engine/EditorBlueprintResources/StandardMacros.IsValid` _array_element_4
      (:`Is Valid`
        (bind _bordervisual_2 (`/Game/Blueprints/RoomGen_Master.BorderVisual` _array_element_4))
        (`/Engine/EditorBlueprintResources/StandardMacros.IsValid` _bordervisual_2
          (:`Is Valid`
            (bind _returnvalue_4 (`SceneComponent.K2_GetComponentLocation` _bordervisual_2))
            (bind (_x_2 _y_2) (`KismetMathLibrary.BreakVector3f` (`BoxComponent.GetScaledBoxExtent` _bordervisual_2)))
            (bind _outhits_3 (`KismetSystemLibrary.BoxTraceMultiForObjects` :`Start` _returnvalue_4 :`End` _returnvalue_4 :`HalfSize` (`KismetMathLibrary.MakeVector` (* _x_2 1.25) (* _y_2 1.25) 500.0) :`ObjectTypes` (`|MakeArray` "ObjectTypeQuery8" :!type "EObjectTypeQuery Enum") :`DrawDebugType` _returnvalue :`DrawTime` 30.0))
            (for _array_element_5 _outhits_3
              (bind (_bblockinghit_2 _binitialoverlap_2 _time_2 _distance_2 _location_2 _impactpoint_2 _normal_2 _impactnormal_2 _physmat_2 _hitactor_2) (`GameplayStatics.BreakHitResult` _array_element_5))
              (if _bblockinghit_2
                (bind _asobject_entry_door (cast `/Game/Blueprints/Objects/ObjectEntry_Door` _hitactor_2))
                (`/Engine/EditorBlueprintResources/StandardMacros.IsValid` (`/Game/Blueprints/Objects/ObjectEntry_Master.ParentRoomRef` _asobject_entry_door)
                  (:`Is Valid`
                    (if (`KismetArrayLibrary.Array_Contains` _signdoors _asobject_entry_door)
                      _
                      (elif (not (`KismetArrayLibrary.Array_Contains` _signdoors (`/Game/Blueprints/Objects/ObjectEntry_Door.DoorPartner` _asobject_entry_door)))
                        (`KismetArrayLibrary.Array_Add` _signdoors _asobject_entry_door))))))))))))
  (`KismetArrayLibrary.Array_Clear` (`local.FoundRooms`))
  (for _array_element_6 (`local.SignDoors`)
    (bind _returnvalue_5 (`KismetMathLibrary.MakeVector` (.x (`self.K2_GetActorLocation` _array_element_6)) (.y (`self.K2_GetActorLocation` _array_element_6)) 150.0))
    (bind _outhits_4 (`KismetSystemLibrary.SphereTraceMultiForObjects` :`Start` _returnvalue_5 :`End` _returnvalue_5 :`Radius` 250.0 :`ObjectTypes` (`|MakeArray` "ObjectTypeQuery13" :!type "EObjectTypeQuery Enum") :`DrawTime` 30.0))
    (for _array_element_7 _outhits_4
      (bind (_bblockinghit_3 _binitialoverlap_3 _time_3 _distance_3 _location_3 _impactpoint_3 _normal_3 _impactnormal_3 _physmat_3 _hitactor_3) (`GameplayStatics.BreakHitResult` _array_element_7))
      (if _bblockinghit_3
        (bind _asroom_gen_master_3 (cast `/Game/Blueprints/RoomGen_Master` _hitactor_3))
        (if (`/Game/Blueprints/RoomGen_Master.IsMainRoom` _asroom_gen_master_3)
          (if (`KismetArrayLibrary.Array_Contains` _foundrooms _asroom_gen_master_3)
            _
            (elif (`KismetArrayLibrary.Array_Contains` _signtargets _array_element_6)
              _
              (elif (not (>= (`KismetArrayLibrary.Array_Length` _signtargets) (`self.MaxSigns`)))
                (`KismetArrayLibrary.Array_Add` _signtargets _array_element_6)
                (`KismetArrayLibrary.Array_Add` (`self.SignTargets_MainRoom`) _asroom_gen_master_3)
                (`KismetArrayLibrary.Array_Add` _foundrooms _asroom_gen_master_3)))))))))

(fn `SetSignTargetsVisual`
  (locals (StringCutLength :type Integer :default 0))
  (bind _arrowl (`self.ArrowL`))
  (bind _arrowr (`self.ArrowR`))
  (bind _signoffset (`self.SignOffset`))
  (bind _returnvalue (+ _signoffset (* (`self.SignWidth`) 30.0)))
  (for (_array_element _array_index) (`self.SignTargets`)
    (`/Engine/EditorBlueprintResources/StandardMacros.IsValid` _array_element
      (:`Is Valid`
        (bind _returnvalue_2 (`AddComponent|NODE_AddArrowComponent-0` :`RelativeTransform` (`KismetMathLibrary.MakeTransform` (+ (0.0 0.0 100.0) (`KismetMathLibrary.MakeVector` 0.0 0.0 (* _array_index 50.0))) (struct) (1.75 1.75 1.75))))
        (bind _returnvalue_3 (`KismetMathLibrary.MakeVector` (.x (+ (* (`KismetMathLibrary.GetForwardVector` (`KismetMathLibrary.MakeRotator` (.roll (`SceneComponent.K2_GetComponentRotation` _returnvalue_2)) (.pitch (`SceneComponent.K2_GetComponentRotation` _returnvalue_2)) (.yaw (`KismetMathLibrary.FindLookAtRotation` (`KismetMathLibrary.MakeVector` (.x (`self.K2_GetActorLocation`)) (.y (`self.K2_GetActorLocation`))) (`KismetMathLibrary.MakeVector` (.x (`self.K2_GetActorLocation` _array_element)) (.y (`self.K2_GetActorLocation` _array_element))))))) 100.0) (`SceneComponent.K2_GetComponentLocation` _returnvalue_2))) (.y (+ (* (`KismetMathLibrary.GetForwardVector` (`KismetMathLibrary.MakeRotator` (.roll (`SceneComponent.K2_GetComponentRotation` _returnvalue_2)) (.pitch (`SceneComponent.K2_GetComponentRotation` _returnvalue_2)) (.yaw (`KismetMathLibrary.FindLookAtRotation` (`KismetMathLibrary.MakeVector` (.x (`self.K2_GetActorLocation`)) (.y (`self.K2_GetActorLocation`))) (`KismetMathLibrary.MakeVector` (.x (`self.K2_GetActorLocation` _array_element)) (.y (`self.K2_GetActorLocation` _array_element))))))) 100.0) (`SceneComponent.K2_GetComponentLocation` _returnvalue_2)))))
        (`SceneComponent.K2_SetWorldRotation` _returnvalue_2 (select `bool` (< (`KismetMathLibrary.VSize` (- _returnvalue_3 (`KismetMathLibrary.MakeVector` (.x (+ (* (`SceneComponent.GetForwardVector` _arrowr) 100.0) (`SceneComponent.K2_GetComponentLocation` _arrowr))) (.y (+ (* (`SceneComponent.GetForwardVector` _arrowr) 100.0) (`SceneComponent.K2_GetComponentLocation` _arrowr)))))) (`KismetMathLibrary.VSize` (- _returnvalue_3 (`KismetMathLibrary.MakeVector` (.x (+ (* (`SceneComponent.GetForwardVector` _arrowl) 100.0) (`SceneComponent.K2_GetComponentLocation` _arrowl))) (.y (+ (* (`SceneComponent.GetForwardVector` _arrowl) 100.0) (`SceneComponent.K2_GetComponentLocation` _arrowl))))))) :`false` (`SceneComponent.K2_GetComponentRotation` _arrowl) :`true` (`SceneComponent.K2_GetComponentRotation` _arrowr)) false false)
        (`SceneComponent.K2_AttachToComponent` _returnvalue_2 (`self.Offset`) "None" "KeepRelative" "KeepRelative" "KeepRelative" true)
        (bind _returnvalue_4 (`AddComponent|NODE_AddStaticMeshComponent-0` :`bManualAttachment` true :`RelativeTransform` (`KismetMathLibrary.MakeTransform` (`KismetMathLibrary.MakeVector` _signoffset) (struct :`Yaw` -90.0 :`Roll` 90.0) (`KismetMathLibrary.MakeVector` 0.1 0.45 (`self.SignWidth`)))))
        (`SceneComponent.K2_AttachToComponent` _returnvalue_4 _returnvalue_2 "None" "KeepRelative" "KeepRelative" "KeepWorld" true)
        (bind _returnvalue_5 (`AddComponent|NODE_AddTextRenderComponent-0` :`bManualAttachment` true :`RelativeTransform` (`KismetMathLibrary.MakeTransform` (`KismetMathLibrary.MakeVector` _returnvalue 3.5) (struct :`Yaw` 90.0) (0.33 0.33 0.33))))
        (bind _returnvalue_6 (`AddComponent|NODE_AddTextRenderComponent-1` :`bManualAttachment` true :`RelativeTransform` (`KismetMathLibrary.MakeTransform` (`KismetMathLibrary.MakeVector` _returnvalue -3.5) (struct :`Yaw` -90.0) (0.33 0.33 0.33))))
        (`SceneComponent.K2_AttachToComponent` _returnvalue_5 _returnvalue_2 "None" "KeepRelative" "KeepRelative" "KeepRelative" true)
        (`SceneComponent.K2_AttachToComponent` _returnvalue_6 _returnvalue_2 "None" "KeepRelative" "KeepRelative" "KeepRelative" true)
        (bind _asroom_gen_master (cast `/Game/Blueprints/RoomGen_Master` (`|GetArrayItem` (`self.SignTargets_MainRoom`) _array_index)))
        (bind _output_get (set `local.StringCutLength` (`KismetMathLibrary.FTrunc` (`KismetMathLibrary.Lerp` 0.0 22.0 (/ (`self.SignWidth`) 1.45)))))
        (bind _roomname (`/Game/Blueprints/RoomGen_Master.RoomName` _asroom_gen_master))
        (bind _returnvalue_7 (`KismetTextLibrary.Conv_StringToText` (`KismetStringLibrary.Concat_StrStr` (`KismetStringLibrary.GetSubstring` _roomname 0 _output_get) (select `bool` (>= _output_get (`KismetStringLibrary.Len` _roomname)) :`false` "..."))))
        (`TextRenderComponent.K2_SetText` _returnvalue_5 _returnvalue_7)
        (`TextRenderComponent.K2_SetText` _returnvalue_6 _returnvalue_7)))))

(fn `UserConstructionScript`
  (`parent.UserConstructionScript`)
  (`self.SetSignTargetsVisual`))