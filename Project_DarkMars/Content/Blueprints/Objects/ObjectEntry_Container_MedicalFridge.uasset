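; Medical fridge container object that fills its interior with randomized decorative vials.
; On construction and again at BeginPlay, SetInternalVisuals destroys the previous vial components and rebuilds them from the VisualBottlesSlots instance transforms.
; Each slot has a weighted random chance to spawn a static mesh with jittered position and yaw, relative to Offset.
; Mesh and second-slot material are random picks, with duplicated Select options biasing the odds.
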(event `self.ReceiveBeginPlay`
  (`parent.ReceiveBeginPlay`)
  (`self.SetInternalVisuals`))

(fn `SetInternalVisuals`
  (bind _visualbottlesslots (`self.VisualBottlesSlots`))
  (bind _returnvalue (`SceneComponent.K2_GetComponentToWorld` (`self.Offset`)))
  (for _array_element (`self.InternalVisuals`)
    (`/Engine/EditorBlueprintResources/StandardMacros.IsValid` _array_element
      (:`Is Valid`
        (`ActorComponent.K2_DestroyComponent` _array_element))))
  (for _index (range (`InstancedStaticMeshComponent.GetInstanceCount` _visualbottlesslots))
    (if (`KismetMathLibrary.RandomBoolWithWeight` 0.5)
      (bind _outinstancetransform (`InstancedStaticMeshComponent.GetInstanceTransform` _visualbottlesslots _index true))
      (bind _returnvalue_2 (`AddComponent|NODE_AddStaticMeshComponent-0` :`RelativeTransform` (`KismetMathLibrary.MakeTransform` (`KismetMathLibrary.MakeVector` (+ (.x (`KismetMathLibrary.InverseTransformLocation` _returnvalue (.location _outinstancetransform))) (`KismetMathLibrary.RandomFloatInRange` -10.0 10.0)) (+ (.y (`KismetMathLibrary.InverseTransformLocation` _returnvalue (.location _outinstancetransform))) (`KismetMathLibrary.RandomFloatInRange` -10.0 10.0)) (.z (`KismetMathLibrary.InverseTransformLocation` _returnvalue (.location _outinstancetransform)))) (`KismetMathLibrary.MakeRotator` (.roll (`KismetMathLibrary.InverseTransformRotation` _returnvalue (.rotation _outinstancetransform))) (.pitch (`KismetMathLibrary.InverseTransformRotation` _returnvalue (.rotation _outinstancetransform))) (+ (`KismetMathLibrary.RandomFloatInRange` -45.0 45.0) (.yaw (`KismetMathLibrary.InverseTransformRotation` _returnvalue (.rotation _outinstancetransform))))))))
      (`SceneComponent.K2_AttachToComponent` (`self.Offset`) _returnvalue_2 "None" "KeepWorld" "KeepWorld" "KeepWorld" true)
      (`KismetArrayLibrary.Array_Add` (`self.InternalVisuals`) _returnvalue_2)
      (`StaticMeshComponent.SetStaticMesh` _returnvalue_2 (select `int` (`KismetMathLibrary.RandomIntegerInRange` 0 10) :`0` "/Game/Meshes/OpenSourceProps/GlassVials/Vial_1.Vial_1" :`1` "/Game/Meshes/OpenSourceProps/GlassVials/Vial_2.Vial_2" :`2` "/Game/Meshes/OpenSourceProps/GlassVials/Vial_3.Vial_3" :`3` "/Game/Meshes/OpenSourceProps/GlassVials/Vial_4.Vial_4" :`4` "/Game/Meshes/OpenSourceProps/GlassVials/Vial_5.Vial_5" :`5` "/Game/Meshes/OpenSourceProps/GlassVials/Vial_6.Vial_6" :`6` "/Game/Meshes/OpenSourceProps/GlassVials/Vial_7.Vial_7" :`7` "/Game/Meshes/OpenSourceProps/GlassVials/Vial_1.Vial_1" :`8` "/Game/Meshes/OpenSourceProps/GlassVials/Vial_1.Vial_1" :`9` "/Game/Meshes/OpenSourceProps/GlassVials/Vial_6.Vial_6" :`10` "/Game/Meshes/OpenSourceProps/GlassVials/Vial_6.Vial_6" :!type "StaticMesh Object Reference"))
      (`PrimitiveComponent.SetMaterial` _returnvalue_2 0 "/Game/ScienceLab/Materials/Furniture/MI_Furniture_Glass.MI_Furniture_Glass")
      (`PrimitiveComponent.SetMaterial` _returnvalue_2 2 "/Game/Materials/BasicMat_Master_Item_1.BasicMat_Master_Item_1")
      (`PrimitiveComponent.SetMaterial` _returnvalue_2 1 (select `int` (`KismetMathLibrary.RandomIntegerInRange` 0 7) :`0` "/Game/Materials/BasicUnlit_Container_1.BasicUnlit_Container_1" :`1` "/Game/Materials/BasicUnlit_Container_1.BasicUnlit_Container_1" :`2` "/Game/Materials/BasicUnlit_Container_3.BasicUnlit_Container_3" :`3` "/Game/Materials/BasicUnlit_Container_2.BasicUnlit_Container_2" :`4` "/Game/Materials/BasicUnlit_Container_1.BasicUnlit_Container_1" :`5` "/Game/Materials/BasicUnlit_Container_1.BasicUnlit_Container_1" :`6` "/Game/Materials/BasicUnlit_Container_1.BasicUnlit_Container_1" :`7` "/Game/Materials/BasicUnlit_Container_1.BasicUnlit_Container_1" :!type "MaterialInterface Object Reference")))))

(fn `UserConstructionScript`
  (`parent.UserConstructionScript`)
  (`self.SetInternalVisuals`))