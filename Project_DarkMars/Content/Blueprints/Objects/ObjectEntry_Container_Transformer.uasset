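; Power transformer container that links to nearby fuse slots and passes power state to its connected generator.
; After world gen, it sphere-traces for unclaimed slots outside dungeon or locked rooms, shuffles them, claims a seeded random count, and randomly adds items, slug spawn markers or breakage.
; Power can be toggled, drops on death or when any linked fuse stops flowing, and drives indicator materials.
; A one-time reward refills player suit power.
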(event `RewardGiven`
  (params (Reward :type Integer))
  (bind _playerref (`self.PlayerRef`))
  ;[1 0 0] Comment
  (if (not (`self.RewardObtained`))
    (set `self.RewardObtained` true)
    (switch `int` Reward
      (:`0`
        _)
      (:`1`
        _))
    ;;[1 1 1] suit power
    (`/Game/Blueprints/BP_TopDownCharacter.Power_AddPlayerPower` _playerref (`/Game/Blueprints/BP_TopDownCharacter.PlayerPowerMax` _playerref))))

(event `self.ReceiveBeginPlay`
  (`parent.ReceiveBeginPlay`)
  (`self.DoAfterWorldGen`
    (:`GenComplete`
      (`KismetSystemLibrary.Delay` 5.0)
      (set `self.DesiredConnectionCount` (`KismetMathLibrary.RandomIntegerInRangeFromStream` (`self.DesiredConnectionCount_Min`) (`self.DesiredConnectionCount`) (`/Game/Blueprints/WorldGen_Master.Seed` (`self.WorldGenRef`))))
      (`self.FindFuses`))))

(event `ToggleOnPower`
  (if (`self.IsPowerOn`)
    (set `self.IsPowerOn` false :!label _label)
    (elif (`self.IsDead`)
      (goto _label)
      (else
        (set `self.IsPowerOn` true)
        (for _array_element (`self.ConnectedFuses`)
          (`self.MarkObjectOnRadar` _array_element false)))))
  (`self.SetContainerVisual`))

(event `FindFuses`
  (bind _inrangeref (`self.InRangeRef`))
  (bind _playerref (`self.PlayerRef`))
  (bind _returnvalue (`SceneComponent.K2_GetComponentLocation` (`self.Button`)))
  (bind _outhits (`KismetSystemLibrary.SphereTraceMultiForObjects` _returnvalue _returnvalue (`self.ConnectionDistance`) (`|MakeArray` "ObjectTypeQuery8" :!type "EObjectTypeQuery Enum")))
  (set `self.InRangeRef` _outhits)
  (`KismetArrayLibrary.Array_Shuffle` _inrangeref)
  (for _array_element _inrangeref
    (if (not (>= (`self.Desired Connection CountRef`) (`self.DesiredConnectionCount`)))
      (bind (_bblockinghit _binitialoverlap _time _distance _location _impactpoint _normal _impactnormal _physmat _hitactor) (`GameplayStatics.BreakHitResult` _array_element))
      (if _bblockinghit
        (bind _asobject_entry_container_fuse_slot (cast `/Game/Blueprints/Objects/ObjectEntry_Container_FuseSlot` _hitactor))
        (set `self.FoundError` false)
        (for _array_element_2 (`/Game/Blueprints/Objects/ObjectEntry_Container_FuseSlot.ConnectedRooms` _asobject_entry_container_fuse_slot)
          (if (or (`/Game/Blueprints/RoomGen_Master.IsDungeonRoom` _array_element_2) (`/Game/Blueprints/RoomGen_Master.IsDungeonSubRoom` _array_element_2) (`/Game/Blueprints/RoomGen_Master.DoorsLocked` _array_element_2))
            (set `self.FoundError` true)))
        (if (not (`self.FoundError`))
          (`/Engine/EditorBlueprintResources/StandardMacros.IsValid` (`/Game/Blueprints/Objects/ObjectEntry_Container_FuseSlot.ConnectedTransformer` _asobject_entry_container_fuse_slot)
            (:`Is Not Valid`
              (bind (_foundrooms _valid) (`/Game/Blueprints/WorldGen_Master.GetRoomsAtLocation` (`self.WorldGenRef`) (`self.K2_GetActorLocation` _asobject_entry_container_fuse_slot)))
              (if _valid
                (set `/Game/Blueprints/Objects/ObjectEntry_Container_FuseSlot.ConnectedTransformer` self _asobject_entry_container_fuse_slot)
                (set `/Game/Blueprints/Objects/ObjectEntry_Container_FuseSlot.TransformerConnected` true _asobject_entry_container_fuse_slot)
                (`KismetArrayLibrary.Array_Add` (`self.ConnectedFuses`) _asobject_entry_container_fuse_slot)
                (`|ExecutionSequence`
                  (:`then_0`
                    ;[1 1 1] set fuse board variables
                    (if (`KismetMathLibrary.RandomBoolWithWeightFromStream` 0.5 (`/Game/Blueprints/WorldGen_Master.Seed` (`self.WorldGenRef`)))
                      (`/Game/Blueprints/BP_TopDownCharacter.Inv_GiveItem` _playerref _asobject_entry_container_fuse_slot "15" 1 false 0 0 false -1 null false)
                      (elif (`KismetMathLibrary.RandomBoolWithWeightFromStream` 0.2 (`/Game/Blueprints/WorldGen_Master.Seed` (`self.WorldGenRef`)))
                        (`/Game/Blueprints/BP_TopDownCharacter.Inv_GiveItem` _playerref _asobject_entry_container_fuse_slot "17" 1 false 0 0 false -1 null false))))
                  (:`then_1`
                    (if (`KismetMathLibrary.RandomBoolWithWeightFromStream` 0.15 (`/Game/Blueprints/WorldGen_Master.Seed` (`self.WorldGenRef`)))
                      (if (`|EnumEquality` (`/Game/Blueprints/Objects/ObjectEntry_Master.ObjectStartState` _asobject_entry_container_fuse_slot) "NewEnumerator1")
                        (`|SpawnActorFromClass` "/Game/Blueprints/Enemies/EnemyMarkerGen_Master.EnemyMarkerGen_Master_C" (`KismetMathLibrary.MakeTransform` (`SceneComponent.K2_GetComponentLocation` (`/Game/Blueprints/Objects/ObjectEntry_Container_FuseSlot.ArcStart` _asobject_entry_container_fuse_slot))) "Undefined" "OverrideRootScale" null "/Game/Blueprints/Enemies/EnemyEntry_Slug.EnemyEntry_Slug_C" true false false null))))
                  (:`then_2`
                    (if (`KismetMathLibrary.RandomBoolWithWeightFromStream` 0.15 (`/Game/Blueprints/WorldGen_Master.Seed` (`self.WorldGenRef`)))
                      (set `/Game/Blueprints/Objects/ObjectEntry_Master.Health` 0.0 _asobject_entry_container_fuse_slot)
                      (`self.OnDeath` _asobject_entry_container_fuse_slot)))
                  (:`then_3`
                    (`self.OnThisContainerEdit` _asobject_entry_container_fuse_slot)
                    (`self.SetContainerVisual` _asobject_entry_container_fuse_slot)
                    (`/Engine/EditorBlueprintResources/StandardMacros.IncrementInt` (`self.Desired Connection CountRef`))))))))))))

(event `self.OnOpenCloseContainerVisual`
  (params (Open :type Boolean))
  (bind _containerlidvisual_l (`self.ContainerLidVisual_L`))
  ;[1 1 1] open close visuak
  (`/Engine/EditorBlueprintResources/StandardMacros.IsValid` (`SceneComponent.GetChildComponent` _containerlidvisual_l 0)
    (:`Is Valid`
      (if Open
        (bind (_direction _newtrack_0) (`Timeline|Timeline_1` :!label _label_2)
          (:`Update`
            (`SceneComponent.K2_SetRelativeTransform` _containerlidvisual_l (`KismetMathLibrary.TLerp` (`self.CloseLidTransform_2`) (`self.OpenLidTransform_2`) _newtrack_0) false false)))
        (else
          (goto _label_2 :!via `Reverse`))))))

(event `self.OnDeath`
  (`parent.OnDeath`)
  (set `self.IsPowerOn` false)
  (`self.SetContainerVisual`))

(event `self.SetContainerVisual`
  (bind _visual (`self.visual`))
  (bind _connectedfuses (`self.ConnectedFuses`))
  (bind _connectedgenerator (`self.ConnectedGenerator`))
  (bind _returnvalue (select `bool` (`self.IsPowerOn`) :`false` "/Game/Materials/BasicUnlit_Container_2.BasicUnlit_Container_2" :`true` (select `bool` (`self.IsPowerFlowing`) :`false` "/Game/Materials/BasicUnlit_Container_2.BasicUnlit_Container_2" :`true` "/Game/Materials/BasicUnlit_Container_1.BasicUnlit_Container_1" :!type "MaterialInterface Object Reference")))
  (`parent.SetContainerVisual`)
  (if (`KismetArrayLibrary.Array_IsValidIndex` _connectedfuses)
    (set `self.IsPowerFlowing` true)
    (for _array_element _connectedfuses
      (if (not (`/Game/Blueprints/Objects/ObjectEntry_Container_FuseSlot.IsPowerFlowing` _array_element))
        (set `self.IsPowerFlowing` false)))
    (if (`self.IsPowerFlowing`)
      _
      (elif (`self.IsPowerOn`)
        (set `self.IsPowerOn` false))))
  (`PrimitiveComponent.SetMaterial` _visual 4 _returnvalue)
  (`PrimitiveComponent.SetMaterial` _visual 5 _returnvalue)
  (`PrimitiveComponent.SetMaterial` (`self.visual2`) 1 _returnvalue)
  (`PrimitiveComponent.SetMaterial` (`self.visual1`) 1 _returnvalue)
  (`/Engine/EditorBlueprintResources/StandardMacros.IsValid` _connectedgenerator
    (:`Is Valid`
      (`self.SetContainerVisual` _connectedgenerator))))

(fn `UserConstructionScript`
  (`parent.UserConstructionScript`))