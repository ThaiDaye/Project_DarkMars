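; A safe container object entry that places itself once world generation finishes.
; On BeginPlay a DoAfterWorldGen macro polls the world generator every three seconds through a gate until generation completes.
; It then calls SetStartState with a wall-relative placement, rotating to the surface within a check radius, with back-destroy enabled.
; Construction only runs the parent script.
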(event `self.ReceiveBeginPlay`
  (`parent.ReceiveBeginPlay`)
  (`self.DoAfterWorldGen`
    (:`GenComplete`
      (`self.SetStartState__` "NewEnumerator3" "NewEnumerator0" 50.0 true 500.0 true))))

(fn `UserConstructionScript`
  (`parent.UserConstructionScript`))