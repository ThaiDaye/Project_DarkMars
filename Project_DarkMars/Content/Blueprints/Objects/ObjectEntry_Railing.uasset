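; A railing map object that trims its own side pieces to fit its neighbors in the generated world.
; After BeginPlay, the DoAfterWorldGen macro polls WorldGenRef through a gate and delay loop until generation completes.
; SetAdjacentRailings then looks up map entries one step left, forward and right of its Arrow, destroying the matching visual component wherever the entry ID is non-zero.
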(event `self.ReceiveBeginPlay`
  (`parent.ReceiveBeginPlay`)
  (`self.DoAfterWorldGen`
    (:`GenComplete`
      (`self.SetAdjacentRailings`))))

(event `SetAdjacentRailings`
  (bind _returnvalue (`self.K2_GetActorLocation`))
  (bind _arrow (`self.Arrow`))
  (bind _returnvalue_2 (`SceneComponent.GetRightVector` _arrow))
  (for _index (range 3)
    (bind (_x _y _id) (`/Game/Blueprints/WorldGen_Master.GetMapEntryAtLocation` (`self.WorldGenRef`) (select `int` _index :`0` (+ _returnvalue (* _returnvalue_2 -100.0)) :`1` (+ _returnvalue (* (`SceneComponent.GetForwardVector` _arrow) 100.0)) :`2` (+ _returnvalue (* _returnvalue_2 100.0)))))
    (if (not (== _id 0))
      (`ActorComponent.K2_DestroyComponent` (select `int` _index :`0` (`self.visualE`) :`1` (`self.visualS`) :`2` (`self.visualW`))))))

(fn `UserConstructionScript`
  (`parent.UserConstructionScript`))