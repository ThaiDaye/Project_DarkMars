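; Automatic door object that opens while the player or an enemy capsule overlaps its Sphere and closes when they leave.
; Overlap events and interaction rerun the proximity check, which plays or reverses a timeline that shrinks the Door mesh's Z scale to open it.
; A linked DoorPartner mirrors opening and closing, and death hides the door, disables its collision and deals full-health damage to the partner.
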(event `self.ReceiveBeginPlay`
  ;[1 1 1] init
  (`parent.ReceiveBeginPlay`))

(event `self.Sphere.OnComponentBeginOverlap`
  (params (OverlappedComponent :type "PrimitiveComponent Object Reference") (OtherActor :type "Actor Object Reference") (OtherComp :type "PrimitiveComponent Object Reference") (OtherBodyIndex :type Integer) (bFromSweep :type Boolean) (SweepResult :type "HitResult Structure (by ref)"))
  ;[1 1 1] on interact
  (`self.TickAutoOpen` :!label _label))

(event `self.OnInteract`
  ;[1 1 1] on interact
  (`parent.OnInteract`)
  (if (not (`self.Transitioning`))
    (set `self.Open` (not (`self.Open`)))
    (goto _label)))

(event `self.Sphere.OnComponentEndOverlap`
  (params (OverlappedComponent :type "PrimitiveComponent Object Reference") (OtherActor :type "Actor Object Reference") (OtherComp :type "PrimitiveComponent Object Reference") (OtherBodyIndex :type Integer))
  ;[1 1 1] on interact
  (goto _label))

(event `self.OnDeath`
  (bind _doorpartner (`self.DoorPartner`))
  (bind _door (`self.Door`))
  ;[1 1 1] on death
  (`parent.OnDeath`)
  (`PrimitiveComponent.SetCollisionEnabled` _door "NoCollision")
  (`SceneComponent.SetVisibility` _door false true)
  (if (not (`/Game/Blueprints/Objects/ObjectEntry_Master.IsDead` _doorpartner))
    (`self.TakeDamage_Object` _doorpartner (`/Game/Blueprints/Objects/ObjectEntry_Master.Health_TotalMax` _doorpartner) 1.0)))

(event `OpenDoor`
  (bind _door (`self.Door`))
  (bind (_returnvalue_x _returnvalue_y) (`KismetMathLibrary.BreakVector` (`SceneComponent.K2_GetComponentScale` _door)))
  ;[1 1 1] open/close
  (set `self.Transitioning` true)
  (bind (_direction _newtrack_0) (`Timeline|Timeline_0` :!label _label_2)
    (:`Update`
      (`SceneComponent.SetWorldScale3D` _door (`KismetMathLibrary.MakeVector` _returnvalue_x _returnvalue_y (`KismetMathLibrary.Lerp` (* (`self.Door Width`) 0.01) 0.01 _newtrack_0))))
    (:`Finished`
      (set `self.Transitioning` false))))

(event `CloseDoor`
  ;[1 1 1] open/close
  (set `self.Transitioning` true)
  (goto _label_2 :!via `Reverse`))

(event `TickAutoOpen`
  (bind _open (`self.Open`))
  (bind _sphere (`self.Sphere`))
  (bind _doorpartner (`self.DoorPartner`))
  ;[1 1 1] auto open door
  (set `self.FoundEnemyNear` false)
  (for _array_element (`PrimitiveComponent.GetOverlappingActors` _sphere "/Game/Blueprints/Enemies/EnemyEntry_Master.EnemyEntry_Master_C")
    (bind _asenemy_entry_master (cast `/Game/Blueprints/Enemies/EnemyEntry_Master` _array_element))
    (if (`PrimitiveComponent.IsOverlappingComponent` _sphere (`Character.CapsuleComponent` _asenemy_entry_master))
      (set `self.FoundEnemyNear` true)))
  (if (or (`PrimitiveComponent.IsOverlappingActor` _sphere (`self.PlayerRef`)) (`self.FoundEnemyNear`))
    (if (not _open)
      (set `self.Open` true)
      (if (`self.IsDead`) :!label _label_3
        _
        (elif (`self.Open`)
          (`self.OpenDoor`)
          (`/Engine/EditorBlueprintResources/StandardMacros.IsValid` _doorpartner
            (:`Is Valid`
              (`self.OpenDoor` _doorpartner)))
          (else
            (`self.CloseDoor`)
            (`/Engine/EditorBlueprintResources/StandardMacros.IsValid` _doorpartner
              (:`Is Valid`
                (`self.CloseDoor` _doorpartner)))))))
    (elif _open
      (set `self.Open` false)
      (goto _label_3))))

(fn `UserConstructionScript`
  (`parent.UserConstructionScript`))