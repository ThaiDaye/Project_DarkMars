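; Power generator container that switches world generator power on or off through animated wind-up and wind-down sequences.
; Timelines spin the coils and slide the conductors, then shake the screen, set the WorldGen flag and refresh main-powered machines.
; A gated polling macro waits for world generation, then the generator claims a limited, shuffled set of unclaimed transformers.
; Materials show generator power, and up to five lamp pairs show linked transformers' states.
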(event `Generator WindUp`
  (bind _visual_conductor_2 (`self.visual_Conductor_2`))
  (bind _visual_conductor_1 (`self.visual_Conductor_1`))
  (bind (_relativelocation_x _relativelocation_y _relativelocation_z) (`KismetMathLibrary.BreakVector` (`SceneComponent.RelativeLocation` _visual_conductor_2)))
  (bind (_relativelocation_x_2 _relativelocation_y_2 _relativelocation_z_2) (`KismetMathLibrary.BreakVector` (`SceneComponent.RelativeLocation` _visual_conductor_1)))
  ;[1 1 1] wind up
  (set `self.ResetWindup` false)
  (`|ExecutionSequence`
    (:`then_0`
      (`KismetSystemLibrary.Delay` 3.0)
      (bind (_direction _newtrack_1) (`Timeline|Timeline_2` :!via `PlayFromStart`)
        (:`Update`
          (`SceneComponent.K2_SetRelativeLocation` _visual_conductor_1 (`KismetMathLibrary.MakeVector` _relativelocation_x_2 (`KismetMathLibrary.Lerp` 60.0 130.0 _newtrack_1) _relativelocation_z_2) false false)
          (`SceneComponent.K2_SetRelativeLocation` _visual_conductor_2 (`KismetMathLibrary.MakeVector` _relativelocation_x (`KismetMathLibrary.Lerp` -60.0 -130.0 _newtrack_1) _relativelocation_z) false false))
        (:`Finished`
          (`/Game/Blueprints/BP_TopDownCharacter.ScreenShake` (`self.PlayerRef`) 2 "NewEnumerator0" 5000.0 (`self.K2_GetActorLocation`))
          (`KismetSystemLibrary.Delay` 0.2)
          (`self.GeneratorActivated`))))
    (:`then_1`
      (bind (_direction_2 _newtrack_1_2) (`Timeline|Timeline_1` :`NewTime` (select `bool` (`self.WoundUp`) :`true` 5.0 :!type "Float (single-precision)") :!label _label)
        (:`Update`
          (`SceneComponent.K2_AddRelativeRotation` (`self.visual_Coils`) (`KismetMathLibrary.MakeRotator` (* 5.0 _newtrack_1_2)) false false))
        (:`Finished`
          (set `self.WoundUp` true)
          (`KismetSystemLibrary.Delay` 0.0)
          (if (not (`self.ResetWindup`))
            (goto _label)))))))

(event `Generator WindDown`
  (bind _visual_conductor_2 (`self.visual_Conductor_2`))
  (bind _visual_conductor_1 (`self.visual_Conductor_1`))
  (bind (_relativelocation_x _relativelocation_y _relativelocation_z) (`KismetMathLibrary.BreakVector` (`SceneComponent.RelativeLocation` _visual_conductor_1)))
  (bind (_relativelocation_x_2 _relativelocation_y_2 _relativelocation_z_2) (`KismetMathLibrary.BreakVector` (`SceneComponent.RelativeLocation` _visual_conductor_2)))
  ;[1 1 1] wind down
  (set `self.ResetWindup` true)
  (set `self.WoundUp` false)
  (`|ExecutionSequence`
    (:`then_0`
      (`KismetSystemLibrary.Delay` 3.0)
      (bind (_direction _newtrack_1) (`Timeline|Timeline_4` :!via `PlayFromStart`)
        (:`Update`
          (`SceneComponent.K2_SetRelativeLocation` _visual_conductor_1 (`KismetMathLibrary.MakeVector` _relativelocation_x (`KismetMathLibrary.Lerp` 130.0 60.0 _newtrack_1) _relativelocation_z) false false)
          (`SceneComponent.K2_SetRelativeLocation` _visual_conductor_2 (`KismetMathLibrary.MakeVector` _relativelocation_x_2 (`KismetMathLibrary.Lerp` -130.0 -60.0 _newtrack_1) _relativelocation_z_2) false false))
        (:`Finished`
          (`/Game/Blueprints/BP_TopDownCharacter.ScreenShake` (`self.PlayerRef`) 2 "NewEnumerator0" 5000.0 (`self.K2_GetActorLocation`))
          (`KismetSystemLibrary.Delay` 0.2)
          (`self.GeneratorDeactivated`))))
    (:`then_1`
      (bind (_direction_2 _newtrack_1_2) (`Timeline|Timeline_3` :!via `PlayFromStart`)
        (:`Update`
          (`SceneComponent.K2_AddRelativeRotation` (`self.visual_Coils`) (`KismetMathLibrary.MakeRotator` (* 5.0 _newtrack_1_2)) false false))))))

(event `GeneratorDeactivated`
  (set `self.IsPowerOn` false)
  (`self.SetContainerVisual`)
  (set `/Game/Blueprints/WorldGen_Master.GeneratorPowered` false (`self.WorldGenRef`))
  (bind _outactors (`GameplayStatics.GetAllActorsOfClass` "/Game/Blueprints/Objects/ObjectEntry_Master.ObjectEntry_Master_C" :!label _label_2))
  (for _array_element _outactors
    (if (`/Game/Blueprints/Objects/ObjectEntry_Master.IsMachine` _array_element)
      (if (`/Game/Blueprints/Objects/ObjectEntry_Master.Machine_MainPowered` _array_element)
        (`self.SetMachinePower` (`/Game/Blueprints/WorldGen_Master.GeneratorPowered` (`self.WorldGenRef`)))))))

(event `GeneratorActivated`
  (set `self.IsPowerOn` true)
  (`self.SetContainerVisual`)
  (set `/Game/Blueprints/WorldGen_Master.GeneratorPowered` true (`self.WorldGenRef`))
  (goto _label_2))

(event `GetPowerTransformers`
  (bind _outactors (`GameplayStatics.GetAllActorsOfClass` "/Game/Blueprints/Objects/ObjectEntry_Container_Transformer.ObjectEntry_Container_Transformer_C"))
  (bind _output_get (set `self.InRangeRef` _outactors))
  (`KismetArrayLibrary.Array_Shuffle` _output_get)
  (for _array_element (`self.InRangeRef`)
    (if (not (> (`self.DesiredConnectionCount`) (`self.Desired Connection CountRef`)))
      (`/Engine/EditorBlueprintResources/StandardMacros.IsValid` (`/Game/Blueprints/Objects/ObjectEntry_Container_Transformer.ConnectedGenerator` _array_element)
        (:`Is Not Valid`
          (set `/Game/Blueprints/Objects/ObjectEntry_Container_Transformer.ConnectedGenerator` self _array_element)
          (`KismetArrayLibrary.Array_Add` (`self.ConnectedTransformers`) _array_element)
          (`/Engine/EditorBlueprintResources/StandardMacros.IncrementInt` (`self.DesiredConnectionCount`))))))
  (`self.SetContainerVisual`))

(event `self.ReceiveBeginPlay`
  (`parent.ReceiveBeginPlay`)
  (`self.DoAfterWorldGen`
    (:`GenComplete`
      (`self.GetPowerTransformers`))))

(event `self.SetContainerVisual`
  (bind _connectedtransformers (`self.ConnectedTransformers`))
  (bind _returnvalue (select `bool` (`self.IsPowerOn`) :`false` "/Game/Materials/BasicUnlit_Container_2.BasicUnlit_Container_2" :`true` "/Game/Materials/BasicUnlit_Container_1.BasicUnlit_Container_1" :!type "MaterialInterface Object Reference"))
  (`parent.SetContainerVisual`)
  (`PrimitiveComponent.SetMaterial` (`self.visual`) 3 _returnvalue)
  (`PrimitiveComponent.SetMaterial` (`self.Handle_1`) 0 _returnvalue)
  (`PrimitiveComponent.SetMaterial` (`self.Handle_2`) 0 _returnvalue)
  (for _index (range 5)
    (bind _returnvalue_2 (select `int` _index :`0` (`self.Transformer_Light_1_A1`) :`1` (`self.Transformer_Light_1_B1`) :`2` (`self.Transformer_Light_1_C1`) :`3` (`self.Transformer_Light_1_D1`) :`4` (`self.Transformer_Light_1_E1`)))
    (`SceneComponent.SetVisibility` _returnvalue_2 (>= (`KismetArrayLibrary.Array_Length` _connectedtransformers) (+ _index 1)) false)
    (`SceneComponent.SetVisibility` (select `int` _index :`0` (`self.Transformer_Light_1_A`) :`1` (`self.Transformer_Light_1_B`) :`2` (`self.Transformer_Light_1_C`) :`3` (`self.Transformer_Light_1_D`) :`4` (`self.Transformer_Light_1_E`)) (>= (`KismetArrayLibrary.Array_Length` _connectedtransformers) (+ _index 1)) false)
    (bind _output (`|GetArrayItem` _connectedtransformers _index))
    (`/Engine/EditorBlueprintResources/StandardMacros.IsValid` _output
      (:`Is Valid`
        (`PrimitiveComponent.SetMaterial` _returnvalue_2 0 (select `bool` (`/Game/Blueprints/Objects/ObjectEntry_Container_Transformer.IsPowerOn` _output) :`false` "/Game/ScienceLab/Materials/Rooms/MI_Lamp02.MI_Lamp02" :`true` "/Game/ScienceLab/Materials/Rooms/MI_Lamp04.MI_Lamp04" :!type "MaterialInterface Object Reference"))
        (`PrimitiveComponent.SetMaterial` (select `int` _index :`0` (`self.Transformer_Light_1_A`) :`1` (`self.Transformer_Light_1_B`) :`2` (`self.Transformer_Light_1_C`) :`3` (`self.Transformer_Light_1_D`) :`4` (`self.Transformer_Light_1_E`)) 0 (select `bool` (`/Game/Blueprints/Objects/ObjectEntry_Container_Transformer.IsPowerOn` _output) :`false` "/Game/ScienceLab/Materials/Rooms/MI_Lamp02.MI_Lamp02" :`true` "/Game/ScienceLab/Materials/Rooms/MI_Lamp04.MI_Lamp04" :!type "MaterialInterface Object Reference"))))))

(fn `UserConstructionScript`
  (`parent.UserConstructionScript`))