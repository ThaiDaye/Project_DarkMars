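; Interactive door object that toggles open or closed, animating by a timeline that scales the door's Z axis.
; Each toggle mirrors to its DoorPartner, then after a short delay a line trace passes the state to an adjacent door, chaining through ProxyDoorInteract.
; Button materials show locked, open or closed state, and interaction is ignored mid-transition.
; On death it hides, disables door collision and destroys its partner through full-health damage.
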(event `self.ReceiveBeginPlay`
  ;[1 1 1] init
  (`parent.ReceiveBeginPlay`)
  (`self.SetDoorVisuals`))

(event `ProxyDoorInteract`
  (bind _doorpartner (`self.DoorPartner`))
  (bind _open (`self.Open`))
  ;[1 1 1] on interact
  (if (stale `self.OnInteract` _output_get) :!label _label
    (`self.OpenDoor`)
    (set `/Game/Blueprints/Objects/ObjectEntry_Door.Open` _open _doorpartner)
    (`self.OpenDoor` _doorpartner)
    (else
      (`self.CloseDoor`)
      (set `/Game/Blueprints/Objects/ObjectEntry_Door.Open` _open _doorpartner)
      (`self.CloseDoor` _doorpartner)))
  (`self.Open/ClosenearbyDoors`))

(event `self.OnInteract`
  ;[1 1 1] on interact
  (`parent.OnInteract`)
  (if (not (`self.Transitioning`))
    (bind _output_get (set `self.Open` (not (`self.Open`))))
    (goto _label)))

(event `self.OnDeath`
  (bind _doorpartner (`self.DoorPartner`))
  (bind _door (`self.Door`))
  ;[1 1 1] on death
  (`parent.OnDeath`)
  (`PrimitiveComponent.SetCollisionEnabled` _door "NoCollision")
  (`SceneComponent.SetVisibility` _door false true)
  (`SceneComponent.SetVisibility` (`self.Button`) false true)
  (if (not (`/Game/Blueprints/Objects/ObjectEntry_Master.IsDead` _doorpartner))
    (`self.TakeDamage_Object` _doorpartner (`/Game/Blueprints/Objects/ObjectEntry_Master.Health_TotalMax` _doorpartner) 1.0)))

(event `OpenDoor`
  (bind _door (`self.Door`))
  (bind (_returnvalue_x _returnvalue_y) (`KismetMathLibrary.BreakVector` (`SceneComponent.K2_GetComponentScale` _door)))
  ;[1 1 1] open/close
  (set `self.Transitioning` true)
  (bind (_direction _newtrack_0) (`Timeline|Timeline_0` :!label _label_2)
    (:`Update`
      (`SceneComponent.SetWorldScale3D` _door (`KismetMathLibrary.MakeVector` _returnvalue_x _returnvalue_y (`KismetMathLibrary.Lerp` (* (`self.Door Width`) 0.01) 0.01 _newtrack_0))))
    (:`Finished`
      (set `self.Transitioning` false)
      (`self.SetDoorVisuals`))))

(event `Open/CloseNearbyDoors`
  (bind _returnvalue (`SceneComponent.K2_GetComponentLocation` (`self.Arrow`)))
  ;[1 1 1] open/close partner
  (`KismetSystemLibrary.Delay` 0.05)
  (bind _outhit (`KismetSystemLibrary.LineTraceSingleForObjects` _returnvalue (+ _returnvalue (* (`SceneComponent.GetForwardVector` (`self.Button`)) -300)) (`|MakeArray` "ObjectTypeQuery8" :!type "EObjectTypeQuery Enum") false (`|MakeArray` self :!type "Actor Object Reference")))
  (bind (_bblockinghit _binitialoverlap _time _distance _location _impactpoint _normal _impactnormal _physmat _hitactor) (`GameplayStatics.BreakHitResult` _outhit))
  (if _bblockinghit
    (bind _asobject_entry_door (cast `/Game/Blueprints/Objects/ObjectEntry_Door` _hitactor))
    (if (not (`/Game/Blueprints/Objects/ObjectEntry_Door.Transitioning` _asobject_entry_door))
      (set `/Game/Blueprints/Objects/ObjectEntry_Door.Open` (`self.Open`) _asobject_entry_door)
      (`self.ProxyDoorInteract` _asobject_entry_door))))

(event `CloseDoor`
  ;[1 1 1] open/close
  (set `self.Transitioning` true)
  (goto _label_2 :!via `Reverse`))

(fn `SetDoorVisuals`
  (bind _button (`self.Button`))
  (for _index (range (+ (`PrimitiveComponent.GetNumMaterials` _button) 1))
    (`PrimitiveComponent.SetMaterial` _button _index (select `bool` (`self.Locked`) :`false` (select `bool` (`self.Open`) :`false` "/Game/Materials/BasicUnlit_Container_3.BasicUnlit_Container_3" :`true` "/Game/Materials/BasicUnlit_Container_1.BasicUnlit_Container_1" :!type "MaterialInterface Object Reference") :`true` "/Game/Materials/BasicUnlit_Container_2.BasicUnlit_Container_2"))))

(fn `UserConstructionScript`
  (`parent.UserConstructionScript`)
  (`self.SetDoorVisuals`))