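; Master base for world objects that can be damaged, destroyed and interacted with, reporting events through debug prints on the top-down character.
; TakeDamage lowers Health and permanently erodes HealthMax by a given fraction, calling OnDeath at zero.
; Hits play a timeline that jitters the Offset component; death can enable physics on Visual, then optionally destroy the actor after a delay.
; Interaction is flag-gated, including whether dead objects still respond.
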(event `self.ReceiveBeginPlay`
  ;[1 1 1] init
  (bind _outactors (`GameplayStatics.GetAllActorsOfClass` "/Game/Blueprints/BP_TopDownCharacter.BP_TopDownCharacter_C"))
  (set `self.PlayerRef` (`|GetArrayItem` _outactors)))

(event `OnDeath`
  (bind _playerref (`self.PlayerRef`))
  ;[1 1 1] on death
  (if (not (`self.IsDead`))
    (set `self.IsDead` true)
    (`/Engine/EditorBlueprintResources/StandardMacros.IsValid` _playerref
      (:`Is Valid`
        (`/Game/Blueprints/BP_TopDownCharacter.Debug_PrintString_Internal` :`self` _playerref :`Text` (`KismetStringLibrary.Concat_StrStr` (`self.ObjectName`) " Destroyed") :`Colour` (struct :`R` 1.0 :`G` 0.070988 :`B` 0.343843 :`A` 1.0)))
      (:`Is Not Valid`
        _))
    (`self.TakeDamageShake`)
    (if (`self.HasGravityOnDeath`)
      (`self.EnableGravity`)
      (`KismetSystemLibrary.Delay` 2.0)
      (else
        (`KismetSystemLibrary.Delay` 0.2)))
    (if (`self.DestroyOnDeath`)
      (`self.K2_DestroyActor`))))

(event `OnInteract`
  ;[1 1 1] interact
  (if (`self.CanInteract`)
    (if (`self.IsDead`)
      (if (`self.CanInteractWhenDead`)
        (`/Game/Blueprints/BP_TopDownCharacter.Debug_PrintString_Internal` :`self` (`self.PlayerRef`) :`Text` (`KismetStringLibrary.Concat_StrStr` "Interact - " (`self.ObjectName`)) :`Colour` (struct :`R` 1.0 :`G` 0.366636 :`B` 0.933449 :`A` 1.0) :!label _label))
      (else
        (goto _label)))))

(event `TakeDamageShake`
  (bind _offset (`self.Offset`))
  (bind _returnvalue (`KismetSystemLibrary.MakeLiteralDouble` (`self.DamageShake`)))
  (bind _returnvalue_2 (* _returnvalue -1.0))
  (bind _returnvalue_3 (* _returnvalue 0.5))
  ;[1 1 1] damage shake
  (bind (_direction _x _y _z) (`Timeline|Shake` :!via `PlayFromStart`)
    (:`Update`
      (`SceneComponent.K2_SetRelativeLocation` _offset (`KismetMathLibrary.MakeVector` (`KismetMathLibrary.Lerp` _returnvalue _returnvalue_2 (`KismetMathLibrary.FClamp` _x -1.0)) (`KismetMathLibrary.Lerp` _returnvalue _returnvalue_2 (`KismetMathLibrary.FClamp` _y -1.0)) (`KismetMathLibrary.Lerp` _returnvalue_3 (* _returnvalue_3 -1.0) (`KismetMathLibrary.FClamp` _z -1.0))) false false))
    (:`Finished`
      (`SceneComponent.K2_SetRelativeLocation` _offset (0.0 0.0 0.0) false false))))

(fn `EnableGravity`
  (`PrimitiveComponent.SetSimulatePhysics` (`self.visual`) true)
  (`SceneComponent.K2_AttachToComponent` (`self.Offset`) (`self.visual`) "None" "KeepWorld" "KeepWorld" "KeepWorld" true))

(fn `TakeDamage`
  (params (Damage :type "Float (double-precision)") (`% Max Lost` :type "Float (double-precision)"))
  (returns (IsDead :type Boolean))
  (bind _health_totalmax (`self.Health_TotalMax`))
  (bind _playerref (`self.PlayerRef`))
  (`/Engine/EditorBlueprintResources/StandardMacros.IsValid` _playerref
    (:`Is Valid`
      (`/Game/Blueprints/BP_TopDownCharacter.Debug_PrintString_Internal` :`self` _playerref :`Text` (`KismetStringLibrary.Concat_StrStr` (`KismetStringLibrary.Conv_DoubleToString` Damage) " Damage Taken (" (`KismetStringLibrary.Conv_DoubleToString` (* `% Max Lost` 100.0)) "% permanent)") :`Colour` (struct :`R` 1.0 :`G` 0.366636 :`B` 0.933449 :`A` 1.0)))
    (:`Is Not Valid`
      _))
  (bind _output_get (set `self.Health` (`KismetMathLibrary.FClamp` (- (`self.Health`) Damage) 0.0 (`self.Health_Max`))))
  (set `self.Health_Max` (`KismetMathLibrary.FClamp` (- (`self.Health_Max`) (* Damage `% Max Lost`)) 0.0 _health_totalmax))
  (if (<= _output_get 0.0)
    (if (not (<= _health_totalmax 0.0))
      (`self.TakeDamageShake`))
    (`self.OnDeath`)
    (return true)
    (else
      (`self.TakeDamageShake`)
      (return false))))

(fn `UserConstructionScript`)