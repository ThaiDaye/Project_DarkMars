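; World item pickup, derived from an object-entry parent, that gives its item to the player's inventory on interact.
; ItemID pulls mesh, material, health and interaction data from a data table.
; Sphere traces floor-snap it or find wall attachments, registering it with the supporting object and re-placing it when that is destroyed.
; Retriggerable delays drive fog-visibility dither fades and the player's visible-items list; a scale-and-rise timeline ends pickup with dust and destruction.
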(event `self.ReceiveBeginPlay`
  (`parent.ReceiveBeginPlay`)
  (`self.SetItemVisuals`)
  (`self.SetUniqueNum`)
  (`self.Set Fog Visibility`)
  (`KismetSystemLibrary.Delay` 0.2)
  (`self.PlaceOnSurface`))

(event `Set Fog Visibility`
  (`SceneComponent.SetHiddenInGame` (`self.visual`) (not (`self.Fog_Visible`)) false))

(event `ItemFogFade`
  (params (FogFadeIn :type Boolean))
  (if FogFadeIn
    (`self.Set Fog Visibility`)
    (bind (_direction _newtrack_0) (`Timeline|Timeline_1` :!label _label)
      (:`Update`
        (`MeshComponent.SetScalarParameterValueOnMaterials` (`self.visual`) "DitherAmnt" (`KismetMathLibrary.Lerp` 500.0 0.0 _newtrack_0)))
      (:`Finished`
        (if (not FogFadeIn)
          (`self.Set Fog Visibility`))))
    (else
      (goto _label :!via `Reverse`))))

(event `ParentDestroyed`
  (`KismetSystemLibrary.Delay` 0.01)
  (`self.PlaceOnSurface`))

(event `StartSetFogVisible_item`
  (bind _canseeitems (`/Game/Blueprints/BP_TopDownCharacter.CanSeeItems` (`self.PlayerRef`)))
  ;[1 1 1] set visibility fog
  (`|ExecutionSequence`
    (:`then_0`
      (set `self.Fog_Visible` true)
      (`self.ItemFogFade` true)
      (`KismetSystemLibrary.RetriggerableDelay` 0.51)
      (set `self.Fog_Visible` false)
      (`self.ItemFogFade` false))
    (:`then_1`
      (if (`KismetArrayLibrary.Array_Contains` _canseeitems self)
        _
        (elif (not (`self.IsDead`))
          (`KismetArrayLibrary.Array_Add` _canseeitems self)))
      (`KismetSystemLibrary.RetriggerableDelay` 5.0)
      (`KismetArrayLibrary.Array_RemoveItem` _canseeitems self))))

(event `self.OnInteract`
  (bind _playerref (`self.PlayerRef`))
  (`parent.OnInteract`)
  (if (not (`self.Animating`))
    (`/Game/Blueprints/BP_TopDownCharacter.Debug_PrintString_Internal` :`self` (`self.PlayerRef`) :`Text` "Picked up item" :`Colour` (struct :`R` 1.0 :`G` 0.041667 :`B` 0.899303 :`A` 1.0))
    (`/Game/Blueprints/BP_TopDownCharacter.Inv_GiveItem` _playerref _playerref (`self.ItemID`) (`self.Stack`) false 0 (`self.CurrentAmmo`) false (`self.UniqueNum`) self false)
    (`/Game/Blueprints/BP_TopDownCharacter.PlaySFXFromSoundBank` (`self.PlayerRef`) "NewEnumerator1" (`self.K2_GetActorLocation`))))

(event `self.OnDeath`
  (`parent.OnDeath`))

(event `ItemPickupInteractEnd`
  (bind _offset (`self.Offset`))
  (set `self.Animating` true)
  (bind _output_get (set `self.Scale` (`SceneComponent.K2_GetComponentScale` (`self.Offset`))))
  (bind (_direction _xy _z) (`Timeline|Timeline_0` :!via `PlayFromStart`)
    (:`Update`
      (`SceneComponent.SetWorldScale3D` _offset (`KismetMathLibrary.MakeVector` (* (.x _output_get) _xy) (* (.y _output_get) _xy) (* (.z _output_get) _z)))
      (`SceneComponent.K2_AddWorldOffset` _offset (0.0 0.0 1.0) false false))
    (:`Finished`
      (`NiagaraFunctionLibrary.SpawnSystemAtLocation` "/Game/VFX/Systems/Dust_ParticleSystem.Dust_ParticleSystem" (`self.K2_GetActorLocation`))
      (`self.K2_DestroyActor`))))

(fn `PlaceOnSurface`
  (bind _returnvalue (`self.K2_GetActorLocation`))
  (switch `/Game/Blueprints/Data/EnemyStartingState_Type` (`self.ObjectStartState`)
    (:`NewEnumerator0`
      (bind _outhit (`KismetSystemLibrary.SphereTraceSingle` _returnvalue (+ _returnvalue (* (`SceneComponent.GetUpVector` (`self.DefaultSceneRoot`)) -200.0)) 10.0 "TraceTypeQuery1" :!label _label))
      (bind (_bblockinghit _binitialoverlap _time _distance _location _impactpoint _normal _impactnormal _physmat _hitactor) (`GameplayStatics.BreakHitResult` _outhit))
      (if _bblockinghit
        (`self.K2_SetActorLocation` _impactpoint)
        (bind _asobject_entry_master (cast `/Game/Blueprints/Objects/ObjectEntry_Master` _hitactor))
        (`KismetArrayLibrary.Array_Add` (`/Game/Blueprints/Objects/ObjectEntry_Master.ChildrenObjectEntries` _asobject_entry_master) self)))
    (:`NewEnumerator1`
      (bind _outhit_2 (`KismetSystemLibrary.SphereTraceSingle` _returnvalue _returnvalue 50.0 "TraceTypeQuery1" :!label _label_2))
      (bind (_bblockinghit_2 _binitialoverlap_2 _time_2 _distance_2 _location_2 _impactpoint_2 _normal_2 _impactnormal_2 _physmat_2 _hitactor_2) (`GameplayStatics.BreakHitResult` _outhit_2))
      (if _bblockinghit_2
        (bind _asobject_entry_master_2 (cast `/Game/Blueprints/Objects/ObjectEntry_Master` _hitactor_2))
        (`KismetArrayLibrary.Array_Add` (`/Game/Blueprints/Objects/ObjectEntry_Master.ChildrenObjectEntries` _asobject_entry_master_2) self)))
    (:`NewEnumerator2`
      (goto _label))
    (:`NewEnumerator3`
      (goto _label_2))))

(fn `SetItemVisuals`
  (bind _visual (`self.visual`))
  (bind (_itemname _itemdescription _itemrarity _itemtype _itemsubstance _itemmaxstack _itemmaxhealth _itemmesh _itemmaterial _itemicon _itemsizex _itemsizey _itemoffset _itemcontaineroffset _itemcanbedestroyed _idequipobject _ammunitiontypeammo _interactduration) (break `/Game/Blueprints/Data/ItemID_Struct` (`self.ItemData`)))
  (bind _returnvalue (`|GetDataTableRow` "/Game/Blueprints/Data/ItemID_Table.ItemID_Table" (`self.ItemID`))
    (:`then`
      (set `self.ItemData` _returnvalue)
      (set `self.ObjectName` _itemname)
      (bind _output_get (set `self.Health` _itemmaxhealth))
      (bind _output_get_2 (set `self.Health_Max` _output_get))
      (set `self.Health_TotalMax` _output_get_2)
      (set `self.Object Substance` _itemsubstance)
      (set `self.Stack` (`KismetMathLibrary.Clamp` (`self.Stack`) 0 _itemmaxstack))
      (`StaticMeshComponent.SetStaticMesh` _visual _itemmesh)
      (for _index (range (+ (`PrimitiveComponent.GetNumMaterials` _visual) 1))
        (`PrimitiveComponent.SetMaterial` (`self.visual`) _index _itemmaterial))
      (set `self.InteractWaitDuration` _interactduration)
      (`SceneComponent.K2_SetRelativeTransform` _visual _itemoffset false false)
      (set `self.DestroyOnDeath` _itemcanbedestroyed))))

(fn `SetUniqueNum`
  (if (== (`self.UniqueNum`) -1)
    (set `self.UniqueNum` (`KismetMathLibrary.RandomInteger` 999999))))

(fn `UserConstructionScript`
  (`parent.UserConstructionScript`)
  (`self.SetItemVisuals`))