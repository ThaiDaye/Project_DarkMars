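; Safe container object entry that positions itself in the procedurally generated world.
; On BeginPlay, a gated delay loop polls the world generator until generation completes.
; It then sets its start state, choosing floor, wall or ceiling placement, with attached placement mapped to floor, and rotating to the surface.
; A weighted random draw from the world seed picks between two wall heights.
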(event `self.ReceiveBeginPlay`
  (`parent.ReceiveBeginPlay`)
  (`self.DoAfterWorldGen`
    (:`GenComplete`
      (`self.SetStartState__` (select `/Game/Blueprints/Data/EnemyStartingState_Type` (`self.ObjectStartState`) :`NewEnumerator0` "NewEnumerator0" :`NewEnumerator1` "NewEnumerator1" :`NewEnumerator2` "NewEnumerator2" :`NewEnumerator3` "NewEnumerator0" :!type "/Game/Blueprints/Data/EnemyStartingState_Type Enum") "NewEnumerator0" (select `bool` (`KismetMathLibrary.RandomBoolWithWeightFromStream` 0.5 (`/Game/Blueprints/WorldGen_Master.Seed` (`self.WorldGenRef`))) :`false` 70.0 :`true` 140.0) true 300.0))))

(fn `UserConstructionScript`
  (`parent.UserConstructionScript`))