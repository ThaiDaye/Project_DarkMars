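; Grid inventory item shown as a 3D actor spanning its cell footprint.
; SetItemVisuals caches the data table row by ID, then sizes the tile and sets mesh, rarity backing, stack count and hotbar marker.
; RotateItem swaps width and height, then refreshes visuals.
; PlaceCheckTrace line-traces each occupied cell, requiring inventory slots for placement and reporting the first blocking item as a swap candidate.
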(event `self.ReceiveBeginPlay`
  (bind _outactors (`GameplayStatics.GetAllActorsOfClass` "/Game/Blueprints/BP_TopDownCharacter.BP_TopDownCharacter_C"))
  (set `self.PlayerRef` (`|GetArrayItem` _outactors))
  (`self.SetItemVisuals`)
  (set `self.SizeY_Start` (`self.SizeY`))
  (set `self.SizeX_Start` (`self.SizeX`))
  (`self.Rotate Item` (`self.Rotated`) true))

(fn `PlaceCheckTrace`
  (params (Location :type "Vector Structure"))
  (returns (ValidPlace :type Boolean) (ValidSwapPlace :type Boolean) (ValidSwapRef :type "/Game/Blueprints/Inventory/ItemEntry_Master Object Reference"))
  (locals (ValidPlaceloc :type Boolean :default true) (ValidPlaceloc_Swap :type Boolean :default true) (ValidSwap :type "/Game/Blueprints/Inventory/ItemEntry_Master Object Reference"))
  (bind _box (`self.Box`))
  (bind _returnvalue (`SceneComponent.GetForwardVector` (`self.Box`)))
  (for _index (range (`self.SizeX`))
    (for _index_2 (range (`self.SizeY`))
      (bind _returnvalue_2 (+ (* (`SceneComponent.GetUpVector` _box) (* _index_2 -1.68)) (* (`SceneComponent.GetRightVector` _box) (* _index -1.68)) (0.0 0.0 0.0) Location))
      (bind _outhit (`KismetSystemLibrary.LineTraceSingleForObjects` (+ _returnvalue_2 (* _returnvalue 2.0)) (+ _returnvalue_2 (* _returnvalue -2.0)) (`|MakeArray` "ObjectTypeQuery16" "ObjectTypeQuery15" :!type "EObjectTypeQuery Enum") false (`|MakeArray` self :!type "Actor Object Reference") "None" false))
      (bind (_bblockinghit _binitialoverlap _time _distance _location _impactpoint _normal _impactnormal _physmat _hitactor) (`GameplayStatics.BreakHitResult` _outhit))
      (if _bblockinghit
        (cast `/Game/Blueprints/Inventory/Inventory3DEntry_Master` _hitactor
          (:`CastFailed`
            (bind _asitem_entry_master (cast `/Game/Blueprints/Inventory/ItemEntry_Master` _hitactor)
              (:`then`
                (set `local.ValidPlaceloc` false)
                (`/Engine/EditorBlueprintResources/StandardMacros.IsValid` (`local.ValidSwap`)
                  (:`Is Not Valid`
                    (set `local.ValidSwap` _asitem_entry_master))))
              (:`CastFailed`
                (set `local.ValidPlaceloc` false)
                (set `local.ValidPlaceloc_Swap` false)))))
        (else
          (set `local.ValidPlaceloc` false)
          (set `local.ValidPlaceloc_Swap` false)))))
  (return (`local.ValidPlaceloc`) (`local.ValidPlaceloc_Swap`) (`local.ValidSwap`)))

(fn `Rotate Item`
  (params (Value :type Boolean) (UseValue :type Boolean))
  (bind _sizey_start (`self.SizeY_Start`))
  (bind _sizex_start (`self.SizeX_Start`))
  (bind _rotated (`self.Rotated`))
  (if UseValue
    (set `self.Rotated` Value)
    (else
      (set `self.Rotated` (not (`self.Rotated`)))))
  (set `self.SizeX` (select `bool` _rotated :`false` _sizex_start :`true` _sizey_start))
  (set `self.SizeY` (select `bool` _rotated :`false` _sizey_start :`true` _sizex_start))
  (`self.SetItemVisuals`))

(fn `SetItemVisuals`
  (bind _id (`self.ID`))
  (bind _textrender (`self.TextRender`))
  (bind _uniquenum (`self.UniqueNum`))
  (bind _visual (`self.visual`))
  (bind _playerref (`self.PlayerRef`))
  (bind _visual_2 (`self.visual`))
  (bind (_itemname _itemdescription _itemrarity _itemtype _itemsubstance _itemmaxstack _itemmaxhealth _itemmesh _itemmaterial _itemicon _itemsizex _itemsizey _itemoffset _itemcontaineroffset) (break `/Game/Blueprints/Data/ItemID_Struct` (`self.ItemData`)))
  (bind _returnvalue (`KismetMathLibrary.Conv_IntToDouble` (`self.SizeY`)))
  (bind _returnvalue_2 (`KismetMathLibrary.Conv_IntToDouble` (`self.SizeX`)))
  (bind _equip_hotbar (`/Game/Blueprints/BP_TopDownCharacter.Equip_Hotbar` _playerref))
  (bind _returnvalue_3 (+ (* _returnvalue_2 -8.4) 8.4))
  (bind _returnvalue_4 (+ (* _returnvalue -8.4) 8.4))
  (bind _returnvalue_5 (`|GetDataTableRow` "/Game/Blueprints/Data/ItemID_Table.ItemID_Table" (`self.ID`))
    (:`then`
      (if (not (`self.IDloaded`))
        (bind _output_get (set `self.ItemData` _returnvalue_5))
        (set `self.IDloaded` true)
        (bind (_itemname_2 _itemdescription_2 _itemrarity_2 _itemtype_2 _itemsubstance_2 _itemmaxstack_2 _itemmaxhealth_2 _itemmesh_2 _itemmaterial_2 _itemicon_2 _itemsizex_2 _itemsizey_2) (break `/Game/Blueprints/Data/ItemID_Struct` _output_get))
        (set `self.SizeX` _itemsizex_2)
        (set `self.SizeY` _itemsizey_2)))
    (:`RowNotFound`
      _))
  (`SceneComponent.SetRelativeScale3D` (`self.Box`) (`KismetMathLibrary.MakeVector` 0.1 _returnvalue_2 _returnvalue))
  (`SceneComponent.SetRelativeScale3D` (`self.Plane`) (`KismetMathLibrary.MakeVector` (* _returnvalue_2 0.168) (* _returnvalue 0.168) 1.0))
  (`SceneComponent.K2_SetRelativeLocation` (`self.Box`) (`KismetMathLibrary.MakeVector` 0.0 _returnvalue_3 _returnvalue_4) false false)
  (`SceneComponent.K2_SetRelativeLocation` (`self.Plane`) (`KismetMathLibrary.MakeVector` -6.0 _returnvalue_3 _returnvalue_4) false false)
  (`SceneComponent.K2_SetRelativeLocation` (`self.VisualOffset`) (`KismetMathLibrary.MakeVector` -10.0 _returnvalue_3 _returnvalue_4) false false)
  (`SceneComponent.K2_SetRelativeRotation` (`self.VisualOffset`) (`KismetMathLibrary.MakeRotator` 0.0 -90.0) false false)
  (`SceneComponent.K2_SetRelativeRotation` (`self.Scene2`) (`KismetMathLibrary.MakeRotator` 0.0 0.0 (select `bool` (`self.Rotated`) :`true` 270.0 :!type "Float (single-precision)")) false false)
  (`SceneComponent.SetWorldScale3D` _textrender (select `bool` (== (`.ItemMaxStack_36_F4AD081E4B2758961C11FA9F2A05277D` (break `/Game/Blueprints/Data/ItemID_Struct` (`self.ItemData`))) 1) :`false` (0.02 0.02 0.02) :!type "Vector Structure"))
  (`SceneComponent.SetWorldScale3D` (`self.HotbarFav`) (select `bool` (and (`KismetArrayLibrary.Array_Contains` _equip_hotbar _uniquenum) (== _playerref (`/Game/Blueprints/Inventory/Inventory3DWidget_Master.ContainerRef` (`self.ParentInv`)))) :`true` (0.0125 0.0125 0.0125) :!type "Vector Structure"))
  (`TextRenderComponent.K2_SetText` (`self.TextRender1`) (`KismetTextLibrary.Conv_IntToText` (+ (`KismetArrayLibrary.Array_Find` _equip_hotbar _uniquenum) 1) false true 1 1))
  (`TextRenderComponent.K2_SetText` _textrender (`KismetTextLibrary.Conv_IntToText` (`self.Stack`) false true 1 3))
  (if (not (or (== _id "None") (== _id "None")))
    (`TextRenderComponent.SetTextRenderColor` _textrender (`KismetMathLibrary.LinearColor_ToRGBE` (select `bool` (== (`self.Stack`) (`.ItemMaxStack_36_F4AD081E4B2758961C11FA9F2A05277D` (break `/Game/Blueprints/Data/ItemID_Struct` (`self.ItemData`)))) :`false` (struct :`R` 1.0 :`G` 1.0 :`B` 1.0 :`A` 1.0) :`true` (struct :`R` 0.547744 :`G` 0.962312 :`B` 1.0 :`A` 1.0) :!type "LinearColor Structure")))
    (`StaticMeshComponent.SetStaticMesh` _visual_2 _itemmesh)
    (for _index (range (+ (`PrimitiveComponent.GetNumMaterials` _visual_2) 1))
      (`PrimitiveComponent.SetMaterial` _visual _index _itemmaterial)
      (`MeshComponent.SetScalarParameterValueOnMaterials` _visual "E" 0.2))
    (`SceneComponent.K2_SetRelativeTransform` _visual_2 _itemcontaineroffset false false)
    (`PrimitiveComponent.SetMaterial` (`self.Plane`) 0 (select `/Game/Blueprints/Data/ItemRarity_Type` _itemrarity :`NewEnumerator3` "/Game/Materials/UIMat_master_Inst9.UIMat_master_Inst9" :`NewEnumerator0` "/Game/Materials/UIMat_master_Inst10_2.UIMat_master_Inst10_2" :`NewEnumerator1` "/Game/Materials/UIMat_master_Inst10.UIMat_master_Inst10" :`NewEnumerator2` "/Game/Materials/UIMat_master_Inst11.UIMat_master_Inst11" :`NewEnumerator4` "/Game/Materials/UIMat_master_Inst10_3.UIMat_master_Inst10_3" :`NewEnumerator5` "/Game/Materials/UIMat_master_Inst11_2.UIMat_master_Inst11_2" :!type "MaterialInterface Object Reference"))))

(fn `UserConstructionScript`)