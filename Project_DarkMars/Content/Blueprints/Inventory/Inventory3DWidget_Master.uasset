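; Master actor for a 3D inventory that builds a slot grid and places stored items on it at BeginPlay.
; Line traces step across the ItemEntryArea box, spawning an attached Inventory3DEntry_Master at each hit outside ItemDenyArea, which allows irregular layouts.
; The player character then spawns each ItemInventoryList item at its saved slot using data table stack limits; ResetItems re-runs only this step.
; It also passes ContainerRef to the slots and interact-screen widget.
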(event `self.ReceiveBeginPlay`
  (bind _3dinteractscreen (`self.3DInteractScreen`))
  (bind _outactors (`GameplayStatics.GetAllActorsOfClass` "/Game/Blueprints/BP_TopDownCharacter.BP_TopDownCharacter_C"))
  (set `self.PlayerRef` (`|GetArrayItem` _outactors))
  (`self.Setinventory`)
  (`/Engine/EditorBlueprintResources/StandardMacros.IsValid` _3dinteractscreen
    (:`Is Valid`
      (bind _as3dinteract_screen_master (cast `/Game/Blueprints/Inventory/Screens/3DinteractScreen_Master` (`WidgetComponent.GetWidget` _3dinteractscreen)))
      (set `/Game/Blueprints/Inventory/Screens/3DinteractScreen_Master.ContainerRef` (`self.ContainerRef`) _as3dinteract_screen_master)
      (set `self.ScreenRef` _as3dinteract_screen_master))))

(event `SetInventory`
  (bind _itementryarea (`self.ItemEntryArea`))
  (bind _itementryarea_2 (`self.ItemEntryArea`))
  (bind _inventoryslotsref (`self.InventorySlotsRef`))
  (bind _itementryarea_3 (`self.ItemEntryArea`))
  (bind _returnvalue (`SceneComponent.GetForwardVector` (`self.ItemEntryArea`)))
  (bind (_relativescale3d_x _relativescale3d_y _relativescale3d_z) (`KismetMathLibrary.BreakVector` (`SceneComponent.RelativeScale3D` (`self.ItemEntryArea`))))
  (bind (_relativescale3d_x_2 _relativescale3d_y_2 _relativescale3d_z_2) (`KismetMathLibrary.BreakVector` (`SceneComponent.RelativeScale3D` _itementryarea_3)))
  (bind (_relativescale3d_x_3 _relativescale3d_y_3 _relativescale3d_z_3) (`KismetMathLibrary.BreakVector` (`SceneComponent.RelativeScale3D` (`self.ItemEntryArea`))))
  (bind _returnvalue_2 (* (.y (`BoxComponent.BoxExtent` (`self.ItemEntryArea`))) 0.1))
  (bind _returnvalue_3 (* (.z (`BoxComponent.BoxExtent` (`self.ItemEntryArea`))) 0.1))
  ;[1 1 1] draw grid
  (for _array_element _inventoryslotsref
    (`self.K2_DestroyActor` _array_element))
  (`KismetArrayLibrary.Array_Clear` _inventoryslotsref)
  (set `self.CurrentIndex` 0)
  (for _index (range (`KismetMathLibrary.Round` _returnvalue_3))
    (for _index_2 (range (`KismetMathLibrary.Round` _returnvalue_2))
      (bind _returnvalue_4 (+ (* (`SceneComponent.GetUpVector` _itementryarea_2) (* _index (* _relativescale3d_z_3 -1.0) 2.0)) (* (`SceneComponent.GetRightVector` _itementryarea_2) (* _index_2 _relativescale3d_y_3 2.0)) (+ (* (* _relativescale3d_y_2 -1.0) (`SceneComponent.GetUpVector` _itementryarea_3)) (* _relativescale3d_z_2 (`SceneComponent.GetRightVector` _itementryarea_3))) (+ (`SceneComponent.K2_GetComponentLocation` (`self.ItemEntryArea`)) (* (`SceneComponent.GetRightVector` _itementryarea) (* _returnvalue_2 (* _relativescale3d_y -1.0))) (* (`SceneComponent.GetUpVector` _itementryarea) (* _returnvalue_3 _relativescale3d_z)))))
      (bind _outhit (`KismetSystemLibrary.LineTraceSingleForObjects` :`Start` (+ _returnvalue_4 (* _returnvalue -1.0)) :`End` (+ _returnvalue_4 (* _returnvalue 1.0)) :`ObjectTypes` (`|MakeArray` "ObjectTypeQuery15" :!type "EObjectTypeQuery Enum") :`bIgnoreSelf` false))
      (bind (_bblockinghit _binitialoverlap _time _distance _location _impactpoint _normal _impactnormal _physmat _hitactor _hitcomponent) (`GameplayStatics.BreakHitResult` _outhit))
      (if _bblockinghit
        (if (not (== _hitcomponent (`self.ItemDenyArea`)))
          (bind _returnvalue_5 (`|SpawnActorFromClass` "/Game/Blueprints/Inventory/Inventory3DEntry_Master.Inventory3DEntry_Master_C" (`KismetMathLibrary.MakeTransform` _impactpoint (`SceneComponent.K2_GetComponentRotation` (`self.ItemEntryArea`))) "AlwaysSpawn" "OverrideRootScale" null (`self.CurrentIndex`) _index_2 _index (`self.ContainerRef`) null))
          (`self.K2_AttachToActor` _returnvalue_5 self "None" "KeepWorld" "KeepWorld" "KeepWorld" true)
          (`KismetArrayLibrary.Array_Add` (`self.InventorySlotsRef`) _returnvalue_5)
          (set `self.CurrentIndex` (+ (`self.CurrentIndex`) 1))))))
  (`ActorComponent.K2_DestroyComponent` (`self.ItemDenyArea`))
  (`PrimitiveComponent.SetCollisionEnabled` (`self.Inventory`) "NoCollision")
  (for (_array_element_2 _array_index) (`self.ItemInventoryList`) :!label _label
    (bind (_itemid _uniquenumber _sizex _sizey _rotated _entryindex _stack _currentammo) (break `/Game/Blueprints/Data/ItemData_Struct` _array_element_2))
    (bind _returnvalue_6 (`|GetDataTableRow` "/Game/Blueprints/Data/ItemID_Table.ItemID_Table" _itemid)
      (:`then`
        (`/Game/Blueprints/BP_TopDownCharacter.Inv_SpawnItemAtEntry_DEBUG` (`self.PlayerRef`) _sizex _sizey (`|GetArrayItem` (`self.InventorySlotsRef`) _entryindex) _rotated self _array_index _itemid _stack (`.ItemMaxStack_36_F4AD081E4B2758961C11FA9F2A05277D` (break `/Game/Blueprints/Data/ItemID_Struct` _returnvalue_6)) _currentammo _uniquenumber)
        (`KismetArrayLibrary.Array_Set` (`self.ItemInventoryList`) _array_index (make `/Game/Blueprints/Data/ItemData_Struct` _itemid _uniquenumber _sizex _sizey _rotated _entryindex _stack _currentammo) true)))))

(event `ResetItems`
  (goto _label))

(fn `UserConstructionScript`)