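; InteractHoverUI_BP is an actor that shows an interaction hover widget at the player's current interact location.
; On BeginPlay it finds the BP_TopDownCharacter and hands itself to its InteractHoverUI_Widget as HoverRef.
; Each tick it moves to the player's InteractLoc and shows the widget while that location is valid.
; The widget is hidden when no valid location exists or the fullscreen inventory is open.
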(event `self.ReceiveBeginPlay`
  (bind _outactors (`GameplayStatics.GetAllActorsOfClass` "/Game/Blueprints/BP_TopDownCharacter.BP_TopDownCharacter_C"))
  (set `self.PlayerRef` (`|GetArrayItem` _outactors))
  (bind _asinteract_hover_ui_widget (cast `/Game/Blueprints/Gamemode/InteractHoverUI_Widget` (`WidgetComponent.GetWidget` (`self.Widget`))))
  (bind _output_get (set `self.WidgetRef` _asinteract_hover_ui_widget))
  (set `/Game/Blueprints/Gamemode/InteractHoverUI_Widget.HoverRef` self _output_get))

(event `self.ReceiveTick`
  (params (DeltaSeconds :type "Float (single-precision)"))
  (bind _playerref (`self.PlayerRef`))
  (bind _widget (`self.Widget`))
  (`/Engine/EditorBlueprintResources/StandardMacros.IsValid` _playerref
    (:`Is Valid`
      (if (`/Game/Blueprints/BP_TopDownCharacter.ValidInteractLoc` _playerref)
        (`self.K2_SetActorLocation` (`/Game/Blueprints/BP_TopDownCharacter.InteractLoc` _playerref))
        (`SceneComponent.SetVisibility` _widget true false)
        (else
          (`SceneComponent.SetVisibility` _widget false false)))
      (`/Engine/EditorBlueprintResources/StandardMacros.IsValid` (`/Game/Blueprints/BP_TopDownCharacter.FullscreenInventoryRef` _playerref)
        (:`Is Valid`
          (`SceneComponent.SetVisibility` _widget false false))))))

(fn `UserConstructionScript`)