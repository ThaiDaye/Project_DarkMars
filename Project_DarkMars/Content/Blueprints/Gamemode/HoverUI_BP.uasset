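; HoverUI_BP is an actor that shows a floating name label for whatever the top-down player character hovers over.
; Each Tick it reads the player's hover target, moves to the hover location and fills HoverUI_Widget with name, state and rarity for items, containers or enemies.
; Item pickups and enemies update the label only when fog-visible.
; Zoom-dragging, no target or an unsupported type hides it.
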(event `self.ReceiveBeginPlay`
  (bind _outactors (`GameplayStatics.GetAllActorsOfClass` "/Game/Blueprints/BP_TopDownCharacter.BP_TopDownCharacter_C"))
  (set `self.PlayerRef` (`|GetArrayItem` _outactors))
  (bind _ashover_ui_widget (cast `/Game/Blueprints/Gamemode/HoverUI_Widget` (`WidgetComponent.GetWidget` (`self.Widget`))))
  (bind _output_get (set `self.WidgetRef` _ashover_ui_widget))
  (set `/Game/Blueprints/Gamemode/HoverUI_Widget.HoverRef` self _output_get))

(event `self.ReceiveTick`
  (params (DeltaSeconds :type "Float (single-precision)"))
  (bind _playerref (`self.PlayerRef`))
  (bind _widgetref (`self.WidgetRef`))
  (bind _widgetref_2 (`self.WidgetRef`))
  (bind _widgetref_3 (`self.WidgetRef`))
  (bind _widgetref_4 (`self.WidgetRef`))
  (bind _hoveractortarget (`/Game/Blueprints/BP_TopDownCharacter.HoverActorTarget` _playerref))
  (bind _hoveractortarget_2 (`/Game/Blueprints/BP_TopDownCharacter.HoverActorTarget` (`self.PlayerRef`)))
  (`/Engine/EditorBlueprintResources/StandardMacros.IsValid` _playerref
    (:`Is Valid`
      (bind _asobject_entry_item_pickup (cast `/Game/Blueprints/Objects/ObjectEntry_ItemPickup` _hoveractortarget)
        (:`then`
          (`/Engine/EditorBlueprintResources/StandardMacros.IsValid` _asobject_entry_item_pickup
            (:`Is Valid`
              (if (`/Game/Blueprints/Objects/ObjectEntry_ItemPickup.Fog_Visible` _asobject_entry_item_pickup)
                (if (`/Game/Blueprints/BP_TopDownCharacter.ZoomDragging` _playerref) :!label _label
                  (`SceneComponent.SetVisibility` (`self.Widget`) false false :!label _label_2)
                  (else
                    (`/Engine/EditorBlueprintResources/StandardMacros.IsValid` _hoveractortarget
                      (:`Is Valid`
                        (`self.K2_SetActorLocation` (`/Game/Blueprints/BP_TopDownCharacter.HoverLocation` _playerref))
                        (`SceneComponent.SetVisibility` (`self.Widget`) true false)
                        (bind _asobject_entry_item_pickup_2 (cast `/Game/Blueprints/Objects/ObjectEntry_ItemPickup` _hoveractortarget_2)
                          (:`then`
                            (bind (_itemname _itemdescription _itemrarity) (break `/Game/Blueprints/Data/ItemID_Struct` (`/Game/Blueprints/Objects/ObjectEntry_ItemPickup.ItemData` _asobject_entry_item_pickup_2)))
                            (bind _stack (`/Game/Blueprints/Objects/ObjectEntry_ItemPickup.Stack` _asobject_entry_item_pickup_2))
                            (set `/Game/Blueprints/Gamemode/HoverUI_Widget.ItemText` (`KismetStringLibrary.Concat_StrStr` _itemname (select `bool` (== _stack 1) :`false` (`KismetStringLibrary.Concat_StrStr` " (" (`KismetStringLibrary.Conv_IntToString` _stack) ")") :`true` (select `bool` (== (`/Game/Blueprints/Objects/ObjectEntry_ItemPickup.CurrentAmmo` _asobject_entry_item_pickup_2) 0) :`false` (`KismetStringLibrary.Concat_StrStr` " (" "Loaded" ")"))) (select `bool` (`/Game/Blueprints/Objects/ObjectEntry_Master.IsDead` _asobject_entry_item_pickup_2) :`true` "(Destroyed)")) _widgetref_2)
                            (set `/Game/Blueprints/Gamemode/HoverUI_Widget.ItemRarity` _itemrarity _widgetref_2))
                          (:`CastFailed`
                            (bind _asobject_entry_container (cast `/Game/Blueprints/Objects/ObjectEntry_Container` _hoveractortarget_2)
                              (:`then`
                                (set `/Game/Blueprints/Gamemode/HoverUI_Widget.ItemText` (`KismetStringLibrary.Concat_StrStr` (`/Game/Blueprints/Objects/ObjectEntry_Master.ObjectName` _asobject_entry_container) (select `bool` (`/Game/Blueprints/Objects/ObjectEntry_Container.Locked` _asobject_entry_container) :`false` (select `bool` (and (!= (`/Game/Blueprints/Objects/ObjectEntry_Container.InventorySizeRef` _asobject_entry_container) 0) (== (`KismetArrayLibrary.Array_Length` (`/Game/Blueprints/Objects/ObjectEntry_Container.ItemInventoryList` _asobject_entry_container)) 0)) :`true` " (Empty)") :`true` " (Locked)") (select `bool` (`/Game/Blueprints/Objects/ObjectEntry_Master.IsDead` _asobject_entry_container) :`true` "(Destroyed)")) _widgetref_4)
                                (set `/Game/Blueprints/Gamemode/HoverUI_Widget.ItemRarity` "NewEnumerator3" _widgetref_4))
                              (:`CastFailed`
                                (bind _asitem_entry_master (cast `/Game/Blueprints/Inventory/ItemEntry_Master` _hoveractortarget_2)
                                  (:`then`
                                    (bind (_itemname_2 _itemdescription_2 _itemrarity_2) (break `/Game/Blueprints/Data/ItemID_Struct` (`/Game/Blueprints/Inventory/ItemEntry_Master.ItemData` _asitem_entry_master)))
                                    (bind _stack_2 (`/Game/Blueprints/Inventory/ItemEntry_Master.Stack` _asitem_entry_master))
                                    (set `/Game/Blueprints/Gamemode/HoverUI_Widget.ItemText` (`KismetStringLibrary.Concat_StrStr` _itemname_2 (select `bool` (== _stack_2 1) :`false` (`KismetStringLibrary.Concat_StrStr` " (" (`KismetStringLibrary.Conv_IntToString` _stack_2) ")") :`true` (select `bool` (== (`/Game/Blueprints/Inventory/ItemEntry_Master.CurrentAmmo` _asitem_entry_master) 0) :`false` (`KismetStringLibrary.Concat_StrStr` " (" "Loaded" ")")))) _widgetref)
                                    (set `/Game/Blueprints/Gamemode/HoverUI_Widget.ItemRarity` _itemrarity_2 _widgetref))
                                  (:`CastFailed`
                                    (bind _asenemy_entry_master (cast `/Game/Blueprints/Enemies/EnemyEntry_Master` _hoveractortarget_2)
                                      (:`then`
                                        (set `/Game/Blueprints/Gamemode/HoverUI_Widget.ItemText` (`KismetStringLibrary.Concat_StrStr` (`/Game/Blueprints/Enemies/EnemyEntry_Master.Enemy Name` _asenemy_entry_master) (select `bool` (`/Game/Blueprints/Enemies/EnemyEntry_Master.IsDead` _asenemy_entry_master) :`true` " (Dead)")) _widgetref_3)
                                        (set `/Game/Blueprints/Gamemode/HoverUI_Widget.ItemRarity` "NewEnumerator5" _widgetref_3))
                                      (:`CastFailed`
                                        (goto _label_2))))))))))
                      (:`Is Not Valid`
                        (goto _label_2)))))))
            (:`Is Not Valid`
              (bind _asenemy_entry_master_2 (cast `/Game/Blueprints/Enemies/EnemyEntry_Master` _hoveractortarget :!label _label_3)
                (:`then`
                  (if (`/Game/Blueprints/Enemies/EnemyEntry_Master.Fog_Visible` _asenemy_entry_master_2)
                    (goto _label)))
                (:`CastFailed`
                  (goto _label))))))
        (:`CastFailed`
          (goto _label_3))))))

(fn `UserConstructionScript`)