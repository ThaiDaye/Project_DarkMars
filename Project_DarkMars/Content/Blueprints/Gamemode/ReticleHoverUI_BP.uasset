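; World-space aiming reticle actor that follows the top-down character's aim and shows its widget component only while the player is aiming.
; On BeginPlay it caches the first BP_TopDownCharacter and hands itself to ReticleHoverUI_Widget.
; Each tick it moves to AimTargetHitLocation.
; For non-focus aiming with one weapon equip type, it instead projects the cursor hit onto the TraceAim line, clamped to melee reach and trace end.
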(event `self.ReceiveBeginPlay`
  (bind _outactors (`GameplayStatics.GetAllActorsOfClass` "/Game/Blueprints/BP_TopDownCharacter.BP_TopDownCharacter_C"))
  (set `self.PlayerRef` (`|GetArrayItem` _outactors))
  (bind _asreticle_hover_ui_widget (cast `/Game/Blueprints/Gamemode/ReticleHoverUI_Widget` (`WidgetComponent.GetWidget` (`self.Widget`))))
  (set `self.WidgetRef` _asreticle_hover_ui_widget)
  (set `/Game/Blueprints/Gamemode/ReticleHoverUI_Widget.HoverRef` self _asreticle_hover_ui_widget))

(event `self.ReceiveTick`
  (params (DeltaSeconds :type "Float (single-precision)"))
  (bind _playerref (`self.PlayerRef`))
  (bind _playerref_2 (`self.PlayerRef`))
  (bind _widget (`self.Widget`))
  (bind _trace_aim (`/Game/Blueprints/BP_TopDownCharacter.Trace_Aim` _playerref_2))
  (bind _returnvalue (`self.K2_GetActorLocation` _trace_aim))
  (bind _endloc (`/Game/Blueprints/Gamemode/VisualTrace_BP.EndLoc` _trace_aim))
  (`/Engine/EditorBlueprintResources/StandardMacros.IsValid` _playerref
    (:`Is Valid`
      (`self.K2_SetActorLocation` (select `bool` (and (`/Game/Blueprints/BP_TopDownCharacter.Aiming` _playerref) (not (`/Game/Blueprints/BP_TopDownCharacter.FocusAiming` _playerref)) (`|EnumEquality` (`/Game/Blueprints/BP_TopDownCharacter.WeaponEquipType` _playerref) "NewEnumerator1")) :`false` (`/Game/Blueprints/BP_TopDownCharacter.AimTargetHitLocation` _playerref) :`true` (`KismetMathLibrary.FindClosestPointOnSegment` (`.Location` (`GameplayStatics.BreakHitResult` (`PlayerController.GetHitResultUnderCursorByChannel` (`GameplayStatics.GetPlayerController` 0) "TraceTypeQuery1" true))) _returnvalue (`KismetMathLibrary.FindClosestPointOnSegment` (+ _returnvalue (* (`KismetMathLibrary.Conv_RotatorToVector` (`KismetMathLibrary.FindLookAtRotation` _returnvalue _endloc)) (+ (`/Game/Blueprints/BP_TopDownCharacter.MeleeRadius` _playerref_2) (`/Game/Blueprints/BP_TopDownCharacter.MeleeRange` _playerref_2) (`CapsuleComponent.GetScaledCapsuleRadius` (`Character.CapsuleComponent` _playerref_2))))) _returnvalue _endloc))))
      (if (`/Game/Blueprints/BP_TopDownCharacter.Aiming` _playerref)
        (`SceneComponent.SetVisibility` _widget true false)
        (else
          (`SceneComponent.SetVisibility` _widget false false))))))

(fn `UserConstructionScript`)