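; VisualTrace_BP draws a straight visual trace from the top-down player character to a target point, EndLoc.
; SetVisual runs on construction and every tick, anchoring the actor at the player's WeaponOffset for two weapon equip types, otherwise at the spine_04 socket.
; It rotates the Scene toward EndLoc, stretches the mesh to that distance, and applies the Width, Material and Visible variables.
; FocusAiming does not change the chosen anchor.
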(event `self.ReceiveBeginPlay`
  (bind _outactors (`GameplayStatics.GetAllActorsOfClass` "/Game/Blueprints/BP_TopDownCharacter.BP_TopDownCharacter_C"))
  (set `self.PlayerRef` (`|GetArrayItem` _outactors)))

(event `self.ReceiveTick`
  (params (DeltaSeconds :type "Float (single-precision)"))
  (`self.SetVisual`))

(fn `SetVisual`
  (bind _staticmesh (`self.StaticMesh`))
  (bind _endloc (`self.EndLoc`))
  (bind _scene (`self.Scene`))
  (bind _width (`self.Width`))
  (bind _playerref (`self.PlayerRef`))
  (bind _returnvalue (`SceneComponent.K2_GetComponentLocation` _scene))
  (bind _weaponequiptype (`/Game/Blueprints/BP_TopDownCharacter.WeaponEquipType` _playerref))
  (bind _returnvalue_2 (`SceneComponent.K2_GetComponentLocation` (`/Game/Blueprints/BP_TopDownCharacter.WeaponOffset` _playerref)))
  (bind _returnvalue_3 (or (`|EnumEquality` _weaponequiptype "NewEnumerator2") (`|EnumEquality` _weaponequiptype "NewEnumerator3")))
  (`/Engine/EditorBlueprintResources/StandardMacros.IsValid` _playerref
    (:`Is Valid`
      (`self.K2_SetActorLocation` (select `bool` (and _returnvalue_3 (`/Game/Blueprints/BP_TopDownCharacter.FocusAiming` _playerref)) :`false` (select `bool` _returnvalue_3 :`false` (`SceneComponent.GetSocketLocation` (`Character.Mesh` _playerref) "spine_04") :`true` _returnvalue_2) :`true` _returnvalue_2)))
    (:`Is Not Valid`
      _))
  (`SceneComponent.K2_SetWorldRotation` _scene (`KismetMathLibrary.FindLookAtRotation` _returnvalue _endloc) false false)
  (`SceneComponent.SetWorldScale3D` _staticmesh (`KismetMathLibrary.MakeVector` _width _width (* (`KismetMathLibrary.VSize` (- _returnvalue _endloc)) 0.01)))
  (`PrimitiveComponent.SetMaterial` _staticmesh 0 (`self.Material`))
  (`SceneComponent.SetVisibility` _staticmesh (`self.Visible`) false))

(fn `UserConstructionScript`
  (`self.SetVisual`))