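; Master room actor that builds a grid room from painted Door, WallNoWall and Objects marker instances.
; Line traces per cell pick floor or wall art, with perimeter walls by default, flipped by WallNoWall and opened by Door, drawn through data-table-driven HISM components.
; The construction script previews the room with text tags on door and object markers.
; BeginPlay rebuilds it, spawns door and object actors, then has WorldGen_Master set up doors.
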(event `self.ReceiveBeginPlay`
  (bind _worldgenref (`self.WorldGenRef`))
  (`self.GenerateRoom`)
  (bind _outactors (`GameplayStatics.GetAllActorsOfClass` "/Game/Blueprints/WorldGen_Master.WorldGen_Master_C"))
  (set `self.WorldGenRef` (`|GetArrayItem` _outactors))
  (`self.GenerateObjects`)
  (`/Game/Blueprints/WorldGen_Master.SetupDoors` _worldgenref)
  (`/Game/Blueprints/WorldGen_Master.SetupAutoDoors` _worldgenref))

(fn `GenerateObjectDebugTags`
  (bind _objects (`self.Objects`))
  (bind _door (`self.Door`))
  (for _index (range (`InstancedStaticMeshComponent.GetInstanceCount` _objects))
    (bind _returnvalue (`AddComponent|NODE_AddTextRenderComponent-0` :`RelativeTransform` (`KismetMathLibrary.MakeTransform` (`KismetMathLibrary.MakeVector` (.x (.location (`InstancedStaticMeshComponent.GetInstanceTransform` _objects _index false))) (.y (.location (`InstancedStaticMeshComponent.GetInstanceTransform` _objects _index false))) 350.0) (struct :`Pitch` 90.0 :`Yaw` 180.0))))
    (bind _output (`|GetArrayItem` (`self.Objects_Data`) _index))
    (bind _returnvalue_2 (`KismetSystemLibrary.IsValidClass` _output))
    (bind _returnvalue_3 (`|GetDataTableRow` "/Game/Blueprints/Data/ObjectID_Table.ObjectID_Table" (select `bool` _returnvalue_2 :`false` (`|GetArrayItem` (`self.Objects_DataID`) _index)))
      (:`then`
        _)
      (:`RowNotFound`
        _))
    (`TextRenderComponent.K2_SetText` _returnvalue (`KismetTextLibrary.Conv_StringToText` (`KismetStringLibrary.Concat_StrStr` "#" (`KismetStringLibrary.Conv_IntToString` _index) " \n" (select `bool` _returnvalue_2 :`false` (`.ObjectName_29_A149150649B7F1F4BC9EF89D8B87C088` (break `/Game/Blueprints/Data/ObjectID_Struct` _returnvalue_3)) :`true` (`.RightS` (`KismetStringLibrary.Split` (`KismetStringLibrary.LeftChop` (`KismetSystemLibrary.GetClassDisplayName` (select `bool` _returnvalue_2 :`false` "/Game/Blueprints/Objects/ObjectEntry_Master.ObjectEntry_Master_C" :`true` _output)) 2) "ObjectEntry_")))))))
  (for _index_2 (range (`InstancedStaticMeshComponent.GetInstanceCount` _door))
    (bind _returnvalue_4 (`AddComponent|NODE_AddTextRenderComponent-1` :`RelativeTransform` (`KismetMathLibrary.MakeTransform` (`KismetMathLibrary.MakeVector` (.x (.location (`InstancedStaticMeshComponent.GetInstanceTransform` _door _index_2 false))) (.y (.location (`InstancedStaticMeshComponent.GetInstanceTransform` _door _index_2 false))) 400.0) (struct :`Pitch` 90.0 :`Yaw` 180.0))))
    (`TextRenderComponent.K2_SetText` _returnvalue_4 (`KismetTextLibrary.Conv_StringToText` (`KismetStringLibrary.Concat_StrStr` "#" (`KismetStringLibrary.Conv_IntToString` _index_2) " \n" (select `int` (`|GetArrayItem` (`self.Doors_Type`) _index_2) :`0` "Door" :`1` "Locked" :`2` "AutoDoor"))))))

(fn `GenerateObjects`
  (bind _objects (`self.Objects`))
  (bind _door (`self.Door`))
  ;[1 1 1] doors
  (for _index (range (`InstancedStaticMeshComponent.GetInstanceCount` _door))
    (bind _output (`|GetArrayItem` (`self.Doors_Type`) _index))
    (bind _rotation (.rotation (`InstancedStaticMeshComponent.GetInstanceTransform` _door _index true)))
    (bind _returnvalue (`|SpawnActorFromClass` (select `int` _output :`0` "/Game/Blueprints/Objects/ObjectEntry_Door.ObjectEntry_Door_C" :`1` "/Game/Blueprints/Objects/ObjectEntry_Door.ObjectEntry_Door_C" :`2` "/Game/Blueprints/Objects/ObjectEntry_AutoDoor.ObjectEntry_AutoDoor_C" :!type "/Game/Blueprints/Objects/ObjectEntry_Master Class Reference") (`KismetMathLibrary.MakeTransform` (+ (`KismetMathLibrary.MakeVector` (.x (.location (`InstancedStaticMeshComponent.GetInstanceTransform` _door _index true))) (.y (.location (`InstancedStaticMeshComponent.GetInstanceTransform` _door _index true)))) (* (`KismetMathLibrary.Conv_RotatorToVector` _rotation) 0.1)) _rotation) "AlwaysSpawn" "OverrideRootScale" null "None" "NewEnumerator0" null null))
    (bind _asobject_entry_door (cast `/Game/Blueprints/Objects/ObjectEntry_Door` _returnvalue)
      (:`then`
        (set `/Game/Blueprints/Objects/ObjectEntry_Door.Locked` (select `int` _output :`0` false :`1` true :`2` false) _asobject_entry_door)
        (set `/Game/Blueprints/Objects/ObjectEntry_Door.Open` false _asobject_entry_door)
        (`/Game/Blueprints/Objects/ObjectEntry_Door.SetDoorVisuals` _asobject_entry_door)
        (set `/Game/Blueprints/Objects/ObjectEntry_Door.IndestructableDoors` true _asobject_entry_door))
      (:`CastFailed`
        _))
    (set `/Game/Blueprints/Objects/ObjectEntry_Master.Debug_KeepOnWorldGen` true _returnvalue))
  ;[1 1 1] objects
  (for _index_2 (range (`InstancedStaticMeshComponent.GetInstanceCount` _objects))
    (bind _returnvalue_2 (`KismetMathLibrary.MakeVector` (.x (.location (`InstancedStaticMeshComponent.GetInstanceTransform` _objects _index_2 true))) (.y (.location (`InstancedStaticMeshComponent.GetInstanceTransform` _objects _index_2 true)))))
    (bind _outhit (`KismetSystemLibrary.LineTraceSingleForObjects` :`Start` (+ _returnvalue_2 (0.0 0.0 500.0)) :`End` _returnvalue_2 :`ObjectTypes` (`|MakeArray` "ObjectTypeQuery8" :!type "EObjectTypeQuery Enum") :`bIgnoreSelf` false))
    (bind _output_2 (`|GetArrayItem` (`self.Objects_Data`) _index_2))
    (bind _returnvalue_3 (`KismetSystemLibrary.IsValidClass` _output_2))
    (bind (_bblockinghit _binitialoverlap _time _distance _location) (`GameplayStatics.BreakHitResult` _outhit))
    (bind _returnvalue_4 (`|SpawnActorFromClass` (select `bool` _returnvalue_3 :`false` "/Game/Blueprints/Objects/ObjectEntry_Master.ObjectEntry_Master_C" :`true` _output_2) (`KismetMathLibrary.MakeTransform` (select `bool` _bblockinghit :`false` _returnvalue_2 :`true` _location) (.rotation (`InstancedStaticMeshComponent.GetInstanceTransform` _objects _index_2 true))) "AlwaysSpawn" "OverrideRootScale" null (select `bool` _returnvalue_3 :`false` (`|GetArrayItem` (`self.Objects_DataID`) _index_2)) "NewEnumerator0" null null))
    (set `/Game/Blueprints/Objects/ObjectEntry_Master.Debug_KeepOnWorldGen` true _returnvalue_4)))

(fn `GenerateRoom`
  (locals (XRef :type Integer) (YRef :type Integer))
  (bind _xref (`local.XRef`))
  (bind _yref (`local.YRef`))
  (bind _floor_artenty (`self.Floor_ArtEnty`))
  (bind _wall_artenty (`self.Wall_ArtEnty`))
  (bind _returnvalue (or (== _xref 0) (== _yref 0) (== (`self.X`) _xref) (== (`self.Y`) _yref)))
  (bind _returnvalue_2 (`KismetMathLibrary.MakeVector` (* (* (`local.XRef`) (`self.GridSize`)) -1.0) (* (`local.YRef`) (`self.GridSize`)) 50.0))
  (bind _returnvalue_3 (+ (`self.K2_GetActorLocation`) _returnvalue_2))
  (`self.GenerateVisualInstanceMesh`)
  (for _index (range (+ (`self.X`) 1))
    (set `local.XRef` _index)
    (for _index_2 (range (+ (`self.Y`) 1))
      (set `local.YRef` _index_2)
      (bind _outhit (`KismetSystemLibrary.LineTraceSingleForObjects` :`Start` (+ _returnvalue_3 (0.0 0.0 1000.0)) :`End` (+ _returnvalue_3 (0.0 0.0 -1000.0)) :`ObjectTypes` (`|MakeArray` "ObjectTypeQuery5" :!type "EObjectTypeQuery Enum") :`bIgnoreSelf` false))
      (bind (_bblockinghit _binitialoverlap _time _distance _location _impactpoint _normal _impactnormal _physmat _hitactor _hitcomponent) (`GameplayStatics.BreakHitResult` _outhit))
      (bind (_instanceactor _entry_data) (`self.GetEntryVisualData` (select `bool` (== _hitcomponent (`self.Door`)) :`false` (select `bool` (== _hitcomponent (`self.Wall/NoWall`)) :`false` (select `bool` _returnvalue :`false` _floor_artenty :`true` _wall_artenty) :`true` (select `bool` _returnvalue :`false` _wall_artenty :`true` _floor_artenty)) :`true` _floor_artenty) true))
      (`InstancedStaticMeshComponent.AddInstance` _instanceactor (`KismetMathLibrary.MakeTransform` (+ _returnvalue_2 (.location (`.Transform_14_97A00E1140F889FE27B143846CA6B0D5` (break `/Game/Blueprints/Data/EntryID_Struct` _entry_data)))) (struct) (.scale (`.Transform_14_97A00E1140F889FE27B143846CA6B0D5` (break `/Game/Blueprints/Data/EntryID_Struct` _entry_data)))) false)))
  (`PrimitiveComponent.SetCollisionResponseToAllChannels` (`self.Wall/NoWall`) "ECR_Ignore")
  (`PrimitiveComponent.SetCollisionResponseToAllChannels` (`self.Door`) "ECR_Ignore")
  (`PrimitiveComponent.SetCollisionResponseToAllChannels` (`self.Objects`) "ECR_Ignore"))

(fn `GenerateVisualInstanceMesh`
  (bind _entry_visuals_instance_mesh (`self.Entry Visuals Instance Mesh`))
  (bind _art_entry_visuals_instance_mesh (`self.Art Entry Visuals Instance Mesh`))
  ;[1 1 1] Craete Instance Masters
  (for _array_element _entry_visuals_instance_mesh
    (`ActorComponent.K2_DestroyComponent` _array_element))
  (`KismetArrayLibrary.Array_Clear` _entry_visuals_instance_mesh)
  (bind _outrownames (`DataTableFunctionLibrary.GetDataTableRowNames` "/Game/Blueprints/Data/EntryID_Table.EntryID_Table"))
  (for _array_element_2 _outrownames
    (bind _returnvalue (`|GetDataTableRow` "/Game/Blueprints/Data/EntryID_Table.EntryID_Table" _array_element_2)
      (:`then`
        (bind _returnvalue_2 (`AddComponent|NODE_AddHierarchicalInstancedStaticMeshComponent-0` :`RelativeTransform` (`KismetMathLibrary.MakeTransform` (0.0 0.0 0.0))))
        (if (`self.Debug_UseCulling`)
          (`InstancedStaticMeshComponent.SetCullDistances` _returnvalue_2 5000 5000))
        (bind (_id _name _material _mesh _transform _notvisible _nocollision) (break `/Game/Blueprints/Data/EntryID_Struct` _returnvalue))
        (if _nocollision
          (`PrimitiveComponent.SetCollisionEnabled` _returnvalue_2 "QueryOnly"))
        (if _notvisible
          (`PrimitiveComponent.SetCollisionObjectType` _returnvalue_2 "ECC_GameTraceChannel8")
          (`PrimitiveComponent.SetCollisionResponseToChannel` _returnvalue_2 "ECC_Visibility" "ECR_Ignore")
          (`PrimitiveComponent.SetCollisionResponseToChannel` _returnvalue_2 "ECC_Camera" "ECR_Ignore")
          (`SceneComponent.SetVisibility` _returnvalue_2 false false))
        (`StaticMeshComponent.SetStaticMesh` _returnvalue_2 _mesh)
        (for (_array_element_3 _array_index) _material
          (`PrimitiveComponent.SetMaterial` _returnvalue_2 _array_index _array_element_3))
        (`KismetArrayLibrary.Array_Add` (`self.Entry Visuals Instance Mesh`) _returnvalue_2))))
  ;[1 1 1] generate art entries
  (for _array_element_4 _art_entry_visuals_instance_mesh
    (`ActorComponent.K2_DestroyComponent` _array_element_4))
  (`KismetArrayLibrary.Array_Clear` _art_entry_visuals_instance_mesh)
  (bind _outrownames_2 (`DataTableFunctionLibrary.GetDataTableRowNames` "/Game/Blueprints/Data/ArtEntryID_Table.ArtEntryID_Table"))
  (for _array_element_5 _outrownames_2
    (bind _returnvalue_3 (`|GetDataTableRow` "/Game/Blueprints/Data/ArtEntryID_Table.ArtEntryID_Table" _array_element_5)
      (:`then`
        (bind _returnvalue_4 (`AddComponent|NODE_AddHierarchicalInstancedStaticMeshComponent-1` :`RelativeTransform` (`KismetMathLibrary.MakeTransform` (0.0 0.0 0.0))))
        (if (`self.Debug_UseCulling`)
          (`InstancedStaticMeshComponent.SetCullDistances` _returnvalue_4 5000 5000))
        (bind (_id_2 _name_2 _material_2 _mesh_2 _transform_2 _notvisible_2 _nocollision_2) (break `/Game/Blueprints/Data/EntryID_Struct` _returnvalue_3))
        (if _nocollision_2
          (`PrimitiveComponent.SetCollisionEnabled` _returnvalue_4 "QueryOnly"))
        (if _notvisible_2
          (`PrimitiveComponent.SetCollisionObjectType` _returnvalue_4 "ECC_GameTraceChannel8")
          (`PrimitiveComponent.SetCollisionResponseToChannel` _returnvalue_4 "ECC_Visibility" "ECR_Ignore")
          (`PrimitiveComponent.SetCollisionResponseToChannel` _returnvalue_4 "ECC_Camera" "ECR_Ignore")
          (`SceneComponent.SetVisibility` _returnvalue_4 false false))
        (`StaticMeshComponent.SetStaticMesh` _returnvalue_4 _mesh_2)
        (for (_array_element_6 _array_index_2) _material_2
          (`PrimitiveComponent.SetMaterial` _returnvalue_4 _array_index_2 _array_element_6))
        (`KismetArrayLibrary.Array_Add` (`self.Art Entry Visuals Instance Mesh`) _returnvalue_4)))))

(fn `GetEntryVisualData`
  (params (ID :type Integer) (ArtVersion :type Boolean))
  (returns (InstanceActor :type "InstancedStaticMeshComponent Object Reference") (`Entry Data` :type "/Game/Blueprints/Data/EntryID_Struct Structure"))
  (if ArtVersion
    (bind _returnvalue (`|GetDataTableRow` "/Game/Blueprints/Data/ArtEntryID_Table.ArtEntryID_Table" (`KismetStringLibrary.Conv_StringToName` (`KismetStringLibrary.Conv_IntToString` ID)))
      (:`then`
        (return (`|GetArrayItem` (`self.Art Entry Visuals Instance Mesh`) (+ ID 1)) _returnvalue)))
    (else
      (bind _returnvalue_2 (`|GetDataTableRow` "/Game/Blueprints/Data/EntryID_Table.EntryID_Table" (`KismetStringLibrary.Conv_StringToName` (`KismetStringLibrary.Conv_IntToString` ID)))
        (:`then`
          (return (`|GetArrayItem` (`self.Entry Visuals Instance Mesh`) (+ ID 1)) _returnvalue_2))))))

(fn `UserConstructionScript`
  (`self.GenerateRoom`)
  (`self.GenerateObjectDebugTags`))