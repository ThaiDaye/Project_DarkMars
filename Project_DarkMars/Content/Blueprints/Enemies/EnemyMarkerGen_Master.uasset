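; Enemy spawn marker that loads and unloads an enemy during play, with debug spheres showing its state.
; While the player overlaps its sphere after world generation, it retries spawning every few seconds, only out of line of sight or far away, under a world enemy cap.
; Spawns get a weighted, seeded start state, overridden when machine-attached, plus Vaper rust-cloud setup.
; UnloadEnemy moves the marker to the enemy before destroying it, permanently retiring markers whose enemy died.
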(event `self.ReceiveBeginPlay`
  ;[1 1 1] begin
  (bind _outactors (`GameplayStatics.GetAllActorsOfClass` "/Game/Blueprints/BP_TopDownCharacter.BP_TopDownCharacter_C"))
  (set `self.PlayerRef` (`|GetArrayItem` _outactors))
  (bind _outactors_2 (`GameplayStatics.GetAllActorsOfClass` "/Game/Blueprints/WorldGen_Master.WorldGen_Master_C"))
  (set `self.WorldRef` (`|GetArrayItem` _outactors_2))
  (`SceneComponent.SetHiddenInGame` (`self.LoadedSphere`) (`/Game/Blueprints/WorldGen_Master.Debug_HideEnemyGenMarkers` (`self.WorldRef`)) false)
  (`SceneComponent.SetHiddenInGame` (`self.DeadSphere`) (`/Game/Blueprints/WorldGen_Master.Debug_HideEnemyGenMarkers` (`self.WorldRef`)) false)
  (`SceneComponent.SetHiddenInGame` (`self.AttemptLoadSphere`) (`/Game/Blueprints/WorldGen_Master.Debug_HideEnemyGenMarkers` (`self.WorldRef`)) false)
  (`SceneComponent.SetHiddenInGame` (`self.SphereSpawn`) (`/Game/Blueprints/WorldGen_Master.Debug_HideEnemyGenMarkers` (`self.WorldRef`)) false)
  (`SceneComponent.SetHiddenInGame` (`self.Sphere`) (`/Game/Blueprints/WorldGen_Master.Debug_HideEnemyGenMarkers` (`self.WorldRef`)) false))

(event `self.Sphere.OnComponentBeginOverlap`
  (params (OverlappedComponent :type "PrimitiveComponent Object Reference") (OtherActor :type "Actor Object Reference") (OtherComp :type "PrimitiveComponent Object Reference") (OtherBodyIndex :type Integer) (bFromSweep :type Boolean) (SweepResult :type "HitResult Structure (by ref)"))
  (bind (_returnvalue_x _returnvalue_y) (`KismetMathLibrary.BreakVector` (`self.K2_GetActorLocation`)))
  (bind (_returnvalue_x_2 _returnvalue_y_2) (`KismetMathLibrary.BreakVector` (`self.K2_GetActorLocation` (`self.PlayerRef`))))
  (bind _returnvalue (`KismetMathLibrary.MakeVector` _returnvalue_x _returnvalue_y 200.0))
  (bind _returnvalue_2 (`KismetMathLibrary.MakeVector` _returnvalue_x_2 _returnvalue_y_2 200.0))
  ;[1 1 1] check load
  (`self.DoAfterWorldGen`
    (:`GenComplete`
      (if (== OtherActor (`self.PlayerRef`))
        (`|ExecutionSequence`
          (:`then_0`
            (goto _label :!via `Open`))
          (:`then_1`
            (`/Engine/EditorBlueprintResources/StandardMacros.Gate` true :!label _label
              (:`Exit`
                (`|ExecutionSequence`
                  (:`then_0`
                    (if (`self.Loaded`)
                      _
                      (elif (not (`self.EntryIsDead`))
                        (bind _outhit (`KismetSystemLibrary.LineTraceSingleForObjects` :`Start` _returnvalue :`End` _returnvalue_2 :`ObjectTypes` (`|MakeArray` "ObjectTypeQuery2" "ObjectTypeQuery8" :!type "EObjectTypeQuery Enum") :`DrawTime` 1.0))
                        (if (`GameplayStatics.BreakHitResult` _outhit)
                          (bind _randomlocation (`NavigationSystemV1.K2_GetRandomLocationInNavigableRadius` (`self.K2_GetActorLocation`) 10.0 null null :!label _label_2))
                          (`self.LoadEnemy` _randomlocation)
                          (elif (> (`KismetMathLibrary.VSize` (- _returnvalue _returnvalue_2)) 2000.0)
                            (goto _label_2)
                            (else
                              (`SceneComponent.SetVisibility` (`self.Sphere`) false false)
                              (`SceneComponent.SetVisibility` (`self.DeadSphere`) false false)
                              (`SceneComponent.SetVisibility` (`self.LoadedSphere`) false false)
                              (`SceneComponent.SetVisibility` (`self.SphereSpawn`) false false)
                              (`SceneComponent.SetVisibility` (`self.AttemptLoadSphere`) true false)))))))
                  (:`then_1`
                    (`KismetSystemLibrary.Delay` 2.0)
                    (goto _label)))))))))))

(event `self.Sphere.OnComponentEndOverlap`
  (params (OverlappedComponent :type "PrimitiveComponent Object Reference") (OtherActor :type "Actor Object Reference") (OtherComp :type "PrimitiveComponent Object Reference") (OtherBodyIndex :type Integer))
  ;[1 1 1] check load
  (`self.DoAfterWorldGen`
    (:`GenComplete`
      (if (== OtherActor (`self.PlayerRef`))
        (`|ExecutionSequence`
          (:`then_0`
            (goto _label :!via `Close`))
          (:`then_1`
            (if (not (`self.Loaded`))
              (`SceneComponent.SetVisibility` (`self.DeadSphere`) false false)
              (`SceneComponent.SetVisibility` (`self.LoadedSphere`) false false)
              (`SceneComponent.SetVisibility` (`self.AttemptLoadSphere`) false false)
              (`SceneComponent.SetVisibility` (`self.Sphere`) true false)
              (`SceneComponent.SetVisibility` (`self.SphereSpawn`) true false))))))))

(event `LoadEnemy`
  (params (Location :type "Vector Structure"))
  (bind _enemyentryref (`self.EnemyEntryRef`))
  (bind _enemyentryref_2 (`self.EnemyEntryRef`))
  (bind _enemyentryref_3 (`self.EnemyEntryRef`))
  ;[1 1 1] load
  (bind _alive (`self.GetAliveEnemies`))
  (if (>= _alive (`/Game/Blueprints/WorldGen_Master.MaxEnemySpawn` (`self.WorldRef`)))
    _
    (elif (not (or (`self.Loaded`) (`self.EntryIsDead`)))
      (bind _returnvalue (`AIBlueprintHelperLibrary.SpawnAIFromClass` (`self.Enemy Class`) null Location (`KismetMathLibrary.MakeRotator` 0.0 0.0 (`KismetMathLibrary.RandomFloatInRange` -180.0 180.0)) true null))
      (set `self.Loaded` true)
      (bind _asenemy_entry_master (cast `/Game/Blueprints/Enemies/EnemyEntry_Master` _returnvalue))
      (set `self.EnemyEntryRef` _asenemy_entry_master)
      (set `/Game/Blueprints/Enemies/EnemyEntry_Master.EnemyGenRef` self _enemyentryref_2)
      (set `self.FoundStartState` false)
      (for _array_element (`/Game/Blueprints/Enemies/EnemyEntry_Master.SpawnStartStates` _enemyentryref_2)
        (if (not (`self.FoundStartState`))
          (bind (_startstate _weight) (break `/Game/Blueprints/Data/EnemyStartStateWeight_Struct` _array_element))
          (if (`KismetMathLibrary.RandomBoolWithWeightFromStream` _weight (`KismetMathLibrary.MakeRandomStream` (`/Game/Blueprints/Enemies/EnemyEntry_Master.UniqueNum` _enemyentryref_2)))
            (set `self.FoundStartState` true)
            (`/Game/Blueprints/Enemies/EnemyEntry_Master.SetStartingState` _enemyentryref (select `bool` (`self.AttachedToMachine`) :`false` _startstate :`true` "NewEnumerator3")))))
      (if (not (`self.FoundStartState`))
        (`/Game/Blueprints/Enemies/EnemyEntry_Master.SetStartingState` _enemyentryref (select `bool` (`self.AttachedToMachine`) :`false` (`/Game/Blueprints/Enemies/EnemyEntry_Master.Start Type` _enemyentryref) :`true` "NewEnumerator3")))
      (set `/Game/Blueprints/Enemies/EnemyEntry_Master.IsReadyForDespawn` (not (`PrimitiveComponent.IsOverlappingActor` (`/Game/Blueprints/WorldGen_Master.SpawnSphereMax` (`self.WorldRef`)) _enemyentryref_3)) _enemyentryref_3)
      (`SceneComponent.SetVisibility` (`self.Sphere`) false false)
      (`SceneComponent.SetVisibility` (`self.DeadSphere`) false false)
      (`SceneComponent.SetVisibility` (`self.AttemptLoadSphere`) false false)
      (`SceneComponent.SetVisibility` (`self.SphereSpawn`) false false)
      (`SceneComponent.SetVisibility` (`self.LoadedSphere`) true false)
      (bind _asenemy_entry_vaper (cast `/Game/Blueprints/Enemies/EnemyEntry_Vaper` (`self.EnemyEntryRef`)))
      (set `/Game/Blueprints/Enemies/EnemyEntry_Vaper.RustSpawnWithCloud` (`self.SpawnWithRustCloud`) _asenemy_entry_vaper)
      (`/Game/Blueprints/Enemies/EnemyEntry_Vaper.SpawnRustCloud` _asenemy_entry_vaper))))

(event `UnloadEnemy`
  (bind _enemyentryref (`self.EnemyEntryRef`))
  ;[1 1 1] unload
  (if (`self.Loaded`)
    (`/Engine/EditorBlueprintResources/StandardMacros.IsValid` _enemyentryref
      (:`Is Valid`
        (`self.K2_SetActorLocation` (`KismetMathLibrary.MakeVector` (.x (`self.K2_GetActorLocation` _enemyentryref)) (.y (`self.K2_GetActorLocation` _enemyentryref)) (.z (`self.K2_GetActorLocation`))))
        (if (`/Game/Blueprints/Enemies/EnemyEntry_Master.IsDead` _enemyentryref)
          (set `self.EntryIsDead` true)
          (`self.K2_DestroyActor` (`self.EnemyEntryRef`))
          (`SceneComponent.SetVisibility` (`self.DeadSphere`) true false)
          (`SceneComponent.SetVisibility` (`self.LoadedSphere`) false false)
          (`SceneComponent.SetVisibility` (`self.Sphere`) false false)
          (`SceneComponent.SetVisibility` (`self.AttemptLoadSphere`) false false)
          (`SceneComponent.SetVisibility` (`self.SphereSpawn`) false false)
          (else
            (`self.K2_DestroyActor` _enemyentryref)
            (set `self.Loaded` false :!label _label_3)
            (set `self.EnemyEntryRef` null)
            (`SceneComponent.SetVisibility` (`self.Sphere`) true false)
            (`SceneComponent.SetVisibility` (`self.SphereSpawn`) true false)
            (`SceneComponent.SetVisibility` (`self.LoadedSphere`) false false)
            (`SceneComponent.SetVisibility` (`self.DeadSphere`) false false)
            (`SceneComponent.SetVisibility` (`self.AttemptLoadSphere`) false false))))
      (:`Is Not Valid`
        (goto _label_3)))))

(fn `GetAliveEnemies`
  (returns (Alive :type Integer))
  (locals (AliveEnemy :type Integer :default 0))
  (bind _outactors (`GameplayStatics.GetAllActorsOfClass` "/Game/Blueprints/Enemies/EnemyEntry_Master.EnemyEntry_Master_C"))
  (for _array_element _outactors
    (if (not (`/Game/Blueprints/Enemies/EnemyEntry_Master.IsDead` _array_element))
      (`/Engine/EditorBlueprintResources/StandardMacros.IncrementInt` (`local.AliveEnemy`))))
  (return (`local.AliveEnemy`)))

(fn `UserConstructionScript`)