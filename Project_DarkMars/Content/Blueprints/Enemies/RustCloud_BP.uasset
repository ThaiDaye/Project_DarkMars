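; RustCloud_BP is an enemy rust cloud that expands over a snapped grid up to a set radius once world generation completes.
; Timers grow RadiusRatio and rerun SetRustCloud, which sizes the spheres and Niagara effect and fills a new HISM component with cells.
; Traces skip cells held by other clouds or blocked by obstacles and doors.
; Old instance components are destroyed unless AddToCloud has restarted growth.
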(event `self.ReceiveBeginPlay`
  (bind _outactors (`GameplayStatics.GetAllActorsOfClass` "/Game/Blueprints/WorldGen_Master.WorldGen_Master_C"))
  (set `self.WorldGen` (`|GetArrayItem` _outactors))
  (set `self.RadiusRatio` (select `bool` (`self.SpawnFilled`) :`true` 1.0))
  (`self.SetRustCloud`)
  (`self.DoAfterWorldGen`
    (:`GenComplete`
      (`KismetSystemLibrary.K2_SetTimerDelegate` (delegate `TickRatioGrow`) (`self.ExpandRate`) true)
      (`KismetSystemLibrary.K2_SetTimer` null "SetRustCloud" 1.0 true))))

(event `TickRatioGrow`
  (bind _output_get (set `self.RadiusRatio` (`KismetMathLibrary.FClamp` (+ (`self.RadiusRatio`) 0.01))))
  (if (== _output_get 1.0)
    (set `self.Growing` false)
    (else
      (set `self.Growing` true))))

(event `AddToCloud`
  (set `self.Adding` true)
  (set `self.RadiusRatio` 0.0))

(fn `SetRustCloud`
  (locals (X :type Integer) (Y :type Integer) (DoorHit :type Boolean :default false) (FoundOtherCloud :type Boolean :default false))
  (bind _lastinstancemanager (`self.LastInstanceManager`))
  (bind _currentinstancemanager (`self.CurrentInstanceManager`))
  (bind _gridsize (`self.GridSize`))
  (bind _currentinstancemanager_2 (`self.CurrentInstanceManager`))
  (bind _returnvalue (`SphereComponent.GetScaledSphereRadius` (`self.RustRadius`)))
  (bind _returnvalue_2 (* (`self.RadiusRatio`) (`self.Radius`)))
  (bind (_x _y) (`KismetMathLibrary.BreakVector3f` (`KismetMathLibrary.Vector_SnappedToGrid` (`self.K2_GetActorLocation`) (`self.GridSize`))))
  (bind (_x_2 _y_2) (`KismetMathLibrary.BreakVector3f` (`KismetMathLibrary.Vector_SnappedToGrid` (`self.K2_GetActorLocation`) (`self.GridSize`))))
  (bind _returnvalue_3 (`KismetMathLibrary.MakeVector` _x_2 _y_2 150.0))
  (bind _returnvalue_4 (`KismetMathLibrary.FTrunc` (/ (* (`SphereComponent.GetScaledSphereRadius` (`self.RustRadius`)) 2.0) (`self.GridSize`))))
  (bind _returnvalue_5 (`KismetMathLibrary.Vector_SnappedToGrid` (`KismetMathLibrary.MakeVector` (+ (- (.x (`self.K2_GetActorLocation`)) _returnvalue) (* (`local.X`) _gridsize)) (+ (- (.y (`self.K2_GetActorLocation`)) _returnvalue) (* (`local.Y`) _gridsize))) (`self.GridSize`)))
  (bind (_x_3 _y_3) (`KismetMathLibrary.BreakVector3f` _returnvalue_5))
  (bind (_x_4 _y_4) (`KismetMathLibrary.BreakVector3f` _returnvalue_5))
  (bind (_x_5 _y_5) (`KismetMathLibrary.BreakVector3f` _returnvalue_5))
  (bind (_x_6 _y_6) (`KismetMathLibrary.BreakVector3f` _returnvalue_5))
  (bind _returnvalue_6 (`KismetMathLibrary.MakeVector` _x_5 _y_5 50.0))
  (bind _returnvalue_7 (`KismetMathLibrary.MakeVector` _x_6 _y_6 150.0))
  ;[1 1 1] sphere setup
  (`SceneComponent.K2_SetWorldLocation` (`self.RustRadius`) (`KismetMathLibrary.Vector_SnappedToGrid` (`self.K2_GetActorLocation`) (`self.GridSize`)) false false)
  (`SceneComponent.K2_SetWorldLocation` (`self.MaxRadius`) (`KismetMathLibrary.Vector_SnappedToGrid` (`self.K2_GetActorLocation`) (`self.GridSize`)) false false)
  (`SceneComponent.K2_SetWorldLocation` (`self.Niagara`) (`KismetMathLibrary.Vector_SnappedToGrid` (`self.K2_GetActorLocation`) (`self.GridSize`)) false false)
  (`SphereComponent.SetSphereRadius` (`self.MaxRadius`) (`self.Radius`) false)
  (`SphereComponent.SetSphereRadius` (`self.RustRadius`) _returnvalue_2 false)
  (`FXSystemComponent.SetFloatParameter` (`self.Niagara`) "CloudRadius" _returnvalue_2)
  (if (`self.Growing`)
    ;[1 1 1] create instance manager
    (`/Engine/EditorBlueprintResources/StandardMacros.IsValid` _currentinstancemanager :!label _label
      (:`Is Valid`
        (set `self.LastInstanceManager` _currentinstancemanager))
      (:`Is Not Valid`
        _))
    (bind _returnvalue_8 (`AddComponent|NODE_AddHierarchicalInstancedStaticMeshComponent-0`))
    (set `self.CurrentInstanceManager` _returnvalue_8)
    ;[1 1 1] make grid
    (for _index (range (+ _returnvalue_4 1))
      (set `local.X` _index)
      (for _index_2 (range (+ _returnvalue_4 1))
        (set `local.Y` _index_2)
        (if (<= (`KismetMathLibrary.VSize` (- (`KismetMathLibrary.MakeVector` _x _y) (`KismetMathLibrary.MakeVector` _x_3 _y_3))) (* (`self.RadiusRatio`) (`self.Radius`)))
          ;[1 1 1] dont overlap
          (set `local.FoundOtherCloud` false)
          (bind _outhits (`KismetSystemLibrary.SphereTraceMultiForObjects` :`Start` _returnvalue_6 :`End` _returnvalue_6 :`Radius` 15.0 :`ObjectTypes` (`|MakeArray` "ObjectTypeQuery10" :!type "EObjectTypeQuery Enum") :`bIgnoreSelf` (not (`self.Adding`))))
          (for _array_element _outhits
            (bind (_bblockinghit _binitialoverlap _time _distance _location _impactpoint _normal _impactnormal _physmat _hitactor) (`GameplayStatics.BreakHitResult` _array_element))
            (if _bblockinghit
              (cast `/Game/Blueprints/Enemies/RustCloud_BP` _hitactor)
              (set `local.FoundOtherCloud` true)))
          (if (not (`local.FoundOtherCloud`))
            (bind _outhit (`KismetSystemLibrary.LineTraceSingleForObjects` :`Start` _returnvalue_3 :`End` _returnvalue_7 :`ObjectTypes` (`|MakeArray` "ObjectTypeQuery2" :!type "EObjectTypeQuery Enum") :`DrawTime` 2.0))
            (if (not (`GameplayStatics.BreakHitResult` _outhit))
              (bind _outhits_2 (`KismetSystemLibrary.LineTraceMultiForObjects` _returnvalue_3 _returnvalue_7 (`|MakeArray` "ObjectTypeQuery8" :!type "EObjectTypeQuery Enum")))
              (set `local.DoorHit` false)
              (for _array_element_2 _outhits_2
                (bind (_bblockinghit_2 _binitialoverlap_2 _time_2 _distance_2 _location_2 _impactpoint_2 _normal_2 _impactnormal_2 _physmat_2 _hitactor_2 _hitcomponent) (`GameplayStatics.BreakHitResult` _array_element_2))
                (bind _asobject_entry_door (cast `/Game/Blueprints/Objects/ObjectEntry_Door` _hitactor_2))
                (if (== (`/Game/Blueprints/Objects/ObjectEntry_Door.Door` _asobject_entry_door) _hitcomponent)
                  (set `local.DoorHit` true)))
              (if (not (`local.DoorHit`))
                (`/Engine/EditorBlueprintResources/StandardMacros.IsValid` _currentinstancemanager_2
                  (:`Is Valid`
                    (`InstancedStaticMeshComponent.AddInstance` _currentinstancemanager_2 (`KismetMathLibrary.MakeTransform` (`KismetMathLibrary.MakeVector` _x_4 _y_4 25.0) (struct) (0.5 0.5 1.0)) true)))))))))
    (if (`self.SpawnFilled`)
      (set `self.SpawnFilled` false))
    (if (not (`self.Adding`))
      (`/Engine/EditorBlueprintResources/StandardMacros.IsValid` _lastinstancemanager
        (:`Is Valid`
          (`ActorComponent.K2_DestroyComponent` _lastinstancemanager))))
    (elif (`self.SpawnFilled`)
      (goto _label))))

(fn `UserConstructionScript`
  (`self.SetRustCloud`))