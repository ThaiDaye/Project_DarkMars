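; Crimson Grass enemy, an eyed tentacle sentry that opens and closes its eye and screams at moving or attacking targets.
; A looping timer checks line of sight and speed, giving a shaking warning before a scream that shocks and staggers the target and rallies nearby enemies, then cools down.
; After world generation it may hide stealthed under an item pickup, waking when that item is gone or it takes damage.
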(event `self.Event_OnFadeComplete`
  (params (FadeIn :type Boolean))
  (bind _fadeoutmesh (`self.FadeOutMesh`))
  (if FadeIn
    (if (`self.IsDead`)
      (`SceneComponent.SetVisibility` _fadeoutmesh false false :!label _label)
      (else
        (`SceneComponent.SetVisibility` (`self.Tentacle_2_ParticleSystem`) true false)
        (`SceneComponent.SetVisibility` (`self.Tentacle_2_ParticleSystem3`) true false)
        (`SceneComponent.SetVisibility` (`self.Tentacle_2_ParticleSystem2`) true false)
        (`SceneComponent.SetVisibility` (`self.Tentacle_2_ParticleSystem4`) true false)
        (`SceneComponent.SetVisibility` _fadeoutmesh false false)))))

(event `self.EnemyFogFade`
  (params (FogFadeIn :type Boolean))
  (`parent.EnemyFogFade` FogFadeIn)
  (if (`self.IsDead`)
    (goto _label)
    (elif (not FogFadeIn)
      (`SceneComponent.SetVisibility` (`self.Tentacle_2_ParticleSystem4`) false false)
      (`SceneComponent.SetVisibility` (`self.Tentacle_2_ParticleSystem2`) false false)
      (`SceneComponent.SetVisibility` (`self.Tentacle_2_ParticleSystem3`) false false)
      (`SceneComponent.SetVisibility` (`self.Tentacle_2_ParticleSystem`) false false)
      (`SceneComponent.SetVisibility` (`self.FadeOutMesh`) true false))))

(event `self.OnDeath`
  (bind _tentacle_2_particlesystem (`self.Tentacle_2_ParticleSystem`))
  (`parent.OnDeath`)
  (`/Engine/EditorBlueprintResources/StandardMacros.IsValid` _tentacle_2_particlesystem
    (:`Is Valid`
      (`ActorComponent.K2_DestroyComponent` _tentacle_2_particlesystem)
      (`ActorComponent.K2_DestroyComponent` (`self.Tentacle_2_ParticleSystem3`))
      (`ActorComponent.K2_DestroyComponent` (`self.Tentacle_2_ParticleSystem2`))
      (`ActorComponent.K2_DestroyComponent` (`self.Tentacle_2_ParticleSystem4`)))))

(event `self.ReceiveBeginPlay`
  (set `self.MainStaticMesh` (`self.RustPool`))
  (set `self.SubStaticMeshs` (`|MakeArray` (`self.FadeOutMesh`)))
  (`parent.ReceiveBeginPlay`)
  (`self.DoAfterWorldGen`
    (:`GenComplete`
      (`self.HideUnderPickup`)
      (`self.SetVisuals`)
      (`self.SetEyeOpen`)
      (`KismetSystemLibrary.K2_SetTimerDelegate` (delegate `SearchForMovement`) 0.5 true))))

(event `SearchForMovement`
  (bind _returnvalue (`self.K2_GetActorLocation`))
  (bind (_returnvalue_x _returnvalue_y) (`KismetMathLibrary.BreakVector` (`self.K2_GetActorLocation`)))
  (bind _returnvalue_2 (`self.K2_GetActorLocation`))
  (bind _target (`self.Target`))
  (bind (_returnvalue_x_2 _returnvalue_y_2) (`KismetMathLibrary.BreakVector` (`self.K2_GetActorLocation` _target)))
  (bind _returnvalue_3 (`SceneComponent.K2_GetComponentLocation` (`self.Tentacle_2_ParticleSystem`)))
  (if (`self.IsDead`)
    _
    (elif (`self.Fleeing`)
      ;[1 1 1] wake up after item is picked up
      (`/Engine/EditorBlueprintResources/StandardMacros.IsValid` (`self.PickupHiddenUnder`)
        (:`Is Not Valid`
          (`self.Event_OnDamageTaken` 0.0)
          (bind _outhits (`KismetSystemLibrary.SphereTraceMultiForObjects` _returnvalue _returnvalue 150.0 (`|MakeArray` "ObjectTypeQuery7" :!type "EObjectTypeQuery Enum")))
          (for _array_element _outhits
            (`/Engine/EditorBlueprintResources/StandardMacros.IsValid` (`self.Target`)
              (:`Is Not Valid`
                (bind (_bblockinghit _binitialoverlap _time _distance _location _impactpoint _normal _impactnormal _physmat _hitactor) (`GameplayStatics.BreakHitResult` _array_element))
                (if _bblockinghit
                  (bind _asbp_top_down_character (cast `/Game/Blueprints/BP_TopDownCharacter` _hitactor))
                  (`self.SetTarget` _asbp_top_down_character)))))))
      (elif (`self.CanSearch`)
        (`/Engine/EditorBlueprintResources/StandardMacros.Gate` true :!label _label_2
          (:`Exit`
            (`/Engine/EditorBlueprintResources/StandardMacros.IsValid` _target
              (:`Is Valid`
                (bind _outhit (`KismetSystemLibrary.LineTraceSingleForObjects` (`KismetMathLibrary.MakeVector` _returnvalue_x _returnvalue_y 100.0) (`KismetMathLibrary.MakeVector` _returnvalue_x_2 _returnvalue_y_2 100.0) (`|MakeArray` "ObjectTypeQuery2" "ObjectTypeQuery8" :!type "EObjectTypeQuery Enum")))
                (if (`GameplayStatics.BreakHitResult` _outhit)
                  _
                  (elif (> (`KismetMathLibrary.VSize` (`self.GetVelocity` (`self.Target`))) (`self.SearchVelocityThreshold`))
                    (if (`self.IsReadyToScream`) :!label _label_3
                      (`self.PlaySFXFromSoundBank` "NewEnumerator3" (`self.K2_GetActorLocation`))
                      ;[1 1 1] alert (spooke instead of dealing damage, enemies that are nearby and have los will get a new target other markers will come over hre)
                      (bind _asbp_top_down_character_2 (cast `/Game/Blueprints/BP_TopDownCharacter` (`self.Target`)))
                      (`/Game/Blueprints/BP_TopDownCharacter.Composure_Shocked` _asbp_top_down_character_2 self 2.0)
                      (`/Game/Blueprints/BP_TopDownCharacter.TakeDamage` _asbp_top_down_character_2 0.0 0.0 (`self.Stagger Duration`) (select `bool` (> (- 1.0 (`KismetMathLibrary.FClamp` (/ (`self.GetDistanceTo` _asbp_top_down_character_2 self) (`self.AgroRadius`)))) 0.666) :`true` (`self.Knockback Amount`)) self false)
                      (set `self.IsReadyToScream` false)
                      (`self.Event_EnemyScream`)
                      (bind _outhits_2 (`KismetSystemLibrary.SphereTraceMultiForObjects` _returnvalue_2 _returnvalue_2 (`self.ScreamCallRange`) (`|MakeArray` "ObjectTypeQuery12" :!type "EObjectTypeQuery Enum")))
                      (for _array_element_2 _outhits_2
                        (if (not (>= (`self.ScreamCallCountRef`) (`self.ScreamCallMax`)))
                          (bind (_bblockinghit_2 _binitialoverlap_2 _time_2 _distance_2 _location_2 _impactpoint_2 _normal_2 _impactnormal_2 _physmat_2 _hitactor_2 _hitcomponent) (`GameplayStatics.BreakHitResult` _array_element_2))
                          (bind _asenemy_entry_master (cast `/Game/Blueprints/Enemies/EnemyEntry_Master` _hitactor_2))
                          (cast `/Game/Blueprints/Enemies/Proxies/EnemyEntry_Proxy_Master` _asenemy_entry_master
                            (:`CastFailed`
                              (cast `/Game/Blueprints/Enemies/EnemyEntry_CrimsonGrass` _asenemy_entry_master
                                (:`CastFailed`
                                  (if (== (`Character.CapsuleComponent` _asenemy_entry_master) _hitcomponent)
                                    (if (`KismetMathLibrary.RandomBoolWithWeight` (`self.ScreamCallChance`))
                                      (`self.SetTarget` _asenemy_entry_master (`self.Target`))
                                      (`self.Event_EnemyScream` _asenemy_entry_master)
                                      (`/Engine/EditorBlueprintResources/StandardMacros.IncrementInt` (`self.ScreamCallCountRef`))))))))))
                      (`NiagaraFunctionLibrary.SpawnSystemAtLocation` "/Game/VFX/Systems/ScreamRefraction_ParticleSystem.ScreamRefraction_ParticleSystem" _returnvalue_3)
                      (`self.StartScreamCooldown`)
                      (`/Game/Blueprints/BP_TopDownCharacter.ScreenShake` (`self.PlayerRef`) 2 "NewEnumerator0" 1000.0 _returnvalue_3)
                      (`KismetSystemLibrary.Delay` 2.0)
                      (`self.OverrideCloseEyes`)
                      (else
                        ;[1 1 1] warning
                        (`self.PlaySFXFromSoundBank` "NewEnumerator2" (`self.K2_GetActorLocation`))
                        (`self.ReadyToScream`)))
                    (else
                      (bind _asbp_top_down_character_3 (cast `/Game/Blueprints/BP_TopDownCharacter` (`self.Target`)))
                      (if (or (`/Game/Blueprints/BP_TopDownCharacter.MeleeAttacking` _asbp_top_down_character_3) (`/Game/Blueprints/BP_TopDownCharacter.Stomping` _asbp_top_down_character_3))
                        (goto _label_3)))))))))))))

(event `SetEyeOpen`
  (bind _tentacle_2_particlesystem (`self.Tentacle_2_ParticleSystem`))
  (bind _tentacle_2_particlesystem_2 (`self.Tentacle_2_ParticleSystem`))
  (if (`self.IsDead`)
    _
    (elif (not (`self.Fleeing`))
      (`|ExecutionSequence` :!label _label_4
        (:`then_0`
          (if (`PrimitiveComponent.IsOverlappingActor` (`self.AgroSphere`) (`self.Target`))
            (goto _label_5 :!via `Open`)))
        (:`then_1`
          (`KismetSystemLibrary.Delay` (select `bool` (`self.IsEyeClosed`) :`false` 6.0 :`true` 3.0))
          (goto _label_4))
        (:`then_2`
          (`/Engine/EditorBlueprintResources/StandardMacros.Gate` true :!label _label_5
            (:`Exit`
              (if (not (`self.IsAlertShake`))
                (bind _output_get (set `self.IsEyeClosed` (not (`self.IsEyeClosed`))))
                (if _output_get
                  (`/Engine/EditorBlueprintResources/StandardMacros.IsValid` _tentacle_2_particlesystem_2 :!label _label_6
                    (:`Is Valid`
                      (`NiagaraComponent.ReinitializeSystem` _tentacle_2_particlesystem_2) ; eye closed
                      (`FXSystemComponent.SetFloatParameter` _tentacle_2_particlesystem_2 "Dynamic_UseIrisLook" 0.0)
                      (`FXSystemComponent.SetFloatParameter` _tentacle_2_particlesystem_2 "Dynamic_EyeClosed" 1.0)
                      (`FXSystemComponent.SetFloatParameter` _tentacle_2_particlesystem_2 "Dynamic_HasTarget" 0.0))
                    (:`Is Not Valid`
                      _))
                  (set `self.IsReadyToScream` false)
                  (set `self.IsAlertShake` false)
                  (`self.PlaySFXFromSoundBank` "NewEnumerator4" (`self.K2_GetActorLocation`))
                  (goto _label_2 :!via `Close`)
                  (else
                    (`/Engine/EditorBlueprintResources/StandardMacros.IsValid` _tentacle_2_particlesystem_2 :!label _label_7
                      (:`Is Valid`
                        (`NiagaraComponent.ReinitializeSystem` _tentacle_2_particlesystem) ; eye open
                        (`FXSystemComponent.SetFloatParameter` _tentacle_2_particlesystem "Dynamic_UseIrisLook" 1.0)
                        (`FXSystemComponent.SetFloatParameter` _tentacle_2_particlesystem "Dynamic_EyeClosed" 0.0)
                        (`FXSystemComponent.SetFloatParameter` _tentacle_2_particlesystem "Dynamic_HasTarget" 0.0))
                      (:`Is Not Valid`
                        _))
                    (`self.PlaySFXFromSoundBank` "NewEnumerator5" (`self.K2_GetActorLocation`))
                    (goto _label_2 :!via `Open`)))))))))))

(event `OverrideCloseEyes`
  (goto _label_6))

(event `self.AgroSphere.OnComponentBeginOverlap`
  (params (OverlappedComponent :type "PrimitiveComponent Object Reference") (OtherActor :type "Actor Object Reference") (OtherComp :type "PrimitiveComponent Object Reference") (OtherBodyIndex :type Integer) (bFromSweep :type Boolean) (SweepResult :type "HitResult Structure (by ref)"))
  (if (not (`self.IsDead`))
    (goto _label_5 :!via `Open`)))

(event `self.AgroSphere.OnComponentEndOverlap`
  (params (OverlappedComponent :type "PrimitiveComponent Object Reference") (OtherActor :type "Actor Object Reference") (OtherComp :type "PrimitiveComponent Object Reference") (OtherBodyIndex :type Integer))
  (if (not (`self.IsDead`))
    (goto _label_5 :!via `Close`)))

(event `self.Event_OnDamageTaken`
  (params (Damage :type "Float (double-precision)") (`NoStagger/Knockback` :type Boolean))
  (if (not (`self.IsDead`))
    (`|ExecutionSequence`
      (:`then_0`
        (if (`self.Fleeing`)
          (set `self.Fleeing` false)
          (`self.SetEnemyStealthed` false)))
      (:`then_1`
        (goto _label_7)))))

(event `ReadyToScream`
  (bind _alertshakeduration (`self.AlertShakeDuration`))
  (bind _tentacle_2_particlesystem (`self.Tentacle_2_ParticleSystem`))
  (bind _tentacle_2_particlesystem_2 (`self.Tentacle_2_ParticleSystem`))
  (if (not (`self.IsDead`))
    (set `self.IsAlertShake` true)
    (`/Engine/EditorBlueprintResources/StandardMacros.IsValid` _tentacle_2_particlesystem
      (:`Is Valid`
        (`NiagaraComponent.ReinitializeSystem` _tentacle_2_particlesystem)
        (`FXSystemComponent.SetFloatParameter` _tentacle_2_particlesystem "Dynamic_HasTarget" 1.0)
        (`self.AlertShake`)
        (`KismetSystemLibrary.Delay` (* _alertshakeduration 0.25))
        (set `self.IsReadyToScream` true)
        (`KismetSystemLibrary.Delay` (* _alertshakeduration 0.75))
        (set `self.IsReadyToScream` false)
        (set `self.IsAlertShake` false)
        (set `self.IsEyeClosed` false)
        (`/Engine/EditorBlueprintResources/StandardMacros.IsValid` _tentacle_2_particlesystem_2
          (:`Is Valid`
            (`NiagaraComponent.ReinitializeSystem` _tentacle_2_particlesystem_2) ; eye closed
            (`FXSystemComponent.SetFloatParameter` _tentacle_2_particlesystem_2 "Dynamic_HasTarget" 0.0)))))))

(event `AlertShake`
  (bind _tentacle_2_particlesystem (`self.Tentacle_2_ParticleSystem`))
  (bind _returnvalue (* 2.0 -1.0))
  (bind _returnvalue_2 (* 2.0 0.25))
  (if (`self.IsAlertShake`) :!label _label_8
    (bind (_direction _x _y _z) (`Timeline|Timeline_1_0` :!via `PlayFromStart`)
      (:`Update`
        (if (`self.IsAlertShake`)
          (`/Engine/EditorBlueprintResources/StandardMacros.IsValid` _tentacle_2_particlesystem
            (:`Is Valid`
              (`SceneComponent.K2_SetRelativeLocation` _tentacle_2_particlesystem (`KismetMathLibrary.MakeVector` (`KismetMathLibrary.Lerp` 2.0 _returnvalue (`KismetMathLibrary.FClamp` _x -1.0)) (`KismetMathLibrary.Lerp` 2.0 _returnvalue (`KismetMathLibrary.FClamp` _y -1.0)) (`KismetMathLibrary.Lerp` _returnvalue_2 (* _returnvalue_2 -1.0) (`KismetMathLibrary.FClamp` _z -1.0))) false false)))))
      (:`Finished`
        (`/Engine/EditorBlueprintResources/StandardMacros.IsValid` _tentacle_2_particlesystem
          (:`Is Valid`
            (`SceneComponent.K2_SetRelativeLocation` _tentacle_2_particlesystem (0.0 0.0 0.0) false false)
            (goto _label_8))
          (:`Is Not Valid`
            (goto _label_8)))))))

(event `StartScreamCooldown`
  (set `self.CanSearch` false)
  (`KismetSystemLibrary.Delay` (`self.ScreamCooldown`))
  (set `self.CanSearch` true))

(fn `HideUnderPickup`
  (locals (NewLocalVar_2 :type "Vector Structure" :default (0.0 0.0 0.0)))
  (bind _returnvalue (`self.K2_GetActorLocation`))
  (bind _returnvalue_2 (enumliteral `EDrawDebugTrace` "None"))
  (bind _capsulecomponent (`self.CapsuleComponent`))
  (bind (_x _y) (`KismetMathLibrary.BreakVector3f` (`self.K2_GetActorLocation`)))
  (bind _capsulehalfheight (`CapsuleComponent.CapsuleHalfHeight` _capsulecomponent))
  (if (`self.Fleeing`)
    _
    (elif (`KismetMathLibrary.RandomBoolWithWeight` (`self.HideChance`))
      (bind _outhits (`KismetSystemLibrary.SphereTraceMultiForObjects` :`Start` _returnvalue :`End` _returnvalue :`Radius` (`KismetSystemLibrary.MakeLiteralDouble` (`self.HideRadius`)) :`ObjectTypes` (`|MakeArray` "ObjectTypeQuery11" "ObjectTypeQuery12" :!type "EObjectTypeQuery Enum") :`DrawDebugType` _returnvalue_2))
      (for _array_element _outhits
        (if (not (`self.Fleeing`))
          (bind (_bblockinghit _binitialoverlap _time _distance _location _impactpoint _normal _impactnormal _physmat _hitactor) (`GameplayStatics.BreakHitResult` _array_element))
          (if _bblockinghit
            (cast `/Game/Blueprints/Enemies/EnemyEntry_CrimsonGrass` _hitactor
              (:`CastFailed`
                (bind _asobject_entry_item_pickup (cast `/Game/Blueprints/Objects/ObjectEntry_ItemPickup` _hitactor))
                (bind _output_get (set `local.NewLocalVar_2` _location))
                (bind (_x_2 _y_2) (`KismetMathLibrary.BreakVector3f` _output_get))
                (bind _outhit (`KismetSystemLibrary.LineTraceSingleForObjects` :`Start` (`KismetMathLibrary.MakeVector` _x _y 150.0) :`End` (`KismetMathLibrary.MakeVector` _x_2 _y_2 150.0) :`ObjectTypes` (`|MakeArray` "ObjectTypeQuery1" "ObjectTypeQuery2" :!type "EObjectTypeQuery Enum") :`DrawDebugType` _returnvalue_2))
                (if (not (`GameplayStatics.BreakHitResult` _outhit))
                  (bind _object_substance (`/Game/Blueprints/Objects/ObjectEntry_Master.Object Substance` _asobject_entry_item_pickup))
                  (if (`KismetMathLibrary.RandomBoolWithWeight` (select `bool` (or (`|EnumEquality` _object_substance "NewEnumerator6") (`|EnumEquality` _object_substance "NewEnumerator3")) :`false` 0.25 :`true` 1.0 :!type "Float (single-precision)"))
                    (bind _returnvalue_3 (+ (`self.K2_GetActorLocation` _asobject_entry_item_pickup) (`KismetMathLibrary.MakeVector` 0.0 0.0 _capsulehalfheight)))
                    (bind _outhit_2 (`KismetSystemLibrary.CapsuleTraceSingleForObjects` _returnvalue_3 _returnvalue_3 (* (`CapsuleComponent.CapsuleRadius` _capsulecomponent) 0.9) (* _capsulehalfheight 0.9) (`|MakeArray` "ObjectTypeQuery8" :!type "EObjectTypeQuery Enum")))
                    (bind (_bblockinghit_2 _binitialoverlap_2 _time_2 _distance_2 _location_2 _impactpoint_2 _normal_2 _impactnormal_2 _physmat_2 _hitactor_2) (`GameplayStatics.BreakHitResult` _outhit_2))
                    (if _bblockinghit_2
                      (if (== _hitactor_2 _asobject_entry_item_pickup)
                        (`self.K2_SetActorLocation` _returnvalue_3 :!label _label)
                        (`self.SetEnemyStealthed` true)
                        (`self.OverrideCloseEyes`)
                        (set `self.PickupHiddenUnder` _asobject_entry_item_pickup)
                        (set `self.Fleeing` true))
                      (else
                        (goto _label)))))))))))))

(fn `SetVisuals`
  (locals (NewLocalVar_0 :type "Vector Structure" :default (0.0 0.0 0.0)) (NewLocalVar_1 :type "Float (double-precision)"))
  (bind _returnvalue (`KismetMathLibrary.RandomFloatInRange` 0.0175 0.03))
  (bind _rustpool (`self.RustPool`))
  (bind _tentacle_2_particlesystem (`self.Tentacle_2_ParticleSystem`))
  ;[1 1 1] set main weed
  (`SceneComponent.K2_SetRelativeRotation` _rustpool (`KismetMathLibrary.MakeRotator` 0.0 0.0 (`KismetMathLibrary.RandomFloatInRange` 0.0 360.0)) false false)
  (`SceneComponent.SetRelativeScale3D` _rustpool (`KismetMathLibrary.MakeVector` _returnvalue _returnvalue 1.0))
  (bind _output_get (set `self.UniqueNumRand` (`KismetMathLibrary.RandomFloatInRangeFromStream` -50.0 50.0 (`KismetMathLibrary.MakeRandomStream` (`self.UniqueNum`)))))
  (`FXSystemComponent.SetFloatParameter` (`self.Tentacle_2_ParticleSystem`) "Dynamic_Rand" _output_get)
  (`FXSystemComponent.SetFloatParameter` _tentacle_2_particlesystem "WidthMax" (`KismetMathLibrary.RandomFloatInRange` 12.5 17.5))
  (`FXSystemComponent.SetFloatParameter` _tentacle_2_particlesystem "HeightMax" (`KismetMathLibrary.RandomFloatInRange` 50.0 100.0))
  (`FXSystemComponent.SetFloatParameter` _tentacle_2_particlesystem "Dynamic_HasTarget" 0.0))

(fn `UserConstructionScript`
  (`parent.UserConstructionScript`)
  (`self.SetVisuals`))