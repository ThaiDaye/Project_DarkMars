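; Vaper enemy that spits out an expanding rust cloud, keeping only one active at a time.
; A new target, damage or entering rust triggers a mesh-squash windup before spawning, and rust presence swaps its spit particle.
; After polling for world generation, it starts an idle scale pulse and can spawn pre-clouded.
; Death switches to gib visuals and calls AddToCloud on nearby clouds found by sphere trace.
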(event `self.Event_NewTarget`
  ;[1 1 1] foudn target
  (`self.StartSpawnRustCloud`))

(event `SpawnRustCloud`
  (bind _enemygenref (`self.EnemyGenRef`))
  ;[1 1 1] spawn rust cloud
  (`/Engine/EditorBlueprintResources/StandardMacros.IsValid` (`self.RustCloudRef`)
    (:`Is Not Valid`
      (`NiagaraFunctionLibrary.SpawnSystemAtLocation` "/Game/VFX/Systems/Rust_Vaper_BigSpit.Rust_Vaper_BigSpit" (`SceneComponent.K2_GetComponentLocation` (`self.Spit_Particle`)))
      (`self.PlaySFXFromSoundBank` "NewEnumerator4" (`self.K2_GetActorLocation`))
      (bind _returnvalue (`|SpawnActorFromClass` "/Game/Blueprints/Enemies/RustCloud_BP.RustCloud_BP_C" (`KismetMathLibrary.MakeTransform` (`self.K2_GetActorLocation`)) "Undefined" "OverrideRootScale" null (`self.RustSpawnWithCloud`) (`self.RustRadius`) (`self.RustExpandRate`) self null))
      (set `self.RustCloudRef` _returnvalue)
      (`/Engine/EditorBlueprintResources/StandardMacros.IsValid` _enemygenref
        (:`Is Valid`
          (set `/Game/Blueprints/Enemies/EnemyMarkerGen_Master.SpawnInAltState` true _enemygenref))))))

(event `StartSpawnRustCloud`
  (bind _vaper_mesh (`self.Vaper_Mesh`))
  (bind (_relativescale3d_x _relativescale3d_y) (`KismetMathLibrary.BreakVector` (`SceneComponent.RelativeScale3D` _vaper_mesh)))
  ;[1 1 1] start spawn cloud shake
  (`/Engine/EditorBlueprintResources/StandardMacros.IsValid` (`self.RustCloudRef`) :!label _label
    (:`Is Not Valid`
      (if (not (or (`self.IsDead`) (`self.Staggered`) (`self.IsAttacking`)))
        (`self.PlaySFXFromSoundBank` "NewEnumerator3" (`self.K2_GetActorLocation`))
        (bind (_direction _newtrack_0) (`Timeline|Timeline_2` :!via `PlayFromStart`)
          (:`Update`
            (set `self.IsAttacking` true)
            (if (`self.Fog_Visible`)
              (if (not (`self.IsDead`))
                (`SceneComponent.SetRelativeScale3D` _vaper_mesh (`KismetMathLibrary.MakeVector` _relativescale3d_x _relativescale3d_y (`KismetMathLibrary.Lerp` 0.6 0.8 _newtrack_0))))))
          (:`Finished`
            (`KismetSystemLibrary.Delay` 0.2)
            (set `self.IsAttacking` false)
            (if (not (or (`self.IsDead`) (`self.Staggered`)))
              (`self.SpawnRustCloud`))))))))

(event `self.Event_OnRustCloudEnter`
  ;[1 1 1] set particle visual
  (`self.StartSpawnRustCloud`)
  (`NiagaraComponent.SetAsset` (`self.Spit_Particle`) (select `bool` (`self.IsInRustCloud`) :`false` "/Game/VFX/Systems/Rust_Vaper_Spit.Rust_Vaper_Spit" :`true` "/Game/VFX/Systems/Rust_Vaper_Spray.Rust_Vaper_Spray" :!type "NiagaraSystem Object Reference") true :!label _label_2))

(event `self.Event_OnDamageTaken`
  (params (Damage :type "Float (double-precision)") (`NoStagger/Knockback` :type Boolean))
  ;[1 1 1] start spawn cloud shake
  (goto _label))

(event `self.Event_OnRustCloudExit`
  ;[1 1 1] set particle visual
  (goto _label_2))

(event `self.ReceiveBeginPlay`
  (bind _vaper_mesh (`self.Vaper_Mesh`))
  (bind (_relativescale3d_x _relativescale3d_y) (`KismetMathLibrary.BreakVector` (`SceneComponent.RelativeScale3D` _vaper_mesh)))
  ;[1 1 1] begin play
  (set `self.MainStaticMesh` (`self.Vaper_Mesh`))
  (set `self.SubStaticMeshs` (`|MakeArray` (`self.R-GibRose1`) (`self.Tonge_Mesh`)))
  (`parent.ReceiveBeginPlay`)
  (`self.DoAfterWorldGen`
    (:`GenComplete`
      (`SceneComponent.K2_SetWorldRotation` (`self.Vaper_Mesh`) (`KismetMathLibrary.MakeRotator` 0.0 0.0 (`KismetMathLibrary.RandomFloatInRange` 0.0 360.0)) false false)
      (if (`self.RustSpawnWithCloud`)
        (`self.SpawnRustCloud`)
        (bind (_direction _newtrack_0) (`Timeline|Timeline_1_0` :!via `PlayFromStart` :!label _label_3)
          (:`Update`
            (if (`self.Fog_Visible`)
              (if (not (or (`self.IsDead`) (`self.IsAttacking`)))
                (`SceneComponent.SetRelativeScale3D` _vaper_mesh (`KismetMathLibrary.MakeVector` _relativescale3d_x _relativescale3d_y (`KismetMathLibrary.Lerp` 0.6 0.8 _newtrack_0))))))
          (:`Finished`
            (`KismetSystemLibrary.Delay` 0.75)
            (goto _label_3 :!via `PlayFromStart`)))
        (else
          (goto _label_3 :!via `PlayFromStart`))))))

(event `self.OnDeath`
  (bind _returnvalue (`self.K2_GetActorLocation`))
  (bind _tonge_mesh (`self.Tonge_Mesh`))
  (bind _r_gibrose1 (`self.R-GibRose1`))
  ;[1 1 1] on death
  (`parent.OnDeath`)
  (`MeshComponent.SetScalarParameterValueOnMaterials` (`self.MainStaticMesh`) "ROpacity" -500.0)
  (`SceneComponent.SetVisibility` _tonge_mesh false false)
  (`SceneComponent.SetVisibility` (`self.Spit_Particle`) false false)
  (`SceneComponent.SetHiddenInGame` _tonge_mesh true false)
  (`SceneComponent.SetHiddenInGame` (`self.Spit_Particle`) true false)
  (`SceneComponent.SetVisibility` _r_gibrose1 true false)
  (`SceneComponent.SetHiddenInGame` _r_gibrose1 false false)
  (bind _outhits (`KismetSystemLibrary.SphereTraceMultiForObjects` _returnvalue _returnvalue (`self.RustRadius`) (`|MakeArray` "ObjectTypeQuery10" :!type "EObjectTypeQuery Enum")))
  (for _array_element _outhits
    (bind _asrust_cloud_bp (cast `/Game/Blueprints/Enemies/RustCloud_BP` (`.HitActor` (`GameplayStatics.BreakHitResult` _array_element))))
    (`/Game/Blueprints/Enemies/RustCloud_BP.AddToCloud` _asrust_cloud_bp)))

(fn `UserConstructionScript`
  (`parent.UserConstructionScript`)
  (set `self.MainStaticMesh` (`self.Vaper_Mesh`))
  (`self.SetUniqueVisuals` false)
  (`SceneComponent.K2_SetWorldRotation` (`self.Vaper_Mesh`) (`KismetMathLibrary.MakeRotator` 0.0 0.0 (`KismetMathLibrary.RandomFloatInRange` 0.0 360.0)) false false))