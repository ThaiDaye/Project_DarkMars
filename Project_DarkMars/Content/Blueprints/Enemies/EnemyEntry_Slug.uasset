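; Slug enemy that leaps onto characters, latches to their spine, applies a status effect and deals timed damage before detaching.
; Without a target it wanders or seeks pickups to eat, and aggros on Death Stench-marked characters via overlap and line-of-sight checks.
; AI movement feeds timeline rotation into the leap, with a delayed-loop macro pacing bites.
; Overrides add chance-based fleeing and dismemberment effects, including a stench-sack burst affecting the nearby player.
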(event `self.Event_NewTarget`
  (`self.MoveToTarget`))

(event `self.Event_KnockbackEnd`
  ;[1 0.2812 0.2812] Event knockbackEnd (might not need)
  (`self.MoveToTarget`)
  (set `self.IsAttacking` false))

(event `self.ReceiveBeginPlay`
  ;[1 1 1] init
  (set `self.SubStaticMeshs` (`|MakeArray` (`self.B-GibRose`) (`self.G-GibRose`) (`self.R-GibRose`)))
  (`parent.ReceiveBeginPlay`)
  (`self.SetCollisionIsOverlap` false)
  (`self.MoveToTarget`)
  (`self.Idle_NoTarget`)
  (`KismetSystemLibrary.K2_SetTimerDelegate` (delegate `Idle_NoTarget`) 10.0 true))

(event `self.CapsuleComponent.OnComponentBeginOverlap`
  (params (OverlappedComponent :type "PrimitiveComponent Object Reference") (OtherActor :type "Actor Object Reference") (OtherComp :type "PrimitiveComponent Object Reference") (OtherBodyIndex :type Integer) (bFromSweep :type Boolean) (SweepResult :type "HitResult Structure (by ref)"))
  (bind _isactorattached (`self.IsActorAttached`))
  ;[1 1 1] ATTACKING
  (if (`self.CollisionIsOverlap`)
    (if (not (or (`self.IsDead`) (`self.Fleeing`) (`self.IsAttacking`)))
      (bind _asbp_top_down_character (cast `/Game/Blueprints/BP_TopDownCharacter` OtherActor))
      (`self.K2_AttachToComponent` self (`Character.Mesh` _asbp_top_down_character) "spine_05" "KeepWorld" "KeepWorld" "KeepWorld" true)
      (`ActorComponent.Deactivate` (`self.CharacterMovement`))
      (`self.K2_AddActorWorldRotation` (struct :`Roll` -45.0))
      (`/Engine/EditorBlueprintResources/StandardMacros.IsValid` (`Character.Mesh` _asbp_top_down_character)
        (:`Is Valid`
          (set `self.IsAttacking` true)
          (`self.K2_SetActorLocation` (+ (`SceneComponent.GetSocketLocation` (`Character.Mesh` _asbp_top_down_character) "spine_05") (* (`self.GetActorUpVector`) 25.0)))
          (set `self.IsActorAttached` true)
          (`KismetSystemLibrary.Delay` 0.5)
          (`/Game/Blueprints/BP_TopDownCharacter.Apply Status Effects` _asbp_top_down_character "NewEnumerator1")
          (`self.ForLoopDelay` 0 2 :!label _label
            (:`LoopBody`
              (if _isactorattached
                (`/Game/Blueprints/BP_TopDownCharacter.TakeDamage` _asbp_top_down_character (`self.BaseDamage`) 0.15 (`self.Stagger Duration`) (`self.Knockback Amount`) self)
                (`/Game/Blueprints/BP_TopDownCharacter.ImpactVFX` (`self.PlayerRef`) (`self.K2_GetActorLocation` _asbp_top_down_character) (`KismetMathLibrary.Conv_VectorToRotator` (`self.GetActorUpVector`)) false (make `/Game/Blueprints/Data/VFXData_Struct` "/Game/VFX/Systems/BulletEffectParticle/EquipEffect_Bullet_ParticleSystem.EquipEffect_Bullet_ParticleSystem" "/Game/VFX/Systems/Decal/Decal_ParticleSystem.Decal_ParticleSystem" "/Game/VFX/Systems/Debris/Debris_ParticleSystem.Debris_ParticleSystem" "/Game/VFX/sA_Megapack_v1/sA_ShootingVfxPack/FX/NiagaraSystems/NS_AR_Muzzleflash_1_ONCE.NS_AR_Muzzleflash_1_ONCE" "/Game/VFX/Systems/ImpactDust_ParticleSystem.ImpactDust_ParticleSystem" "/Game/VFX/Systems/Trail_Particle.Trail_Particle" "/Game/VFX/Systems/Projectile_Mag_Case_particle_System.Projectile_Mag_Case_particle_System" "/Game/VFX/Systems/Projectile_Bullet_Case_Particle_System.Projectile_Bullet_Case_Particle_System" "/Game/VFX/Systems/MeleeTrail_Particle.MeleeTrail_Particle" 0.5 "/Game/VFX/Systems/Charge_Low_ParticleSystem.Charge_Low_ParticleSystem" "/Game/VFX/Systems/Charge_Mid_ParticleSystem.Charge_Mid_ParticleSystem" "/Game/VFX/Systems/Charge_High_ParticleSystem.Charge_High_ParticleSystem" null) (`self.BaseDamage`))
                (`self.PlaySFXFromSoundBank` "NewEnumerator5" (`self.K2_GetActorLocation`))))
            (:`Complete`
              (if _isactorattached
                (`self.K2_DetachFromActor` self "KeepWorld" "KeepWorld" "KeepWorld")
                (`self.K2_SetActorRelativeRotation` (struct))
                (bind _randomlocation (`NavigationSystemV1.K2_GetRandomLocationInNavigableRadius` (`self.K2_GetActorLocation`) 150.0 null null))
                (`self.K2_SetActorLocation` _randomlocation)
                (`ActorComponent.Activate` (`self.CharacterMovement`) true)
                (set `self.IsActorAttached` false)
                (set `self.IsAttacking` false)
                (`self.SetCollisionIsOverlap` false)
                (`self.MoveToTarget`)))
            (:`OutDelay`
              (`KismetSystemLibrary.Delay` 2.0)
              (goto _label :!via `InDelay`))))))))

(event `Idle_NoTarget`
  (bind (_returnvalue_roll _returnvalue_pitch) (`KismetMathLibrary.BreakRotator` (`self.K2_GetActorRotation`)))
  (bind _eattarget (`self.EatTarget`))
  (bind _returnvalue (`SceneComponent.K2_GetComponentLocation` (`self.Mesh`)))
  (bind (_returnvalue_roll_2 _returnvalue_pitch_2 _returnvalue_yaw) (`KismetMathLibrary.BreakRotator` (`KismetMathLibrary.FindLookAtRotation` (`self.K2_GetActorLocation`) (`self.K2_GetActorLocation` (`self.EatTarget`)))))
  ;[1 1 1] idle walk
  (if (not (`self.IsDead`))
    (`/Engine/EditorBlueprintResources/StandardMacros.IsValid` (`self.Target`)
      (:`Is Not Valid`
        (if (`self.IsEating`)
          _
          (elif (`KismetMathLibrary.RandomBoolWithWeight` 0.5)
            ;[1 1 1] idle eat
            (if (not (or (`self.CollisionIsOverlap`) (`self.Fleeing`) (`self.Staggered`)))
              (set `self.EatTarget` null)
              (bind _outhits (`KismetSystemLibrary.SphereTraceMultiForObjects` _returnvalue _returnvalue 500.0 (`|MakeArray` "ObjectTypeQuery11" :!type "EObjectTypeQuery Enum")))
              (for _array_element _outhits
                (bind (_bblockinghit _binitialoverlap _time _distance _location _impactpoint _normal _impactnormal _physmat _hitactor) (`GameplayStatics.BreakHitResult` _array_element))
                (if _bblockinghit
                  (bind _asobject_entry_item_pickup (cast `/Game/Blueprints/Objects/ObjectEntry_ItemPickup` _hitactor))
                  (`/Engine/EditorBlueprintResources/StandardMacros.IsValid` (`self.EatTarget`)
                    (:`Is Valid`
                      (if (`/Game/Blueprints/Objects/ObjectEntry_ItemPickup.IsPlayerDropped` _asobject_entry_item_pickup)
                        (if (`|EnumEquality` (`/Game/Blueprints/Objects/ObjectEntry_Master.Object Substance` _asobject_entry_item_pickup) "NewEnumerator3") :!label _label_2
                          (set `self.EatTarget` _asobject_entry_item_pickup))))
                    (:`Is Not Valid`
                      (if (`KismetMathLibrary.RandomBoolWithWeight` 0.5)
                        (goto _label_2))))))
              (`/Engine/EditorBlueprintResources/StandardMacros.IsValid` _eattarget
                (:`Is Valid`
                  (`|AIMoveTo` self (0.0 0.0 0.0) _eattarget 75.0
                    (:`OnSuccess`
                      (`self.K2_SetActorRotation` (`KismetMathLibrary.MakeRotator` _returnvalue_roll _returnvalue_pitch _returnvalue_yaw))
                      (set `self.IsEating` true))))))
            (elif (`KismetMathLibrary.RandomBoolWithWeight` 0.75)
              (set `self.IdleRotateWeight` (`KismetMathLibrary.RandomFloatInRange` -0.25 0.25))
              (bind (_direction _newtrack_0) (`Timeline|Timeline_2` :!via `PlayFromStart`)
                (:`Update`
                  (if (not (`self.Staggered`))
                    (`self.AddMovementInput` (`self.GetActorForwardVector`) 0.6)
                    (`self.AddMovementInput` (`self.GetActorRightVector`) (* _newtrack_0 (`self.IdleRotateWeight`) 0.1))))))))))))

(event `MoveToTarget`
  ;[1 1 1] MOVE TO TARGET
  (if (not (`self.IsDead`))
    (`/Engine/EditorBlueprintResources/StandardMacros.IsValid` (`self.Target`)
      (:`Is Valid`
        (if (not (or (`self.CollisionIsOverlap`) (`self.Fleeing`) (`self.Staggered`)))
          (`self.SetIsMovingToTarget` true)
          (`|AIMoveTo` self (0.0 0.0 0.0) (`self.Target`) (`self.MoveRadius`) true
            (:`OnSuccess`
              (`self.SetIsMovingToTarget` false)
              (if (`self.AttackCooldown`)
                (`/Engine/EditorBlueprintResources/StandardMacros.Gate` false :!label _label_3
                  (:`Exit`
                    (`|ExecutionSequence`
                      (:`then_0`
                        _)
                      (:`then_1`
                        (goto _label_3 :!via `Close`))
                      (:`then_2`
                        (`self.SetCanAttack` false)
                        (`KismetSystemLibrary.Delay` 10.0)
                        (`self.SetCanAttack` true)
                        (goto _label_3 :!via `Open`))))))
              (`self.RotateToTarget` true))
            (:`OnFail`
              (`self.SetIsMovingToTarget` false)
              (`self.RotateToTarget` false))))))))

(event `RotateToTarget`
  (params (AttackAfter :type Boolean))
  (bind _capsulecomponent (`self.CapsuleComponent`))
  ;[1 1 1] ROTATE TO TARGET
  (set `self.RotationStart` (`SceneComponent.K2_GetComponentRotation` (`self.CapsuleComponent`)))
  (`self.PlaySFXFromSoundBank` "NewEnumerator3" (`self.K2_GetActorLocation`))
  (bind (_direction _newtrack_0) (`Timeline|Timeline_1_0` :!via `PlayFromStart`)
    (:`Update`
      (`/Engine/EditorBlueprintResources/StandardMacros.IsValid` (`self.Target`)
        (:`Is Valid`
          (if (not (or (`self.IsDead`) (`self.Fleeing`) (`self.Staggered`)))
            (`SceneComponent.K2_SetWorldRotation` _capsulecomponent (`KismetMathLibrary.RLerp` (`self.RotationStart`) (`KismetMathLibrary.MakeRotator` (.roll (`SceneComponent.K2_GetComponentRotation` _capsulecomponent)) (.pitch (`SceneComponent.K2_GetComponentRotation` _capsulecomponent)) (.yaw (`KismetMathLibrary.FindLookAtRotation` (`self.K2_GetActorLocation` self) (`self.K2_GetActorLocation` (`self.Target`))))) _newtrack_0 true) false false)))))
    (:`Finished`
      (if AttackAfter
        (`self.Leap` false)
        (else
          (`self.MoveToTarget`))))))

(event `self.MarkedAgroSphere.OnComponentBeginOverlap`
  (params (OverlappedComponent :type "PrimitiveComponent Object Reference") (OtherActor :type "Actor Object Reference") (OtherComp :type "PrimitiveComponent Object Reference") (OtherBodyIndex :type Integer) (bFromSweep :type Boolean) (SweepResult :type "HitResult Structure (by ref)"))
  (bind _potentialtarget (`self.PotentialTarget`))
  ;[1 1 1] marked gain agro
  (if (not (`self.IsDead`))
    (`/Engine/EditorBlueprintResources/StandardMacros.IsValid` (`self.Target`)
      (:`Is Not Valid`
        (bind _asbp_top_down_character (cast `/Game/Blueprints/BP_TopDownCharacter` OtherActor))
        (if (`/Game/Blueprints/BP_TopDownCharacter.Status_DeathStenchMark` _asbp_top_down_character)
          (set `self.PotentialTarget` _asbp_top_down_character)
          (`|ExecutionSequence`
            (:`then_0`
              (goto _label_4 :!via `Open`))
            (:`then_1`
              (`/Engine/EditorBlueprintResources/StandardMacros.Gate` true :!label _label_4
                (:`Exit`
                  (`|ExecutionSequence`
                    (:`then_0`
                      (bind _outhit (`KismetSystemLibrary.LineTraceSingle` :`Start` (`self.K2_GetActorLocation`) :`End` (`self.K2_GetActorLocation` _potentialtarget) :`TraceChannel` "TraceTypeQuery1" :`DrawDebugType` (select `bool` (`self.Debug_HideCollisions`) :`false` "ForDuration" :!type "EDrawDebugTrace Enum")))
                      (bind (_bblockinghit _binitialoverlap _time _distance _location _impactpoint _normal _impactnormal _physmat _hitactor) (`GameplayStatics.BreakHitResult` _outhit))
                      (if _bblockinghit
                        (if (== _hitactor (`self.PotentialTarget`))
                          (`self.SetTarget` (`self.PotentialTarget`) :!label _label_5)
                          (set `self.PotentialTarget` null))
                        (else
                          (goto _label_5))))
                    (:`then_1`
                      (`/Engine/EditorBlueprintResources/StandardMacros.IsValid` _potentialtarget
                        (:`Is Valid`
                          (`KismetSystemLibrary.Delay` 1.0)
                          (goto _label_4))))))))))))))

(event `self.MarkedAgroSphere.OnComponentEndOverlap`
  (params (OverlappedComponent :type "PrimitiveComponent Object Reference") (OtherActor :type "Actor Object Reference") (OtherComp :type "PrimitiveComponent Object Reference") (OtherBodyIndex :type Integer))
  (bind _potentialtarget (`self.PotentialTarget`))
  ;[1 1 1] marked gain agro
  (if (`self.IsDead`)
    _
    (elif (== OtherActor _potentialtarget)
      (bind _asbp_top_down_character (cast `/Game/Blueprints/BP_TopDownCharacter` _potentialtarget))
      (if (`/Game/Blueprints/BP_TopDownCharacter.Status_DeathStenchMark` _asbp_top_down_character)
        (set `self.PotentialTarget` null)
        (goto _label_4 :!via `Close`)))))

(event `Leap`
  (params (NoGravity :type Boolean))
  (bind _charactermovement (`self.CharacterMovement`))
  ;[1 1 1] LEAP
  (if (not (`self.IsDead`))
    (`NiagaraFunctionLibrary.SpawnSystemAtLocation` "/Game/VFX/Systems/Rust_Leap_ImpactDust_ParticleSystem1.Rust_Leap_ImpactDust_ParticleSystem1" (`self.K2_GetActorLocation`))
    (`self.SetCollisionIsOverlap` true)
    (if (`self.Staggered`)
      _
      (elif NoGravity
        (`MovementComponent.StopMovementImmediately` (`self.CharacterMovement`) :!label _label_6)
        (`self.PlaySFXFromSoundBank` "NewEnumerator4" (`self.K2_GetActorLocation`))
        (`CharacterMovementComponent.AddImpulse` _charactermovement (0.0 0.0 550.0) true)
        (`KismetSystemLibrary.Delay` 0.01)
        (`CharacterMovementComponent.AddImpulse` _charactermovement (* (`SceneComponent.GetForwardVector` (`self.ForwardArrow`)) 350.0) true)
        (elif (not (`NavMovementComponent.IsFalling` (`self.CharacterMovement`)))
          (goto _label_6))))))

(event `self.ReceiveHit`
  (params (MyComp :type "PrimitiveComponent Object Reference") (Other :type "Actor Object Reference") (OtherComp :type "PrimitiveComponent Object Reference") (bSelfMoved :type Boolean) (HitLocation :type "Vector Structure") (HitNormal :type "Vector Structure") (NormalImpulse :type "Vector Structure") (Hit :type "HitResult Structure (by ref)"))
  ;[1 1 1] LEAP
  (`|ExecutionSequence`
    (:`then_0`
      (`/Engine/EditorBlueprintResources/StandardMacros.Gate` false :!label _label_7
        (:`Exit`
          (`|ExecutionSequence`
            (:`then_0`
              (if (`self.CollisionIsOverlap`)
                (if (not (`self.IsActorAttached`))
                  (if (not (`|EnumEquality` (`PrimitiveComponent.GetCollisionObjectType` (`.HitComponent` (`GameplayStatics.BreakHitResult` Hit))) "ECC_GameTraceChannel3"))
                    (bind _asobject_entry_master (cast `/Game/Blueprints/Objects/ObjectEntry_Master` Other)
                      (:`then`
                        (`/Game/Blueprints/Objects/ObjectEntry_Master.TakeDamage_Object` _asobject_entry_master (`self.BaseDamage`) 0.5))
                      (:`CastFailed`
                        _)))
                  (`self.SetCollisionIsOverlap` false)
                  (`self.MoveToTarget`)
                  (set `self.IsAttacking` false)
                  (`NiagaraFunctionLibrary.SpawnSystemAtLocation` (select `bool` (`self.DeadSimulating`) :`false` "/Game/VFX/Systems/Dust_ParticleSystem.Dust_ParticleSystem" :`true` "/Game/VFX/Systems/Rust_Leap_ImpactDust_ParticleSystem1.Rust_Leap_ImpactDust_ParticleSystem1" :!type "NiagaraSystem Object Reference") (`self.K2_GetActorLocation`)))))
            (:`then_1`
              (`KismetSystemLibrary.Delay` 0.5)
              (goto _label_7 :!via `Open`))))))
    (:`then_1`
      (goto _label_7 :!via `Close`))))

(event `self.Event_DismemberAction`
  (params (RGBSelect :type Integer))
  (bind _playerref (`self.PlayerRef`))
  (bind _arrowg (`self.ArrowG`))
  (bind _returnvalue (`SceneComponent.K2_GetComponentLocation` (`self.Mesh`)))
  (bind _returnvalue_2 (`SceneComponent.K2_GetComponentLocation` _arrowg))
  (`self.PlaySFXFromSoundBank` (select `int` RGBSelect :`0` "NewEnumerator6" :`1` "NewEnumerator7" :`2` "NewEnumerator13" :!type "/Game/Blueprints/Data/SoundBank_Enemy_Type Enum") (`self.K2_GetActorLocation`))
  (switch `int` RGBSelect
    (:`0`
      ;[1 0.7742 0.7242] Slug dismember - skull
      (if (not (`self.BoneDestroyedR`))
        (`|SpawnActorFromClass` "/Game/Blueprints/Projectiles/Gib_Skull.Gib_Skull_C" (`KismetMathLibrary.MakeTransform` (.location (`SceneComponent.K2_GetComponentToWorld` (`self.ArrowR`))) (`KismetMathLibrary.MakeRotator` (.roll (.rotation (`SceneComponent.K2_GetComponentToWorld` (`self.ArrowR`)))) (+ (.pitch (.rotation (`SceneComponent.K2_GetComponentToWorld` (`self.ArrowR`)))) (`KismetMathLibrary.RandomFloatInRange` -45.0 45.0)) (+ (.yaw (.rotation (`SceneComponent.K2_GetComponentToWorld` (`self.ArrowR`)))) (`KismetMathLibrary.RandomFloatInRange` -45.0 45.0)))) "AlwaysSpawn" "OverrideRootScale" null null 0.0 0.0 0.0 0.0 0.0 0.0 0.0 "NewEnumerator0" false false true (struct) "ECC_GameTraceChannel3" null)))
    (:`1`
      ;[1 1 1] dismember torso
      (bind _outhits (`KismetSystemLibrary.SphereTraceMultiForObjects` _returnvalue _returnvalue 150.0 (`|MakeArray` "ObjectTypeQuery7" :!type "EObjectTypeQuery Enum")))
      (for _array_element _outhits
        (bind (_bblockinghit _binitialoverlap _time _distance _location _impactpoint _normal _impactnormal _physmat _hitactor) (`GameplayStatics.BreakHitResult` _array_element))
        (if _bblockinghit
          (if (== _hitactor _playerref)
            (`/Game/Blueprints/BP_TopDownCharacter.Apply Status Effects` _playerref "NewEnumerator1"))))
      (`NiagaraFunctionLibrary.SpawnSystemAtLocation` "/Game/VFX/Systems/ImpactBloodDust_StenchSack_ParticleSystem.ImpactBloodDust_StenchSack_ParticleSystem" _returnvalue_2)
      (`NiagaraFunctionLibrary.SpawnSystemAtLocation` "/Game/VFX/Systems/Rust_Blood_ParticleSystem.Rust_Blood_ParticleSystem" _returnvalue_2 (`SceneComponent.K2_GetComponentRotation` _arrowg)))))

(event `self.Event_EnemyFlee`
  (bind _playerref (`self.PlayerRef`))
  (bind _playerref_2 (`self.PlayerRef`))
  ;[1 1 1] ENEMY FLEE
  (if (not (`self.Fleeing`))
    (`/Engine/EditorBlueprintResources/StandardMacros.IsValid` _playerref_2
      (:`Is Valid`
        (`/Game/Blueprints/BP_TopDownCharacter.Debug_PrintString_Internal` :`self` _playerref_2 :`Text` "Enemy Flee Chance" :`Colour` (struct :`R` 0.208059 :`G` 0.649368 :`B` 1.0 :`A` 1.0)))
      (:`Is Not Valid`
        _))
    (if (`KismetMathLibrary.RandomBoolWithWeight` 0.25)
      (set `self.Fleeing` true)
      (`MovementComponent.StopMovementImmediately` (`self.CharacterMovement`))
      (`/Engine/EditorBlueprintResources/StandardMacros.IsValid` _playerref
        (:`Is Valid`
          (`/Game/Blueprints/BP_TopDownCharacter.Debug_PrintString_Internal` :`self` _playerref :`Text` "SUCCESS" :`Colour` (struct :`R` 0.208059 :`G` 0.649368 :`B` 1.0 :`A` 1.0)))
        (:`Is Not Valid`
          _))
      (`self.Event_EnemyFleeSuccess`)
      (else
        (`/Engine/EditorBlueprintResources/StandardMacros.IsValid` _playerref
          (:`Is Valid`
            (`/Game/Blueprints/BP_TopDownCharacter.Debug_PrintString_Internal` :`self` _playerref :`Text` "FAILURE" :`Colour` (struct :`R` 0.208059 :`G` 0.649368 :`B` 1.0 :`A` 1.0))))))))

(event `self.Event_EnemyFleeSuccess`
  (bind _playerref (`self.PlayerRef`))
  (bind _target (`self.Target`))
  ;[1 1 1] ENEMY FLEE
  (`parent.Event_EnemyFleeSuccess`)
  (if (not (`self.IsDead`))
    (`/Engine/EditorBlueprintResources/StandardMacros.IsValid` _target
      (:`Is Valid`
        (set `self.IdleRotateWeight` (`KismetMathLibrary.RandomFloatInRange` -0.25 0.25))
        (bind (_direction _newtrack_0) (`Timeline|Timeline_3` :!via `PlayFromStart`)
          (:`Update`
            (if (not (`self.Staggered`))
              (`/Engine/EditorBlueprintResources/StandardMacros.IsValid` (`self.Target`)
                (:`Is Valid`
                  (`self.AddMovementInput` (`KismetMathLibrary.Conv_RotatorToVector` (`KismetMathLibrary.MakeRotator` 0.0 0.0 (.yaw (`KismetMathLibrary.FindLookAtRotation` (`self.K2_GetActorLocation` _target) (`self.K2_GetActorLocation`))))) 2.0)
                  (`self.AddMovementInput` (`self.GetActorRightVector`) (* _newtrack_0 0.75))))))
          (:`Finished`
            (`self.SetTarget` null)
            (set `self.Fleeing` false)
            (`/Engine/EditorBlueprintResources/StandardMacros.IsValid` _playerref
              (:`Is Valid`
                (`/Game/Blueprints/BP_TopDownCharacter.Debug_PrintString_Internal` :`self` _playerref :`Text` "Enemy Finished Fleeing" :`Colour` (struct :`R` 0.208059 :`G` 0.649368 :`B` 1.0 :`A` 1.0))))))))))

(fn `UserConstructionScript`
  (`parent.UserConstructionScript`))